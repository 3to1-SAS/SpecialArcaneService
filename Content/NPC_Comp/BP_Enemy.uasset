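; BP_Enemy is an AI-driven enemy that loads its BetaEnemy stats from DT_Enemies into HP and its Blackboard.
; Spell overlaps subtract damage looked up in DT_Spells by class-derived row name, while sword overlaps kill instantly.
; Hits turn it toward the source, and death destroys it and updates the game mode's enemy count.
; SpellDetected flags noise investigation at the player's location when within hearing radius.
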(event OnComponentBeginOverlap(CapsuleComponent)
  (params (OverlappedComponent :type Primitive%20Component%20Object%20Reference) (OtherActor :type Actor%20Object%20Reference) (OtherComp :type Primitive%20Component%20Object%20Reference) (OtherBodyIndex :type Integer) (bFromSweep :type Boolean) (SweepResult :type Hit%20Result%20Structure%20%28by%20ref%29))
  (bind _returnvalue (Utilities|GetClass OtherActor))
  ;[0.15 0.15 0.15 0.5] Calculates damage based on spell
  (if (Actor|ActorHasTag OtherActor "Spell")
    (bind _returnname (CallFunction|GetRowName _returnvalue))
    (bind _returnvalue_2 (Utilities|GetDataTableRow "/Game/DataTables/Spells/DT_Spells.DT_Spells" _returnname)
      (:then
        (Variables|Default|SetHP (- (Variables|Default|GetHP) (.SpellDamage (Utilities|Struct|BreakSpellStructure _returnvalue_2))))
        (Transformation|SetActorRotation (Math|Rotator|MakeRotator 0.0 0.0 (.yaw (Math|Rotator|FindLookatRotation (Transformation|GetActorLocation) (Transformation|GetActorLocation OtherActor)))) :!label _label)
        ;[0.15 0.15 0.15 0.5] Destroys enemy when health is 0
        (if (<= (Variables|Default|GetHP) 0.0)
          (Actor|DestroyActor)
          (bind _asbp_first_person_game_mode (Utilities|Casting|CastToBP_FirstPersonGameMode (Game|GetGameMode)))
          (Default|UpdateEnemyCount _asbp_first_person_game_mode))))
    (elif (== _returnvalue "/Game/Weapons/MeleeAttacks/BP_Sword.BP_Sword_C")
      (Variables|Default|SetHP (- 0.0 6e+02))
      (goto _label))))

(event EventBeginPlay
  (bind _returnvalue (AI|GetBlackboard 0))
  ;[0.15 0.15 0.15 0.5] Sets The Data Table Row and Spell Cooldown on the Blackboard
  (Utilities|FlowControl|DelayUntilNextTick)
  (Class|BlackboardComponent|SetValueasName _returnvalue (Variables|Default|GetDataTableRow) "BetaEnemy")
  (bind _returnvalue_2 (Utilities|GetDataTableRow "/Game/DataTables/Enemies/DT_Enemies.DT_Enemies" "BetaEnemy")
    (:then
      (AI|Components|Blackboard|SetValueasFloat _returnvalue (Variables|Default|GetSpellCooldown) (.SpellCooldown (Utilities|Struct|BreakEnemiesStructure _returnvalue_2)))
      (Variables|Default|SetHP (.MaxHP (Utilities|Struct|BreakEnemiesStructure _returnvalue_2)))
      (AI|Components|Blackboard|SetValueasFloat _returnvalue (Variables|Default|GetLOSTime) (.ChaseTime (Utilities|Struct|BreakEnemiesStructure _returnvalue_2))))))

(fn ConstructionScript)

(fn GetRowName
  (params (Class :type Actor%20Class%20Reference))
  (if (== Class "/Game/Weapons/MagicAttacks/BetaSpells/BP_BasicSpell.BP_BasicSpell_C")
    (return "BasicSpell")
    (elif (== Class "/Game/Weapons/MagicAttacks/BetaSpells/BP_RapidSpell.BP_RapidSpell_C")
      (return "RapidSpell")
      (elif (== Class "/Game/Weapons/MagicAttacks/BetaSpells/BP_ExplosiveSpell.BP_ExplosiveSpell_C")
        (return "ExplosiveSpell")
        (elif (== Class "/Game/Weapons/MagicAttacks/OfficialSpells/MagicMissile/BP_MagicMissile.BP_MagicMissile_C")
          (return "MagicMissile")
          (elif (== Class "/Game/Weapons/MagicAttacks/OfficialSpells/IceShards/BP_IceShard.BP_IceShard_C")
            (return "IceShards")
            (elif (== Class "/Game/Weapons/MagicAttacks/OfficialSpells/HydroBeam/BP_HydroPierce.BP_HydroPierce_C")
              (return "HydroPierce")
              (elif (== Class "/Game/Weapons/MagicAttacks/OfficialSpells/CombustionSpell/BP_Combustion.BP_Combustion_C")
                (return "Combustion")))))))))

(fn SpellDetected
  (params (DetectedPlayer :type Actor%20Object%20Reference))
  (bind _returnvalue (AI|GetBlackboard 0))
  (bind _returnvalue_2 (Utilities|GetDataTableRow "/Game/DataTables/Enemies/DT_Enemies.DT_Enemies" "BetaEnemy")
    (:then
      ;[0.15 0.15 0.15 0.5] Sets the necessary blackboard values
      (if (<= (Transformation|GetDistanceTo DetectedPlayer) (.HearingRadius (Utilities|Struct|BreakEnemiesStructure _returnvalue_2)))
        (Development|PrintString "Spell Detected")
        (AI|Components|Blackboard|SetValueasBool _returnvalue (LocalVariables|GetInvestigatingNoise) true)
        (AI|Components|Blackboard|SetValueasVector _returnvalue (LocalVariables|GetDetectedLocation) (Transformation|GetActorLocation DetectedPlayer))))))