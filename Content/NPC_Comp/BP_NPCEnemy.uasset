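; Enemy NPC that patrols random reachable points until it sees the player, then permanently switches to ranged attacks.
; A self-recalling Routine picks Patrol or Attack from a flag set by PawnSensing or AIPerception.
; Attack approaches the player and spawns BP_DemoEnemyAttack on a cooldown, adding random aim error beyond FallOffRange.
; Spell overlaps subtract DT_Spells damage, sword overlaps kill outright, and death calls SpawnExtract on the game mode.
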(event OnPerceptionUpdated(AIPerception)
  (params (UpdatedActors :type Array%20of%20Actor%20Object%20References))
  ;[0.15 0.15 0.15 0.5] Handles See Player Event
  (for _array_element UpdatedActors
    (if (== _array_element (Game|GetPlayerCharacter 0))
      (Variables|Default|SetAM true)
      (Development|PrintString "見えたよ！！！！！！！！！！！！！！！！！！！！！！！！！！！！！！！！！！！！！！！！！！！！！！！"))))

(event OnTargetPerceptionUpdated(AIPerception)
  (params (Actor :type Actor%20Object%20Reference) (Stimulus :type AI%20Stimulus%20Structure))
  ;[0.15 0.15 0.15 0.5] Handles See Player Event
  (if (== (Game|GetPlayerCharacter 0) Actor)
    (Variables|Default|SetAM true)
    (Development|PrintString "見えたよ！！！！！！！！！！！！！！！！！！！！！！！！！！！！！！！！！！！！！！！！！！！！！！！")))

(event OnSeePawn(PawnSensing)
  (params (Pawn :type Pawn%20Object%20Reference))
  ;[0.15 0.15 0.15 0.5] Handles See Player Event
  (if (== Pawn (Game|GetPlayerCharacter 0))
    (Variables|Default|SetAM true)
    (Development|PrintString "見えたよ！！！！！！！！！！！！！！！！！！！！！！！！！！！！！！！！！！！！！！！！！！！！！！！")))

(event OnComponentBeginOverlap(CapsuleComponent)
  (params (OverlappedComponent :type Primitive%20Component%20Object%20Reference) (OtherActor :type Actor%20Object%20Reference) (OtherComp :type Primitive%20Component%20Object%20Reference) (OtherBodyIndex :type Integer) (bFromSweep :type Boolean) (SweepResult :type Hit%20Result%20Structure%20%28by%20ref%29))
  (bind _returnvalue (Utilities|GetClass OtherActor))
  ;[0.15 0.15 0.15 0.5] Damage and Death
  (if (Actor|ActorHasTag OtherActor "Spell")
    (bind _returnname (CallFunction|GetRowName _returnvalue))
    (bind _returnvalue_2 (Utilities|GetDataTableRow "/Game/Weapons/MagicAttacks/DT_Spells.DT_Spells" _returnname)
      (:then
        (Variables|Default|SetHP (- (Variables|Default|GetHP) (.SpellDamage (Utilities|Struct|BreakSpellStructure _returnvalue_2))))
        (if (<= (Variables|Default|GetHP) 0.0) :!label _label
          (Actor|DestroyActor)
          (bind _asbp_first_person_game_mode (Utilities|Casting|CastToBP_FirstPersonGameMode (Game|GetGameMode)))
          (Default|SpawnExtract _asbp_first_person_game_mode))))
    (elif (== _returnvalue "/Game/Weapons/MeleeAttacks/BP_Sword.BP_Sword_C")
      (Variables|Default|SetHP (- 0.0 6e+02))
      (goto _label))))

(event Custom|Routine
  ;[0.15 0.15 0.15 0.5] EventTick() but not mid
  (if (Variables|Default|GetAM)
    (CallFunction|Attack)
    (else
      (CallFunction|Patrol))))

(event Custom|Attack
  (bind _returnvalue (Transformation|GetActorTransform))
  (bind _returnvalue_2 (Game|Player|GetPlayerPawn 0))
  (bind _returnvalue_3 (Transformation|GetActorLocation))
  (bind _self self)
  (bind _falloffrange (Variables|Default|GetFallOffRange))
  (bind _returnvalue_4 (Transformation|GetActorLocation _returnvalue_2))
  (bind _returnvalue_5 (Math|Vector|Distance(Vector) _returnvalue_4 _returnvalue_3))
  ;[0.15 0.15 0.15 0.5] Attacking
  (AI|AIMoveTo self (Transformation|GetActorLocation (Game|GetPlayerCharacter 0)) 0 1.5e+03 false
    (:OnSuccess
      _)
    (:OnFail
      _))
  (Development|PrintString "Michael please  comment better")
  (if (Variables|Default|GetAttackCooldown)
    (CallFunction|Routine)
    (else
      (Transformation|SetActorRotation (Math|Rotator|FindLookatRotation (.location (Transformation|GetActorTransform)) (Transformation|GetActorLocation (Game|Player|GetPlayerPawn 0))))
      (if (>= _returnvalue_5 _falloffrange)
        ;[0.15 0.15 0.15 0.5] Adds accuracy fall off if enemy is far enough away
        (Game|SpawnActorfromClass "/Game/Enemies/BP_DemoEnemyAttack.BP_DemoEnemyAttack_C" (Math|Transform|MakeTransform (.location _returnvalue) (Math|Conversions|RotationFromXVector (+ (.rotation _returnvalue) (Math|Vector|MakeVector (Math|Float|Min(Float) (* (/ _returnvalue_5 _falloffrange) (Math|Random|RandomFloatinRange -0.05 0.05)) 0.2) 0.0 0.0))) "1.000000,1.000000,1.000000") "Undefined" "MultiplyWithRoot" 0 0)
        (else
          (Game|SpawnActorfromClass "/Game/Enemies/BP_DemoEnemyAttack.BP_DemoEnemyAttack_C" (Math|Transform|MakeTransform (.location _returnvalue) (.rotation _returnvalue) "1.000000,1.000000,1.000000") "Undefined" "MultiplyWithRoot" _self _self)))
      (Variables|Default|SetAttackCooldown true)
      (CallFunction|Routine)
      (Utilities|FlowControl|Delay 1.5)
      (Variables|Default|SetAttackCooldown false))))

(event Custom|Patrol
  ;[0.15 0.15 0.15 0.5] Patrol
  (Development|PrintString "CALLED PATROL")
  (AI|AIMoveTo self (.RandomLocation (AI|Navigation|GetRandomReachablePointinRadius (Transformation|GetActorLocation) (Math|Random|RandomFloatinRange 2e+02 1.2e+03) 0 0)) 0 5.0 false
    (:OnSuccess
      _)
    (:OnFail
      _))
  (CallFunction|Routine))

(event EventBeginPlay
  (CallFunction|Routine)
  (Development|PrintString "遊んでる今は"))

(fn ConstructionScript
  (|CallParentFunction))

(fn GetRowName
  (params (Class :type Actor%20Class%20Reference))
  (if (== Class "/Game/Weapons/MagicAttacks/BetaSpells/BP_BasicSpell.BP_BasicSpell_C")
    (return "BasicSpell")
    (elif (== Class "/Game/Weapons/MagicAttacks/BetaSpells/BP_RapidSpell.BP_RapidSpell_C")
      (return "RapidSpell")
      (elif (== Class "/Game/Weapons/MagicAttacks/BetaSpells/BP_ExplosiveSpell.BP_ExplosiveSpell_C")
        (return "ExplosiveSpell")))))