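; BP_ExtractZone is an extraction zone actor that shows an extraction timer while the player is inside it.
; Player overlap creates an ExtractTimerUI widget, hands it a reference to the zone and sets InExtract.
; Leaving resets and removes the widget and clears the flag.
; A separate Extract event, not called within this Blueprint, pauses the game and opens ExtractMenuUI.
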(event Custom|Extract
  ;[0.15 0.15 0.15 0.5] Extract menu
  (Game|SetGamePaused true)
  (bind _returnvalue (UserInterface|CreateWidget "/Game/UIWidgets/ExtractMenuUI.ExtractMenuUI_C"))
  (UserInterface|Viewport|AddtoViewport _returnvalue 0))

(event Collision|EventActorEndOverlap
  (params (OtherActor :type Actor%20Object%20Reference))
  ;[0.15 0.15 0.15 0.5] Is thing starting/ending overlap the player
  (if (== (Game|Player|GetPlayerPawn 0) OtherActor)
    (Default|ResetTimer (Variables|Default|GetTimer%20Widget))
    (Variables|Default|SetInExtract false)
    (Widget|RemovefromParent (Variables|Default|GetTimer%20Widget))))

(event Collision|EventActorBeginOverlap
  (params (OtherActor :type Actor%20Object%20Reference))
  ;[0.15 0.15 0.15 0.5] Is thing starting/ending overlap the player
  (if (== OtherActor (Game|Player|GetPlayerPawn 0))
    (bind _returnvalue (UserInterface|CreateWidget "/Game/UIWidgets/ExtractTimerUI.ExtractTimerUI_C" (Game|GetPlayerController 0)))
    (Variables|Default|SetInExtract true)
    (bind _output_get (Variables|Default|SetTimer%20Widget _returnvalue))
    (Variables|/Game/UIWidgets/ExtractTimerUI.ExtractTimerUI_C|SetExtractZone _returnvalue self)
    (UserInterface|Viewport|AddtoViewport _output_get 0)))

(fn ConstructionScript)