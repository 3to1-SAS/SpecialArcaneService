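; BP_ExtractCheck is an extraction zone trigger that pairs itself with a nearby BP_ExtractLocation and reacts to the first-person character.
; On BeginPlay it stores the last location found within Distance as ChoosenExtract; Distance is never updated, so this need not be the closest.
; On character overlap it loops over all locations and calls DestroyActor on itself, not on the location, for any that differs from ChoosenExtract.
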(event OnComponentBeginOverlap(CollisionComponent)
  (params (OverlappedComponent :type Primitive%20Component%20Object%20Reference) (OtherActor :type Actor%20Object%20Reference) (OtherComp :type Primitive%20Component%20Object%20Reference) (OtherBodyIndex :type Integer) (bFromSweep :type Boolean) (SweepResult :type Hit%20Result%20Structure%20%28by%20ref%29))
  (if (== (Utilities|GetClass OtherActor) "/Game/FirstPerson/Blueprints/BP_FirstPersonCharacter.BP_FirstPersonCharacter_C")
    (bind _outactors (Actor|GetAllActorsOfClass "/Game/ObjectiveSystem/ExtractZone/BP_ExtractLocation.BP_ExtractLocation_C"))
    (for _array_element _outactors
      (if (not (== _array_element (Variables|Default|GetChoosenExtract)))
        (Actor|DestroyActor)))))

(event EventBeginPlay
  ;[0.15 0.15 0.15 0.5] Find closest extract location spawner and save it's reference
  (bind _outactors (Actor|GetAllActorsOfClass "/Game/ObjectiveSystem/ExtractZone/BP_ExtractLocation.BP_ExtractLocation_C"))
  (for _array_element _outactors
    (if (< (Transformation|GetDistanceTo _array_element) (Variables|Default|GetDistance))
      (Variables|Default|SetChoosenExtract _array_element))))

(fn ConstructionScript)