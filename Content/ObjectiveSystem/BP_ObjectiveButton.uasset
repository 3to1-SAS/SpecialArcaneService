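; BP_ObjectiveButton is a one-use interactable button that accepts the objective and opens extraction.
; A box overlap shows or hides the first-person character's prompt and sets IsLookedAt, so proximity stands in for a gaze check.
; Pressing E in range flags the ObjectiveInstance, updates a TextRenderActor's text and spawns BP_ExtractZone at BP_ExtractLocation.
; It enables player input on itself and finds those world actors with GetActorOfClass.
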(event OnComponentBeginOverlap(Box)
  (params (OverlappedComponent :type Primitive%20Component%20Object%20Reference) (OtherActor :type Actor%20Object%20Reference) (OtherComp :type Primitive%20Component%20Object%20Reference) (OtherBodyIndex :type Integer) (bFromSweep :type Boolean) (SweepResult :type Hit%20Result%20Structure%20%28by%20ref%29))
  ;[0.15 0.15 0.15 0.5] Shows prompt when looked at
  (bind _asbp_first_person_character (Utilities|Casting|CastToBP_FirstPersonCharacter OtherActor))
  (Default|DisplayInteractivePrompt _asbp_first_person_character (Variables|Default|GetPromptText) true)
  (Variables|Default|SetIsLookedAt true)
  (Variables|Default|SetplayerLookingAt OtherActor))

(event OnComponentEndOverlap(Box)
  (params (OverlappedComponent :type Primitive%20Component%20Object%20Reference) (OtherActor :type Actor%20Object%20Reference) (OtherComp :type Primitive%20Component%20Object%20Reference) (OtherBodyIndex :type Integer))
  ;[0.15 0.15 0.15 0.5] Shows prompt when looked at
  (bind _asbp_first_person_character (Utilities|Casting|CastToBP_FirstPersonCharacter OtherActor))
  (Default|DisplayInteractivePrompt _asbp_first_person_character (Variables|Default|GetPromptText) false)
  (Variables|Default|SetIsLookedAt false)
  (Variables|Default|SetplayerLookingAt 0))

(event Input|EnhancedActionEvents|EnhancedInputActionIA_InteractWithE
  (params (ActionValue :type Boolean) (ElapsedSeconds :type Float%20%28double-precision%29) (TriggeredSeconds :type Float%20%28double-precision%29) (InputAction :type Input%20Action%20Object%20Reference :default "/Game/Input/Actions/IA_InteractWithE.IA_InteractWithE"))
  ;[0.15 0.15 0.15 0.5] When interacted with, sets objective and plays sound
  (if (!= (Variables|Default|GetPressed) true)
    ;;[0.15 0.15 0.15 0.5] Checks if the player's looking
    (Development|PrintString "pressed")
    (if (Variables|Default|GetIsLookedAt)
      (if (not (Variables|Default|GetPressed))
        (bind _returnvalue (Actor|GetActorOfClass "/Game/ObjectiveSystem/ObjectiveInstance.ObjectiveInstance_C"))
        (Variables|/Game/ObjectiveSystem/ObjectiveInstance.ObjectiveInstance_C|SetButtonPushed _returnvalue true)
        (bind _returnvalue_2 (Actor|GetActorOfClass "/Script/Engine.TextRenderActor"))
        (Rendering|Components|TextRender|SetText (Variables|/Script/Engine.TextRenderActor|GetTextRender _returnvalue_2) (Utilities|Text|MakeLiteralText "Objective Accepted"))
        (Variables|Default|SetPressed true)
        (bind _returnvalue_3 (Actor|GetActorOfClass "/Game/ObjectiveSystem/ExtractZone/BP_ExtractLocation.BP_ExtractLocation_C"))
        (Game|SpawnActorfromClass "/Game/ObjectiveSystem/ExtractZone/BP_ExtractZone.BP_ExtractZone_C" (Transformation|GetWorldTransform (Variables|/Script/Engine.Actor|GetRootComponent _returnvalue_3)) "AlwaysSpawn" "MultiplyWithRoot" 0 0)))))

(event EventBeginPlay
  (Input|EnableInput (Game|GetPlayerController 0)))

(fn ConstructionScript)