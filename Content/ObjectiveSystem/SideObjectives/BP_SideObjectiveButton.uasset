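; Interactable button that starts a room's wave-based enemy encounter when the player presses interact inside its overlap box, which also shows the prompt.
; Per-wave kill targets come from a data table row.
; NewWave replaces EnemySpawners matching the current wave and player's room with tagged, strength-scaled enemies.
; UpdateKills advances waves, then triggers the linked Spawn after the last (logged as shop opening), passing on the Final flag.
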(event OnComponentBeginOverlap(Box)
  (params (OverlappedComponent :type Primitive%20Component%20Object%20Reference) (OtherActor :type Actor%20Object%20Reference) (OtherComp :type Primitive%20Component%20Object%20Reference) (OtherBodyIndex :type Integer) (bFromSweep :type Boolean) (SweepResult :type Hit%20Result%20Structure%20%28by%20ref%29))
  ;[0.15 0.15 0.15 0.5] Shows prompt when looked at
  (bind _asbp_first_person_character (Utilities|Casting|CastToBP_FirstPersonCharacter OtherActor))
  (Default|DisplayInteractivePrompt _asbp_first_person_character (Variables|Default|GetPromptText) true)
  (Variables|Default|SetIsLookedAt true)
  (Variables|Default|SetplayerLookingAt OtherActor))

(event OnComponentEndOverlap(Box)
  (params (OverlappedComponent :type Primitive%20Component%20Object%20Reference) (OtherActor :type Actor%20Object%20Reference) (OtherComp :type Primitive%20Component%20Object%20Reference) (OtherBodyIndex :type Integer))
  ;[0.15 0.15 0.15 0.5] Shows prompt when looked at
  (bind _asbp_first_person_character (Utilities|Casting|CastToBP_FirstPersonCharacter OtherActor))
  (Default|DisplayInteractivePrompt _asbp_first_person_character (Variables|Default|GetPromptText) false)
  (Variables|Default|SetIsLookedAt false)
  (Variables|Default|SetplayerLookingAt 0))

(event Custom|NewWave
  ;[0.15 0.15 0.15 0.5] Find every enemy spawner that applies to where the player is
  (Development|PrintString "New Wave")
  (bind _outactors (Actor|GetAllActorsOfClass "/Game/ObjectiveSystem/SideObjectives/EnemySpawner.EnemySpawner_C"))
  (for _array_element _outactors
    (if (== (Variables|/Game/ObjectiveSystem/SideObjectives/EnemySpawner.EnemySpawner_C|GetWave _array_element) (Variables|Default|GetCurrentWave))
      (if (== (Variables|/Game/FirstPerson/Blueprints/BP_FirstPersonCharacter.BP_FirstPersonCharacter_C|GetCurrentRoom (Variables|Default|GetPlayerCharacter)) (Variables|/Game/ObjectiveSystem/SideObjectives/EnemySpawner.EnemySpawner_C|GetRoomName _array_element))
        ;[0.15 0.15 0.15 0.5] Spawn according enemy and tag it as a wave enemy
        (switch Utilities|FlowControl|Switch|SwitchonEnemyTypeEnum (Variables|/Game/ObjectiveSystem/SideObjectives/EnemySpawner.EnemySpawner_C|GetEnemyToSpawn _array_element)
          (:NewEnumerator0
            (bind _returnvalue (Game|SpawnActorfromClass "/Game/Enemies/Arcane/BP_Arcane.BP_Arcane_C" (Transformation|GetActorTransform _array_element) "AdjustIfPossibleButAlwaysSpawn" "MultiplyWithRoot" 0 0))
            (Utilities|Array|Add (Variables|/Script/Engine.Actor|GetTags _returnvalue) "WaveEnemy")
            (Variables|/Game/Enemies/Arcane/BP_Arcane.BP_Arcane_C|SetStrengthMultiplier _returnvalue (Variables|/Game/ObjectiveSystem/SideObjectives/EnemySpawner.EnemySpawner_C|GetStrengthMultiplier _array_element)))
          (:NewEnumerator1
            (bind _returnvalue_2 (Game|SpawnActorfromClass "/Game/Enemies/Knight/BP_Knight.BP_Knight_C" (Transformation|GetActorTransform _array_element) "AdjustIfPossibleButAlwaysSpawn" "MultiplyWithRoot" 0 0))
            (Utilities|Array|Add (Variables|/Script/Engine.Actor|GetTags _returnvalue_2) "WaveEnemy")
            (Variables|/Game/Enemies/Knight/BP_Knight.BP_Knight_C|SetStrengthMultiplier _returnvalue_2 (Variables|/Game/ObjectiveSystem/SideObjectives/EnemySpawner.EnemySpawner_C|GetStrengthMultiplier _array_element)))
          (:NewEnumerator2
            (bind _returnvalue_3 (Game|SpawnActorfromClass "/Game/Enemies/Protector/BP_Protector.BP_Protector_C" (Transformation|GetActorTransform _array_element) "AdjustIfPossibleButAlwaysSpawn" "MultiplyWithRoot" 0 0))
            (Utilities|Array|Add (Variables|/Script/Engine.Actor|GetTags _returnvalue_3) "WaveEnemy")
            (Variables|/Game/Enemies/Protector/BP_Protector.BP_Protector_C|SetStrengthMultiplier _returnvalue_3 (Variables|/Game/ObjectiveSystem/SideObjectives/EnemySpawner.EnemySpawner_C|GetStrengthMultiplier _array_element)))
          (:NewEnumerator4
            (bind _returnvalue_4 (Game|SpawnActorfromClass "/Game/Enemies/Tank/BP_Tank.BP_Tank_C" (Transformation|GetActorTransform _array_element) "AdjustIfPossibleButAlwaysSpawn" "MultiplyWithRoot" 0 0))
            (Utilities|Array|Add (Variables|/Script/Engine.Actor|GetTags _returnvalue_4) "WaveEnemy")
            (Variables|/Game/Enemies/Tank/BP_Tank.BP_Tank_C|SetStrengthMultiplier _returnvalue_4 (Variables|/Game/ObjectiveSystem/SideObjectives/EnemySpawner.EnemySpawner_C|GetStrengthMultiplier _array_element))))
        (Actor|DestroyActor _array_element)
        (else
          (Development|PrintString "Wrong Room")))
      (else
        (Development|PrintString "Wrong Wave")))))

(event Custom|UpdateKills
  (bind _spawn (Variables|Default|GetSpawn))
  (if (== (+ (Variables|Default|GetEnemiesKilled) 1) (Utilities|Array|Get(acopy) (Variables|Default|GetEnemy%20Amount) (Variables|Default|GetCurrentWave)))
    (Variables|Default|SetEnemiesKilled 0)
    (if (== (+ (Variables|Default|GetCurrentWave) 1) (Utilities|Array|Length (Variables|Default|GetEnemy%20Amount)))
      (Development|PrintString "Shop Open" true true "(R=1.000000,G=0.647218,B=0.000000,A=1.000000)")
      (Default|Spawn _spawn)
      (if (Variables|Default|GetFinal)
        (Variables|/Game/Shop/Fixed/Portal.Portal_C|SetFinal (Variables|/Game/Shop/Fixed/Portal.Portal_C|GetLinked (Variables|/Game/Shop/Fixed/IEGCPortalSpawn.IEGCPortalSpawn_C|GetSpawned _spawn)) true))
      (else
        (Variables|Default|SetCurrentWave (+ (Variables|Default|GetCurrentWave) 1))
        (CallFunction|NewWave)))
    (else
      (Variables|Default|SetEnemiesKilled (+ (Variables|Default|GetEnemiesKilled) 1)))))

(event Input|EnhancedActionEvents|EnhancedInputActionIA_InteractWithE
  (params (ActionValue :type Boolean) (ElapsedSeconds :type Float%20%28double-precision%29) (TriggeredSeconds :type Float%20%28double-precision%29) (InputAction :type Input%20Action%20Object%20Reference :default "/Game/Input/Actions/IA_InteractWithE.IA_InteractWithE"))
  (:Started
    ;[0.15 0.15 0.15 0.5] When interacted with, sets objective and plays sound
    (if (!= (Variables|Default|GetPressed) true)
      ;;[0.15 0.15 0.15 0.5] Checks if the player's looking
      (Development|PrintString "pressed")
      (if (Variables|Default|GetIsLookedAt)
        (if (not (Variables|Default|GetPressed))
          (CallFunction|NewWave)
          (Variables|Default|SetPressed true))))))

(event EventBeginPlay
  ;[0.15 0.15 0.15 0.5] Reference Getting
  (Input|EnableInput (Game|GetPlayerController 0))
  (bind _asbp_first_person_character (Utilities|Casting|CastToBP_FirstPersonCharacter (Game|Player|GetPlayerPawn 0)))
  (Variables|Default|SetPlayerCharacter _asbp_first_person_character)
  (bind _returnvalue (Utilities|GetDataTableRow "/Game/ObjectiveSystem/SideObjectives/WaveDataTables/UnifiedEncountersTable.UnifiedEncountersTable" (Variables|Default|GetRoom))
    (:then
      (bind _output_get (Variables|Default|SetEnemy%20Amount (Utilities|Struct|BreakWaveStruct _returnvalue)))
      (for _array_element _output_get
        (Development|PrintString (Utilities|String|ToString(Integer) _array_element))))))

(fn ConstructionScript)