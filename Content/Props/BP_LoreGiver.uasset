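; BP_LoreGiver is an interactable prop that shows the first-person character a prompt when they come near.
; Its Box overlap events toggle that prompt, set IsLookedAt and track PlayerLookingAt, so "looked at" means inside the box rather than traced.
; The actor enables player 0 input on BeginPlay to receive IA_InteractWithE directly.
; That handler only prints a debug string; its commented objective and sound logic is absent.
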(event OnComponentBeginOverlap(Box)
  (params (OverlappedComponent :type Primitive%20Component%20Object%20Reference) (OtherActor :type Actor%20Object%20Reference) (OtherComp :type Primitive%20Component%20Object%20Reference) (OtherBodyIndex :type Integer) (bFromSweep :type Boolean) (SweepResult :type Hit%20Result%20Structure%20%28by%20ref%29))
  ;[0.15 0.15 0.15 0.5] Shows prompt when looked at
  (bind _asbp_first_person_character (Utilities|Casting|CastToBP_FirstPersonCharacter OtherActor))
  (Default|DisplayInteractivePrompt _asbp_first_person_character (Variables|Default|GetPromptText) true)
  (Variables|Default|SetIsLookedAt true)
  (Variables|Default|SetplayerLookingAt OtherActor))

(event OnComponentEndOverlap(Box)
  (params (OverlappedComponent :type Primitive%20Component%20Object%20Reference) (OtherActor :type Actor%20Object%20Reference) (OtherComp :type Primitive%20Component%20Object%20Reference) (OtherBodyIndex :type Integer))
  ;[0.15 0.15 0.15 0.5] Shows prompt when looked at
  (bind _asbp_first_person_character (Utilities|Casting|CastToBP_FirstPersonCharacter OtherActor))
  (Default|DisplayInteractivePrompt _asbp_first_person_character (Variables|Default|GetPromptText) false)
  (Variables|Default|SetIsLookedAt false)
  (Variables|Default|SetplayerLookingAt 0))

(event Input|EnhancedActionEvents|EnhancedInputActionIA_InteractWithE
  (params (ActionValue :type Boolean) (ElapsedSeconds :type Float%20%28double-precision%29) (TriggeredSeconds :type Float%20%28double-precision%29) (InputAction :type Input%20Action%20Object%20Reference :default "/Game/Input/Actions/IA_InteractWithE.IA_InteractWithE"))
  ;[0.15 0.15 0.15 0.5] When interacted with, sets objective and plays sound
  (if (!= (Variables|Default|GetPressed) true)
    ;;[0.15 0.15 0.15 0.5] Checks if the player's looking
    (Development|PrintString "pressed")
    (if (Variables|Default|GetIsLookedAt)
      (if (Variables|Default|GetPressed)
        _))))

(event EventBeginPlay
  (Input|EnableInput (Game|GetPlayerController 0)))

(fn ConstructionScript)