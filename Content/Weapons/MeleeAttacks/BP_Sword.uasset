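; BP_Sword is a first-person melee weapon that snaps to the player's WeaponGoesHere socket component with collision off.
; Attack enables collision, moves it to WeaponAttackHere, and plays a placeholder timeline swing downward.
; On finish it returns to hand and clears the player's Cooldown, leaving collision on.
; Overlapping a BP_DemoEnemy subtracts Damage from the HP of the GetActorOfClass result, not necessarily the overlapped enemy.
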(event Custom|Attack
  ;[0.15 0.15 0.15 0.5] When attacking the sword will set it's collision on and move infront of the player's camera (Temp before animations)
  (Collision|SetActorEnableCollision true)
  (bind _returnvalue (Actor|GetActorOfClass "/Game/FirstPerson/Blueprints/BP_FirstPersonCharacter.BP_FirstPersonCharacter_C"))
  (Transformation|AttachComponentToComponent (Variables|/Game/FirstPerson/Blueprints/BP_FirstPersonCharacter.BP_FirstPersonCharacter_C|GetWeaponAttackHere _returnvalue) "None" "SnapToTarget" "SnapToTarget" "SnapToTarget" true)
  ;[0.15 0.15 0.15 0.5] Move sword up and down infront of the camera (Temp before animations
  (bind _swordmovement (Timeline|AttackMovementPlaceholder PlayFromStart)
    (:Update
      (bind _returnvalue_2 (Actor|GetActorOfClass "/Game/FirstPerson/Blueprints/BP_FirstPersonCharacter.BP_FirstPersonCharacter_C"))
      (Variables|Default|SetAttackStartLocation (Transformation|GetWorldLocation (Variables|/Game/FirstPerson/Blueprints/BP_FirstPersonCharacter.BP_FirstPersonCharacter_C|GetWeaponAttackHere _returnvalue_2)))
      (Variables|Default|SetAttackEndLocation (- (Transformation|GetWorldLocation (Variables|/Game/FirstPerson/Blueprints/BP_FirstPersonCharacter.BP_FirstPersonCharacter_C|GetWeaponAttackHere _returnvalue_2)) "0.000000,0.000000,60.000000"))
      (Transformation|SetActorLocation (Math|Vector|Lerp(Vector) (Variables|Default|GetAttackStartLocation) (Variables|Default|GetAttackEndLocation) _swordmovement) true false))
    (:Finished
      ;;[0.15 0.15 0.15 0.5] Once the temp animation is done, go back in player's hand
      (bind _returnvalue_3 (Actor|GetActorOfClass "/Game/FirstPerson/Blueprints/BP_FirstPersonCharacter.BP_FirstPersonCharacter_C"))
      (Transformation|AttachComponentToComponent (Variables|/Game/FirstPerson/Blueprints/BP_FirstPersonCharacter.BP_FirstPersonCharacter_C|GetWeaponGoesHere _returnvalue_3) "None" "SnapToTarget" "SnapToTarget" "SnapToTarget" true)
      (Variables|/Game/FirstPerson/Blueprints/BP_FirstPersonCharacter.BP_FirstPersonCharacter_C|SetCooldown _returnvalue_3 false))))

(event Collision|EventActorBeginOverlap
  (params (OtherActor :type Actor%20Object%20Reference))
  ;[0.15 0.15 0.15 0.5] Overlap with enemy and deal damage to it
  (if (== (Utilities|GetClass OtherActor) "/Game/Enemies/BP_DemoEnemy.BP_DemoEnemy_C")
    (bind _returnvalue (Actor|GetActorOfClass "/Game/Enemies/BP_DemoEnemy.BP_DemoEnemy_C"))
    (Variables|/Game/Enemies/BP_DemoEnemy.BP_DemoEnemy_C|SetHP _returnvalue (- (Variables|/Game/Enemies/BP_DemoEnemy.BP_DemoEnemy_C|GetHP _returnvalue) (Variables|Default|GetDamage)))))

(event EventBeginPlay
  ;[0.15 0.15 0.15 0.5] When the Sword exists it will go into the player's hand (set no collision)
  (bind _returnvalue (Actor|GetActorOfClass "/Game/FirstPerson/Blueprints/BP_FirstPersonCharacter.BP_FirstPersonCharacter_C"))
  (Transformation|AttachComponentToComponent (Variables|/Game/FirstPerson/Blueprints/BP_FirstPersonCharacter.BP_FirstPersonCharacter_C|GetWeaponGoesHere _returnvalue) "None" "SnapToTarget" "SnapToTarget" "SnapToTarget" true)
  (Collision|SetActorEnableCollision false))

(fn ConstructionScript)