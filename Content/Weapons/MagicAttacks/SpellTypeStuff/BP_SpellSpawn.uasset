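; BP_SpellSpawn is a spell spawn indicator that shows whether its current location is a valid placement.
; On BeginPlay it gives its cylinder a dynamic material and starts a fast looping timer that runs CheckValidity.
; CheckValidity sets CanPlace if the cylinder overlaps an actor tagged as floor or enemy, falling back to floor-tagged components, then tints the material green or red to match.
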(event EventBeginPlay
  ;[0.15 0.15 0.15 0.5] Material instance for material & starts check function
  (bind _returnvalue (Rendering|Material|CreateDynamicMaterialInstance (Variables|Default|GetCylinder) 0 "/Game/Weapons/MagicAttacks/SpellTypeStuff/M_SpellSpawn.M_SpellSpawn" "None" :!class /Script/Engine.PrimitiveComponent))
  (Variables|Default|SetMateral _returnvalue)
  (Utilities|Time|SetTimerbyFunctionName 0 "CheckValidity" 0.022 true true))

(fn ConstructionScript)

(fn CheckValidity
  (bind _cylinder (Variables|Default|GetCylinder))
  (bind _materal (Variables|Default|GetMateral))
  ;[0.15 0.15 0.15 0.5] Checks the current overlapping actors, and if one of them is the floor or an enemy it sets can place to true
  (bind _array_element (Utilities|Array|ForEachLoopwithBreak (Collision|GetOverlappingActors _cylinder 0 :!class /Script/Engine.PrimitiveComponent) :!label _label)
    (:LoopBody
      (if (or (Actor|ActorHasTag _array_element "IsFloor") (Actor|ActorHasTag _array_element "Enemy"))
        (Variables|Default|SetCanPlace true)
        (goto _label Break)
        (else
          (Variables|Default|SetCanPlace false))))
    (:Completed
      (if (Variables|Default|GetCanPlace)
        ;[0.15 0.15 0.15 0.5] Sets the color based on the value of canplace
        (if (Variables|Default|GetCanPlace) :!label _label_2
          (Rendering|Material|SetVectorParameterValue _materal "Color" "(R=0.014859,G=1.000000,B=0.000000,A=1.000000)" :!class /Script/Engine.MaterialInstanceDynamic)
          (else
            (Rendering|Material|SetVectorParameterValue _materal "Color" "(R=1.000000,G=0.000000,B=0.000212,A=1.000000)" :!class /Script/Engine.MaterialInstanceDynamic)))
        (else
          (bind _array_element_2 (Utilities|Array|ForEachLoopwithBreak (Class|PrimitiveComponent|GetOverlappingComponents _cylinder) :!label _label_3)
            (:LoopBody
              (if (Components|ComponentHasTag _array_element_2 "IsFloor")
                (Variables|Default|SetCanPlace true)
                (goto _label_3 Break)
                (else
                  (Variables|Default|SetCanPlace false))))
            (:Completed
              (goto _label_2))))))))