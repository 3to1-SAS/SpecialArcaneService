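; Spell-firing Blueprint that casts the player's equipped spell when selected, off cooldown and with non-negative mana.
; BasicSpellShoot reads the SpellsData row and dispatches on SpellType to Single, randomly spread Burst, triple-spawn Beam or wand-attached, zero-scale Charge functions.
; Each function spawns the spell and deducts its mana cost.
; Afterwards, every BP_Enemy is notified, and a FireRate delay re-enables firing and clears the character's cooldown.
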(event Custom|BasicSpellShoot
  (bind _returnvalue (Game|Player|GetPlayerPawn 0))
  (bind _returnvalue_2 (Pawn|GetBaseAimRotation _returnvalue))
  ;[0.15 0.15 0.15 0.5] Checks if spell is on cooldown and player has enough mana
  ;;[0.15 0.15 0.15 0.5] Check if spell is selected
  (if (Variables|Default|GetSelected)
    (bind _returnvalue_3 (Actor|GetActorOfClass "/Game/Weapons/MagicAttacks/BP_BasicWand.BP_BasicWand_C"))
    (Variables|Default|SetWand _returnvalue_3)
    (bind _returnvalue_4 (Actor|GetActorOfClass "/Game/FirstPerson/Blueprints/BP_FirstPersonPlayerController.BP_FirstPersonPlayerController_C"))
    (bind _returnvalue_5 (Utilities|GetDataTableRow (Variables|Default|GetSpellsData) (Variables|/Game/FirstPerson/Blueprints/BP_FirstPersonPlayerController.BP_FirstPersonPlayerController_C|GetEquippedSpell _returnvalue_4))
      (:then
        (if (and (Variables|Default|GetIsFireable) (>= (Variables|/Game/FirstPerson/Blueprints/BP_FirstPersonPlayerController.BP_FirstPersonPlayerController_C|GetMana _returnvalue_4) 0.0))
          (Variables|Default|SetSpell (.Spell (Utilities|Struct|BreakSpellStructure _returnvalue_5)))
          (Variables|Default|SetConsumption (.ManaConsumption (Utilities|Struct|BreakSpellStructure _returnvalue_5)))
          (Variables|Default|SetSpellRotation _returnvalue_2)
          ;[0.15 0.15 0.15 0.5] Calls the corresponding function based on the spell's type.
          (Variables|Default|SetSpellLocation (+ (.OutLocation (Actor|GetActorEyesViewPoint _returnvalue)) (* (Math|Vector|GetForwardVector _returnvalue_2) "50.000000,0.000000,0.000000")))
          (if (Utilities|Enum|Equal(Enum) (.SpellType (Utilities|Struct|BreakSpellStructure _returnvalue_5)) "Single")
            (CallFunction|SpawnSingleShot)
            ;[0.15 0.15 0.15 0.5] Calls the function for enemies to detect spells
            (bind _outactors (Actor|GetAllActorsOfClass "/Game/NPC_Comp/BP_Enemy.BP_Enemy_C" :!label _label))
            (for _array_element _outactors
              (Default|SpellDetected _array_element (Components|GetOwner)))
            (Utilities|FlowControl|Delay (.FireRate (Utilities|Struct|BreakSpellStructure _returnvalue_5)))
            (Variables|Default|SetIsFireable true)
            (bind _returnvalue_6 (Actor|GetActorOfClass "/Game/FirstPerson/Blueprints/BP_FirstPersonCharacter.BP_FirstPersonCharacter_C"))
            (Variables|/Game/FirstPerson/Blueprints/BP_FirstPersonCharacter.BP_FirstPersonCharacter_C|SetCooldown _returnvalue_6 false)
            (elif (Utilities|Enum|Equal(Enum) (.SpellType (Utilities|Struct|BreakSpellStructure _returnvalue_5)) "Burst")
              (CallFunction|SpawnBurstShot)
              (goto _label)
              (elif (Utilities|Enum|Equal(Enum) (.SpellType (Utilities|Struct|BreakSpellStructure _returnvalue_5)) "Beam")
                (CallFunction|SpawnBeamShot)
                (goto _label)
                (elif (Utilities|Enum|Equal(Enum) (.SpellType (Utilities|Struct|BreakSpellStructure _returnvalue_5)) "Charge")
                  (CallFunction|SpawnChargeShot)
                  (goto _label)))))
          (elif (not (>= (Variables|/Game/FirstPerson/Blueprints/BP_FirstPersonPlayerController.BP_FirstPersonPlayerController_C|GetMana _returnvalue_4) 0.0))
            (Utilities|FlowControl|Delay 0.2)
            (bind _returnvalue_7 (Actor|GetActorOfClass "/Game/FirstPerson/Blueprints/BP_FirstPersonCharacter.BP_FirstPersonCharacter_C"))
            (Variables|/Game/FirstPerson/Blueprints/BP_FirstPersonCharacter.BP_FirstPersonCharacter_C|SetCooldown _returnvalue_7 false)
            (Development|PrintString "Cancelled cooldown")))))))

(fn SpawnSingleShot
  (Game|SpawnActorfromClass (Variables|Default|GetSpell) (Math|Transform|MakeTransform (Variables|Default|GetSpellLocation) (Variables|Default|GetSpellRotation) "1.000000,1.000000,1.000000") "Undefined" "MultiplyWithRoot" 0 0)
  (Default|PlayAnimation (Variables|Default|GetWand))
  (Development|PrintString "spell spawned")
  (Variables|Default|SetIsFireable false)
  (bind _returnvalue (Actor|GetActorOfClass "/Game/FirstPerson/Blueprints/BP_FirstPersonPlayerController.BP_FirstPersonPlayerController_C"))
  (Variables|/Game/FirstPerson/Blueprints/BP_FirstPersonPlayerController.BP_FirstPersonPlayerController_C|SetMana _returnvalue (- (Variables|/Game/FirstPerson/Blueprints/BP_FirstPersonPlayerController.BP_FirstPersonPlayerController_C|GetMana _returnvalue) (Variables|Default|GetConsumption))))

(fn SpawnBurstShot
  (bind _spellrotation (Variables|Default|GetSpellRotation))
  (bind (_roll _pitch _yaw) (Math|Rotator|BreakRotator _spellrotation))
  (Variables|Default|SetBurstAmount (Math|Random|RandomIntegerinRange 15 22))
  ;[0.15 0.15 0.15 0.5] Spawns a random amount of the actors oh yeahhhhh
  (Game|SpawnActorfromClass (Variables|Default|GetSpell) (Math|Transform|MakeTransform (Variables|Default|GetSpellLocation) (Math|Rotator|MakeRotator _roll (+ _pitch (Math|Random|RandomFloatinRange -2.5 2.5)) (+ _yaw (Math|Random|RandomFloatinRange -2.5 2.5))) "1.000000,1.000000,1.000000") "Undefined" "MultiplyWithRoot" 0 0 :!label _label)
  (bind _output_get (Variables|Default|SetCurrentBurst (+ (Variables|Default|GetCurrentBurst) 1)))
  (if (>= _output_get (Variables|Default|GetBurstAmount))
    (Variables|Default|SetCurrentBurst 0)
    (Default|PlayAnimation (Variables|Default|GetWand))
    (Development|PrintString "spawned burst")
    (Variables|Default|SetIsFireable false)
    (bind _returnvalue (Actor|GetActorOfClass "/Game/FirstPerson/Blueprints/BP_FirstPersonPlayerController.BP_FirstPersonPlayerController_C"))
    (Variables|/Game/FirstPerson/Blueprints/BP_FirstPersonPlayerController.BP_FirstPersonPlayerController_C|SetMana _returnvalue (- (Variables|/Game/FirstPerson/Blueprints/BP_FirstPersonPlayerController.BP_FirstPersonPlayerController_C|GetMana _returnvalue) (Variables|Default|GetConsumption)))
    (else
      (Development|PrintString "Spell Spanwed")
      (goto _label))))

(fn SpawnBeamShot
  (Variables|Default|SetBurstAmount 3)
  (Game|SpawnActorfromClass (Variables|Default|GetSpell) (Math|Transform|MakeTransform (Variables|Default|GetSpellLocation) (Variables|Default|GetSpellRotation) "1.000000,1.000000,1.000000") "Undefined" "MultiplyWithRoot" 0 0 :!label _label)
  (bind _output_get (Variables|Default|SetCurrentBurst (+ 1 (Variables|Default|GetCurrentBurst))))
  (if (>= _output_get (Variables|Default|GetBurstAmount))
    (Variables|Default|SetCurrentBurst 0)
    (Default|PlayAnimation (Variables|Default|GetWand))
    (Development|PrintString "spell spawned")
    (Variables|Default|SetIsFireable false)
    (bind _returnvalue (Actor|GetActorOfClass "/Game/FirstPerson/Blueprints/BP_FirstPersonPlayerController.BP_FirstPersonPlayerController_C"))
    (Variables|/Game/FirstPerson/Blueprints/BP_FirstPersonPlayerController.BP_FirstPersonPlayerController_C|SetMana _returnvalue (- (Variables|/Game/FirstPerson/Blueprints/BP_FirstPersonPlayerController.BP_FirstPersonPlayerController_C|GetMana _returnvalue) (Variables|Default|GetConsumption)))
    (else
      (goto _label))))

(fn SpawnChargeShot
  (bind _returnvalue (Game|SpawnActorfromClass (Variables|Default|GetSpell) (Math|Transform|MakeTransform (Variables|Default|GetSpellLocation) (Variables|Default|GetSpellRotation) "0.000000,0.000000,0.000000") "Undefined" "MultiplyWithRoot" 0 0))
  (Transformation|AttachComponentToComponent _returnvalue (Variables|/Game/Weapons/MagicAttacks/BP_BasicWand.BP_BasicWand_C|GetChargeLocation (Variables|Default|GetWand)) "None" "SnapToTarget" "KeepWorld" "KeepWorld" true)
  (Variables|Default|SetIsFireable false)
  (bind _returnvalue_2 (Actor|GetActorOfClass "/Game/FirstPerson/Blueprints/BP_FirstPersonPlayerController.BP_FirstPersonPlayerController_C"))
  (Variables|/Game/FirstPerson/Blueprints/BP_FirstPersonPlayerController.BP_FirstPersonPlayerController_C|SetMana _returnvalue_2 (- (Variables|/Game/FirstPerson/Blueprints/BP_FirstPersonPlayerController.BP_FirstPersonPlayerController_C|GetMana _returnvalue_2) (Variables|Default|GetConsumption))))