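; BP_BasicWand is the player's wand actor, providing the visual feedback for casting a spell.
; On BeginPlay it snaps to the first-person character's WandGoesHere component, disables its collision and stores that component's starting roll.
; PlayAnimation activates the NSCastSpell effect and runs a timeline that offsets the roll of WandGoesHere, so the mount point moves rather than the wand itself.
; The timeline's finish only prints a debug string.
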(event Custom|PlayAnimation
  (Components|Activation|Activate (Variables|Default|GetNS_CastSpell) true)
  (bind _newtrack_0 (Timeline|FunnyTimeline PlayFromStart)
    (:Update
      (Transformation|SetRelativeRotation (Variables|/Game/FirstPerson/Blueprints/BP_FirstPersonCharacter.BP_FirstPersonCharacter_C|GetWandGoesHere (stale EventBeginPlay _output_get)) (Math|Rotator|MakeRotator (+ (* _newtrack_0 25.0) (Variables|Default|GetRotation)) (.pitch (Variables|/Script/Engine.SceneComponent|GetRelativeRotation (Variables|/Game/FirstPerson/Blueprints/BP_FirstPersonCharacter.BP_FirstPersonCharacter_C|GetWandGoesHere (stale EventBeginPlay _output_get)))) (.yaw (Variables|/Script/Engine.SceneComponent|GetRelativeRotation (Variables|/Game/FirstPerson/Blueprints/BP_FirstPersonCharacter.BP_FirstPersonCharacter_C|GetWandGoesHere (stale EventBeginPlay _output_get))))) false false))
    (:Finished
      (Development|PrintString "screem"))))

(event EventBeginPlay
  (bind _asbp_first_person_character (Utilities|Casting|CastToBP_FirstPersonCharacter (Game|Player|GetPlayerPawn 0)))
  (bind _output_get (Variables|Default|SetFirst%20Person%20Character _asbp_first_person_character))
  (Transformation|AttachComponentToComponent (Variables|/Game/FirstPerson/Blueprints/BP_FirstPersonCharacter.BP_FirstPersonCharacter_C|GetWandGoesHere _output_get) "None" "SnapToTarget" "SnapToTarget" "SnapToTarget" true)
  (Collision|SetActorEnableCollision false)
  (Variables|Default|SetRotation (.roll (Variables|/Script/Engine.SceneComponent|GetRelativeRotation (Variables|/Game/FirstPerson/Blueprints/BP_FirstPersonCharacter.BP_FirstPersonCharacter_C|GetWandGoesHere _output_get)))))

(fn ConstructionScript)