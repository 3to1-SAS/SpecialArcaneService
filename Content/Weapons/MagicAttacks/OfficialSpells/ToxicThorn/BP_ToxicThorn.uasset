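; BP_ToxicThorn is a charge-up spell projectile that reads its stats from DT_Spells on spawn.
; A Charge timeline tracks charge percent until the attack input is released, which scales damage, detaches the thorn, launches it and starts the caster's cooldown.
; Once fired, overlapping anything except the caster or NonBlocking-tagged actors spawns an explosion and destroys it, with EndPlay reusing that path.
; Damage and Impulse are stored but not applied here.
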(event OnComponentBeginOverlap(hitbox)
  (params (OverlappedComponent :type Primitive%20Component%20Object%20Reference) (OtherActor :type Actor%20Object%20Reference) (OtherComp :type Primitive%20Component%20Object%20Reference) (OtherBodyIndex :type Integer) (bFromSweep :type Boolean) (SweepResult :type Hit%20Result%20Structure%20%28by%20ref%29))
  (bind _returnvalue (Transformation|GetActorTransform))
  ;[0.15 0.15 0.15 0.5] Destroys spell on collision or after set lifetime
  (if (not (== OtherActor (Variables|Default|GetPlayerCharacter)))
    (if (not (Actor|ActorHasTag OtherActor "NonBlocking"))
      (if (Variables|Default|GetHasCharged)
        (Niagara|SpawnSystematLocation "/Game/Weapons/MagicAttacks/OfficialSpells/MagicMissile/NS_MissileExplosion.NS_MissileExplosion" (.location _returnvalue) (.rotation _returnvalue))
        (Utilities|FlowControl|Delay 0.025)
        (Actor|DestroyActor)))))

(event Input|EnhancedActionEvents|EnhancedInputActionIA_Attack
  (params (ActionValue :type Boolean) (ElapsedSeconds :type Float%20%28double-precision%29) (TriggeredSeconds :type Float%20%28double-precision%29) (InputAction :type Input%20Action%20Object%20Reference :default "/Game/Input/Actions/IA_Attack.IA_Attack"))
  (bind _projectilemovement (Variables|Default|GetProjectileMovement))
  ;[0.15 0.15 0.15 0.5] Checks when LMB is released, scaling damage accordingly
  (:Completed
    (if (not (Variables|Default|GetHasCharged))
      (Audio|Components|Audio|Stop (Variables|Default|GetCharge))
      (Variables|Default|SetDamage (* (Variables|Default|GetDamage) (Variables|Default|GetChargePercent)))
      ;[0.15 0.15 0.15 0.5] Activates velocity and stuff
      (Variables|Default|SetHasCharged true)
      (Transformation|DetachFromActor "KeepWorld" "KeepWorld" "KeepWorld")
      (Transformation|SetActorLocation (Transformation|GetWorldLocation (Variables|/Game/FirstPerson/Blueprints/BP_FirstPersonCharacter.BP_FirstPersonCharacter_C|GetSpellSpawnHere (Variables|Default|GetPlayerCharacter))) false false)
      (Variables|/Script/Engine.MovementComponent|SetVelocity _projectilemovement (* (Class|MovementComponent|GetMaxSpeed _projectilemovement) (Math|Vector|GetForwardVector (Variables|Default|GetDirection))))
      (Components|Activation|Activate _projectilemovement false)
      (Default|Cooldown (Variables|/Game/FirstPerson/Blueprints/BP_FirstPersonCharacter.BP_FirstPersonCharacter_C|GetBP_SpellFiring (Variables|Default|GetPlayerCharacter)) "ToxicThorn")
      (Variables|/Script/Engine.PrimitiveComponent|SetbGenerateOverlapEvents (Variables|Default|Gethitbox) true))))

(event EventEndPlay
  (params (EndPlayReason :type EEndPlayReason%20Enum :default "Destroyed"))
  (bind _returnvalue (Transformation|GetActorTransform))
  ;[0.15 0.15 0.15 0.5] Destroys spell on collision or after set lifetime
  (Niagara|SpawnSystematLocation "/Game/Weapons/MagicAttacks/OfficialSpells/MagicMissile/NS_MissileExplosion.NS_MissileExplosion" (.location _returnvalue) (.rotation _returnvalue))
  (Utilities|FlowControl|Delay 0.025)
  (Actor|DestroyActor))

(event EventBeginPlay
  (bind _projectilemovement (Variables|Default|GetProjectileMovement))
  ;[0.15 0.15 0.15 0.5] Initialize the projectile (set its values based on the data table)
  (Transformation|SetActorScale3D "0.200000,0.100000,0.100000")
  (bind _asbp_first_person_character (Utilities|Casting|CastToBP_FirstPersonCharacter (Game|GetInstigator))
    (:then
      (Variables|Default|SetPlayerCharacter _asbp_first_person_character)
      (bind _returnvalue (Utilities|GetDataTableRow "/Game/DataTables/Spells/DT_Spells.DT_Spells" (Variables|Default|GetDataTableName))
        (:then
          (Variables|Default|SetDamage (.spelldamage _returnvalue))
          (Actor|SetLifeSpan (.lifetime _returnvalue))
          (Variables|/Script/Engine.ProjectileMovementComponent|SetMaxSpeed _projectilemovement (.travelspeed _returnvalue))
          (Variables|/Script/Engine.ProjectileMovementComponent|SetInitialSpeed _projectilemovement (.travelspeed _returnvalue))
          (Variables|Default|SetImpulse (.impulse _returnvalue))
          (Components|Timeline|SetPlayRate (Variables|Default|GetCharge) (/ 1.0 (.charge_chargetime _returnvalue)))
          ;[0.15 0.15 0.15 0.5] As the spell is charged, updates the percent.
          (bind _chargetrack (Timeline|Charge PlayFromStart)
            (:Update
              (Variables|Default|SetChargePercent _chargetrack))
            (:Finished
              (Development|PrintString "Fully Charged"))))))
    (:CastFailed
      (Development|PrintString "ruh roh" true true "(R=50.000000,G=19.999998,B=0.000000,A=1.000000)"))))

(fn ConstructionScript)