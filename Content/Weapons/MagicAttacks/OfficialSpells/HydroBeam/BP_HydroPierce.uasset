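; BP_HydroPierce is a water spell projectile from the HydroBeam magic attack.
; On BeginPlay it reads Damage and Lifetime from its DT_Spells row, printing an error if the row is missing.
; Overlapping anything except the first player's pawn or another HydroPierce prints that actor's class and spawns an NS_HydroSplash Niagara effect at the projectile.
; The graph neither applies the damage, uses the lifetime, nor destroys the projectile.
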(event Collision|EventActorBeginOverlap
  (params (OtherActor :type Actor%20Object%20Reference))
  (bind _returnvalue (Utilities|GetClass OtherActor))
  (bind _returnvalue_2 (Transformation|GetActorTransform))
  ;[0.15 0.15 0.15 0.5] Spawns effect on collision/lifetime
  (if (not (== OtherActor (Game|Player|GetPlayerPawn 0)))
    (if (not (== _returnvalue "BP_HydroPierce_C"))
      (Development|PrintString (Utilities|GetClassDisplayName _returnvalue))
      (Niagara|SpawnSystematLocation "/Game/Weapons/MagicAttacks/OfficialSpells/HydroBeam/NS_HydroSplash.NS_HydroSplash" (.location _returnvalue_2) (.rotation _returnvalue_2)))))

(event EventBeginPlay
  ;[0.15 0.15 0.15 0.5] Initialize projectile
  (bind _returnvalue (Utilities|GetDataTableRow "/Game/DataTables/Spells/DT_Spells.DT_Spells" (Variables|Default|GetDataTableName))
    (:then
      (Variables|Default|SetDamage (.spelldamage _returnvalue))
      (Variables|Default|SetLifetime (.lifetime _returnvalue)))
    (:RowNotFound
      (Development|PrintString "You did something wrong idiot"))))

(fn ConstructionScript)