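; Projectile actor for the RockBlast spell that flies until it hits something or its lifetime runs out.
; On BeginPlay it reads damage, lifetime and travel speed from its DT_Spells row, then activates ProjectileMovement.
; Overlaps destroy it one tick later, ignoring the player pawn, Hitbox-tagged actors and other BP_RokThing instances.
; It stores Damage but applies none in these graphs.
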(event Custom|Spawn
  (bind _projectilemovement (Variables|Default|GetProjectileMovement))
  ;[0.15 0.15 0.15 0.5] Initialize the projectile (set its values based on the data table)
  (bind _returnvalue (Utilities|GetDataTableRow "/Game/DataTables/Spells/DT_Spells.DT_Spells" (Variables|Default|GetDataTableName))
    (:then
      (Variables|Default|SetDamage (.spelldamage _returnvalue))
      (Variables|Default|SetLifetime (.lifetime _returnvalue))
      (Variables|/Script/Engine.ProjectileMovementComponent|SetMaxSpeed _projectilemovement (.travelspeed _returnvalue))
      (Variables|/Script/Engine.ProjectileMovementComponent|SetInitialSpeed _projectilemovement (.travelspeed _returnvalue))
      (Components|Activation|Activate _projectilemovement false))))

(event Collision|EventActorBeginOverlap
  (params (OtherActor :type Actor%20Object%20Reference))
  ;[0.15 0.15 0.15 0.5] Destroys spell on collision or after set lifetime
  (if (not (== OtherActor (Game|Player|GetPlayerPawn 0)))
    (if (not (Actor|ActorHasTag OtherActor "Hitbox"))
      (if (not (== (Utilities|GetClass OtherActor) "BP_RokThing_C"))
        (Utilities|FlowControl|DelayUntilNextTick)
        (Actor|DestroyActor)))))

(event EventBeginPlay
  ;[0.15 0.15 0.15 0.5] Destroys spell on collision or after set lifetime
  (CallFunction|Spawn)
  (Utilities|FlowControl|Delay (Variables|Default|GetLifetime))
  (Actor|DestroyActor))

(fn ConstructionScript)