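; BP_BoltStrike is the actor for the Bolt Strike magic spell attack.
; On BeginPlay it reads its DT_Spells row to set damage, impulse and lifespan, then spawns the NS_BoltStrike Niagara effect at its location.
; A Sphere overlap with an Enemy-tagged actor destroys it after a short delay.
; Damage and impulse are only stored in this graph, not applied.
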(event OnComponentBeginOverlap(Sphere)
  (params (OverlappedComponent :type Primitive%20Component%20Object%20Reference) (OtherActor :type Actor%20Object%20Reference) (OtherComp :type Primitive%20Component%20Object%20Reference) (OtherBodyIndex :type Integer) (bFromSweep :type Boolean) (SweepResult :type Hit%20Result%20Structure%20%28by%20ref%29))
  ;[0.15 0.15 0.15 0.5] Spawns effect on collision/lifetime
  (if (Actor|ActorHasTag OtherActor "Enemy")
    (Utilities|FlowControl|Delay 0.2)
    (Actor|DestroyActor)))

(event EventBeginPlay
  ;[0.15 0.15 0.15 0.5] Initialize projectile
  (bind _returnvalue (Utilities|GetDataTableRow "/Game/DataTables/Spells/DT_Spells.DT_Spells" (Variables|Default|GetDataTableName))
    (:then
      (Variables|Default|SetDamage (.spelldamage _returnvalue))
      (Actor|SetLifeSpan (.lifetime _returnvalue))
      (Variables|Default|SetImpulse (.impulse _returnvalue))
      (Niagara|SpawnSystematLocation "/Game/Weapons/MagicAttacks/OfficialSpells/BoltStrike/NS_BoltStrike.NS_BoltStrike" (Transformation|GetActorLocation)))
    (:RowNotFound
      (Development|PrintString "You did something wrong idiot"))))

(fn ConstructionScript)