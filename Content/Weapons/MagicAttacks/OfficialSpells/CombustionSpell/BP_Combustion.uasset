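; BP_Combustion is a chargeable spell projectile that explodes, with damage, speed, lifetime and charge time read from DT_Spells.
; A Timeline grows its scale and ChargePercent until releasing IA_Attack scales Damage, detaches and launches it, and clears the character's Cooldown.
; Overlap after launch, lifetime expiry or overholding triggers a shared detonation that scales up the hidden actor and briefly lets CheckBox overlaps call Explode on the player character.
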(event OnComponentBeginOverlap(CheckBox)
  (params (OverlappedComponent :type Primitive%20Component%20Object%20Reference) (OtherActor :type Actor%20Object%20Reference) (OtherComp :type Primitive%20Component%20Object%20Reference) (OtherBodyIndex :type Integer) (bFromSweep :type Boolean) (SweepResult :type Hit%20Result%20Structure%20%28by%20ref%29))
  ;[0.15 0.15 0.15 0.5] Slaughters player if it can
  (bind _asbp_first_person_character (Utilities|Casting|CastToBP_FirstPersonCharacter OtherActor))
  (if (Variables|Default|GetCanHurtPlayer)
    (Default|Explode _asbp_first_person_character self)))

(event Custom|Charge
  (bind _projectilemovement (Variables|Default|GetProjectileMovement))
  ;[0.15 0.15 0.15 0.5] Initialize projectile
  (bind _returnvalue (Utilities|GetDataTableRow "/Game/DataTables/Spells/DT_Spells.DT_Spells" (Variables|Default|GetDataTableName))
    (:then
      (Variables|Default|SetDamage (.SpellDamage (Utilities|Struct|BreakSpellStructure _returnvalue)))
      (Variables|Default|SetLifetime (.Lifetime (Utilities|Struct|BreakSpellStructure _returnvalue)))
      (Variables|/Script/Engine.ProjectileMovementComponent|SetMaxSpeed _projectilemovement (.TravelSpeed (Utilities|Struct|BreakSpellStructure _returnvalue)))
      (Variables|/Script/Engine.ProjectileMovementComponent|SetInitialSpeed _projectilemovement (.TravelSpeed (Utilities|Struct|BreakSpellStructure _returnvalue)))
      (Components|Timeline|SetPlayRate (Variables|Default|GetTimeline) (/ 1.0 (.CHARGE_ChargeTime (Utilities|Struct|BreakSpellStructure _returnvalue))))
      ;[0.15 0.15 0.15 0.5] Scales spell and charge percent up over the course of the charge time
      (bind _newtrack_0 (Timeline|Timeline Play)
        (:Update
          (Transformation|SetActorScale3D (Math|Conversions|ToVector(Float) (* _newtrack_0 0.3)))
          (Variables|Default|SetChargePercent _newtrack_0))
        (:Finished
          ;[0.15 0.15 0.15 0.5] If charged spell is held for too long, detonates
          (Utilities|FlowControl|Delay 3.0)
          (if (not (Variables|Default|GetHasCharged))
            ;[0.15 0.15 0.15 0.5] Stops projectile
            (Components|Activation|Deactivate (Variables|Default|GetProjectileMovement))
            ;[0.15 0.15 0.15 0.5] Explode with effect
            (Rendering|SetActorHiddenInGame true)
            (Transformation|SetActorRelativeScale3D (Math|Conversions|ToVector(Float) (* (Variables|Default|GetChargePercent) 1e+01)))
            (Niagara|SpawnSystematLocation "/Game/Weapons/MagicAttacks/OfficialSpells/CombustionSpell/NS_ComExplosion.NS_ComExplosion" (Transformation|GetActorLocation) (Transformation|GetActorRotation) (Math|Conversions|ToVector(Float) (Variables|Default|GetChargePercent)))
            (Variables|Default|SetCanHurtPlayer true)
            (Variables|/Script/Engine.PrimitiveComponent|SetbGenerateOverlapEvents (Variables|Default|GetCheckBox) true)
            (Utilities|FlowControl|Delay 0.1)
            (Actor|DestroyActor)))))
    (:RowNotFound
      (Development|PrintString "You did something wrong idiot"))))

(event Input|EnhancedActionEvents|EnhancedInputActionIA_Attack
  (params (ActionValue :type Boolean) (ElapsedSeconds :type Float%20%28double-precision%29) (TriggeredSeconds :type Float%20%28double-precision%29) (InputAction :type Input%20Action%20Object%20Reference :default "/Game/Input/Actions/IA_Attack.IA_Attack"))
  (bind _projectilemovement (Variables|Default|GetProjectileMovement))
  ;[0.15 0.15 0.15 0.5] Checks when you release LMB to fire and scales damage accordingly
  (:Completed
    (if (not (Variables|Default|GetHasCharged))
      (Audio|Components|Audio|Stop (Variables|Default|GetTimeline))
      (Variables|Default|SetDamage (* (Variables|Default|GetDamage) (Variables|Default|GetChargePercent)))
      ;[0.15 0.15 0.15 0.5] Orients spell correctly and activates projectile movement
      (Variables|Default|SetHasCharged true)
      (Transformation|DetachFromActor "KeepWorld" "KeepWorld" "KeepWorld")
      (Variables|/Script/Engine.MovementComponent|SetVelocity _projectilemovement (* (Math|Vector|GetForwardVector (Variables|Default|GetArrow)) (Math|Conversions|ToVector(Float) 2.5e+03)))
      (Components|Activation|Activate _projectilemovement false)
      ;[0.15 0.15 0.15 0.5] Turns off cooldown after launching spell
      (bind _returnvalue (Actor|GetActorOfClass "/Game/FirstPerson/Blueprints/BP_FirstPersonCharacter.BP_FirstPersonCharacter_C"))
      (Variables|/Game/FirstPerson/Blueprints/BP_FirstPersonCharacter.BP_FirstPersonCharacter_C|SetCooldown _returnvalue false))))

(event Collision|EventActorBeginOverlap
  (params (OtherActor :type Actor%20Object%20Reference))
  (bind _chargepercent (Variables|Default|GetChargePercent))
  ;[0.15 0.15 0.15 0.5] Upon collision, checks if charged before detonating.
  (if (Variables|Default|GetHasCharged)
    ;[0.15 0.15 0.15 0.5] Stops projectile
    (Components|Activation|Deactivate (Variables|Default|GetProjectileMovement))
    ;[0.15 0.15 0.15 0.5] Explode with effect
    (Rendering|SetActorHiddenInGame true)
    (Transformation|SetActorRelativeScale3D (Math|Conversions|ToVector(Float) (* _chargepercent 1e+01)))
    (Niagara|SpawnSystematLocation "/Game/Weapons/MagicAttacks/OfficialSpells/CombustionSpell/NS_ComExplosion.NS_ComExplosion" (Transformation|GetActorLocation) (Transformation|GetActorRotation) (Math|Conversions|ToVector(Float) _chargepercent))
    (Variables|Default|SetCanHurtPlayer true)
    (Variables|/Script/Engine.PrimitiveComponent|SetbGenerateOverlapEvents (Variables|Default|GetCheckBox) true)
    (Utilities|FlowControl|Delay 0.1)
    (Actor|DestroyActor)))

(event EventBeginPlay
  (bind _chargepercent (Variables|Default|GetChargePercent))
  ;[0.15 0.15 0.15 0.5] Calls initiaizle and delays until lifetime is up
  (CallFunction|Charge)
  (Utilities|FlowControl|Delay (Variables|Default|GetLifetime))
  ;[0.15 0.15 0.15 0.5] Stops projectile
  (Components|Activation|Deactivate (Variables|Default|GetProjectileMovement))
  ;[0.15 0.15 0.15 0.5] Explode with effect
  (Rendering|SetActorHiddenInGame true)
  (Transformation|SetActorRelativeScale3D (Math|Conversions|ToVector(Float) (* _chargepercent 1e+01)))
  (Niagara|SpawnSystematLocation "/Game/Weapons/MagicAttacks/OfficialSpells/CombustionSpell/NS_ComExplosion.NS_ComExplosion" (Transformation|GetActorLocation) (Transformation|GetActorRotation) (Math|Conversions|ToVector(Float) _chargepercent))
  (Variables|Default|SetCanHurtPlayer true)
  (Variables|/Script/Engine.PrimitiveComponent|SetbGenerateOverlapEvents (Variables|Default|GetCheckBox) true)
  (Utilities|FlowControl|Delay 0.1)
  (Actor|DestroyActor))

(fn ConstructionScript)