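; Magic missile spell projectile that flies forward spinning and explodes on overlap or when its lifetime ends.
; On BeginPlay, Spawn reads its DT_Spells row to set damage, lifespan and speed, then activates ProjectileMovement.
; A restarting timeline drives the roll spin.
; Overlaps ignore the player pawn and Hitbox-tagged actors; others, like EndPlay, spawn the Niagara explosion and destroy the actor, with no damage applied here.
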(event Custom|Spawn
  (bind _returnvalue (Transformation|GetActorRotation))
  (bind _projectilemovement (Variables|Default|GetProjectileMovement))
  ;[0.15 0.15 0.15 0.5] Initialize the projectile (set its values based on the data table)
  (bind _returnvalue_2 (Utilities|GetDataTableRow "/Game/DataTables/Spells/DT_Spells.DT_Spells" (Variables|Default|GetDataTableName))
    (:then
      (Variables|Default|SetDamage (.spelldamage _returnvalue_2))
      (Actor|SetLifeSpan (.lifetime _returnvalue_2))
      (Variables|/Script/Engine.ProjectileMovementComponent|SetMaxSpeed _projectilemovement (.travelspeed _returnvalue_2))
      (Variables|/Script/Engine.ProjectileMovementComponent|SetInitialSpeed _projectilemovement (.travelspeed _returnvalue_2))
      (Components|Activation|Activate _projectilemovement false)
      ;[0.15 0.15 0.15 0.5] Spin Animation
      (bind _spin (Timeline|SpinTimeline Play)
        (:Update
          (Transformation|SetActorRotation (Math|Rotator|MakeRotator (* _spin 3.6e+02) (.pitch _returnvalue) (.yaw _returnvalue))))
        (:Finished
          (Timeline|SpinTimeline PlayFromStart))))))

(event EventEndPlay
  (params (EndPlayReason :type EEndPlayReason%20Enum :default "Destroyed"))
  (bind _returnvalue (Transformation|GetActorTransform))
  ;[0.15 0.15 0.15 0.5] Destroys spell on collision or after set lifetime
  (Niagara|SpawnSystematLocation "/Game/Weapons/MagicAttacks/OfficialSpells/MagicMissile/NS_MissileExplosion.NS_MissileExplosion" (.location _returnvalue) (.rotation _returnvalue))
  (Actor|DestroyActor))

(event Collision|EventActorBeginOverlap
  (params (OtherActor :type Actor%20Object%20Reference))
  (bind _returnvalue (Transformation|GetActorTransform))
  ;[0.15 0.15 0.15 0.5] Destroys spell on collision or after set lifetime
  (if (not (== OtherActor (Game|Player|GetPlayerPawn 0)))
    (if (not (Actor|ActorHasTag OtherActor "Hitbox"))
      (Niagara|SpawnSystematLocation "/Game/Weapons/MagicAttacks/OfficialSpells/MagicMissile/NS_MissileExplosion.NS_MissileExplosion" (.location _returnvalue) (.rotation _returnvalue))
      (Actor|DestroyActor))))

(event EventBeginPlay
  ;[0.15 0.15 0.15 0.5] Destroys spell on collision or after set lifetime
  (CallFunction|Spawn))

(fn ConstructionScript)