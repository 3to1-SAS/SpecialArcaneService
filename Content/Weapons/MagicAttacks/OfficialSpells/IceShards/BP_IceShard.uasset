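; Ice shard spell projectile that pulls its damage, lifetime and travel speed from DT_Spells on BeginPlay.
; A Shrink timeline, rate-scaled to the lifetime, scales the mesh to look like melting.
; Lifetime expiry or overlap with anything except player pawn 0 or another shard removes movement, disables overlaps and stops Niagara, then destroys it after a short delay.
; Damage is stored but not applied here.
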(event Custom|Melt
  (bind _projectilemovement (Variables|Default|GetProjectileMovement))
  ;[0.15 0.15 0.15 0.5] Initialize the projectile
  (bind _returnvalue (Utilities|GetDataTableRow "/Game/DataTables/Spells/DT_Spells.DT_Spells" (Variables|Default|GetDataTableName))
    (:then
      (Variables|Default|SetDamage (.SpellDamage (Utilities|Struct|BreakSpellStructure _returnvalue)))
      (Variables|Default|SetLifetime (.Lifetime (Utilities|Struct|BreakSpellStructure _returnvalue)))
      (Variables|/Script/Engine.ProjectileMovementComponent|SetMaxSpeed _projectilemovement (.TravelSpeed (Utilities|Struct|BreakSpellStructure _returnvalue)))
      (Variables|/Script/Engine.ProjectileMovementComponent|SetInitialSpeed _projectilemovement (.TravelSpeed (Utilities|Struct|BreakSpellStructure _returnvalue)))
      (Components|Timeline|SetPlayRate (Variables|Default|GetShrink) (/ 1.0 (Variables|Default|GetLifetime)))
      ;[0.15 0.15 0.15 0.5] Shrinks the actor to make it seem as if it is melting
      (bind _melttrack (Timeline|Shrink Play)
        (:Update
          (Transformation|SetRelativeScale3D (Variables|Default|GetReplaceWithModel) (Math|Vector|MakeVector (* _melttrack 0.3) (* _melttrack 0.3) _melttrack)))
        (:Finished
          (Components|DestroyComponent (Variables|Default|GetProjectileMovement))
          (Variables|/Script/Engine.PrimitiveComponent|SetbGenerateOverlapEvents (Variables|Default|GetReplaceWithModel) false)
          (Variables|/Script/Engine.PrimitiveComponent|SetbGenerateOverlapEvents (Variables|Default|GetBase) false)
          (Components|Activation|Deactivate (Variables|Default|GetNiagara))
          (Utilities|FlowControl|Delay 1.0)
          (Actor|DestroyActor))))
    (:RowNotFound
      (Development|PrintString "You did something wrong idiot"))))

(event Collision|EventActorBeginOverlap
  (params (OtherActor :type Actor%20Object%20Reference))
  ;[0.15 0.15 0.15 0.5] Destroys spell on collision or after set delay
  (if (not (== OtherActor (Game|Player|GetPlayerPawn 0)))
    (if (not (== (Utilities|GetClass OtherActor) "BP_IceShard_C"))
      (Variables|/Script/Engine.PrimitiveComponent|SetbGenerateOverlapEvents (Variables|Default|GetReplaceWithModel) false)
      (Variables|/Script/Engine.PrimitiveComponent|SetbGenerateOverlapEvents (Variables|Default|GetBase) false)
      (Components|DestroyComponent (Variables|Default|GetProjectileMovement))
      (Variables|/Script/Engine.PrimitiveComponent|SetbGenerateOverlapEvents (Variables|Default|GetReplaceWithModel) false)
      (Variables|/Script/Engine.PrimitiveComponent|SetbGenerateOverlapEvents (Variables|Default|GetBase) false)
      (Components|Activation|Deactivate (Variables|Default|GetNiagara))
      (Utilities|FlowControl|Delay 1.0)
      (Actor|DestroyActor))))

(event EventBeginPlay
  ;[0.15 0.15 0.15 0.5] Destroys spell on collision or after set delay
  (CallFunction|Melt)
  (Utilities|FlowControl|Delay (Variables|Default|GetLifetime))
  (Variables|/Script/Engine.PrimitiveComponent|SetbGenerateOverlapEvents (Variables|Default|GetReplaceWithModel) false)
  (Variables|/Script/Engine.PrimitiveComponent|SetbGenerateOverlapEvents (Variables|Default|GetBase) false)
  (Components|DestroyComponent (Variables|Default|GetProjectileMovement))
  (Variables|/Script/Engine.PrimitiveComponent|SetbGenerateOverlapEvents (Variables|Default|GetReplaceWithModel) false)
  (Variables|/Script/Engine.PrimitiveComponent|SetbGenerateOverlapEvents (Variables|Default|GetBase) false)
  (Components|Activation|Deactivate (Variables|Default|GetNiagara))
  (Utilities|FlowControl|Delay 1.0)
  (Actor|DestroyActor))

(fn ConstructionScript)