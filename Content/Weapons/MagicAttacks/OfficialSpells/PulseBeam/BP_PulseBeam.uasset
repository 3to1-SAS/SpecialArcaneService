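; BP_PulseBeam is a spell projectile that reads its damage and lifetime from the spells data table on BeginPlay.
; On sphere overlap, ignoring the player and other pulse beams, it spawns a Niagara impact effect, attached to the capsule for Enemy-tagged actors, otherwise at its location.
; It then shoves the hit component along its arrow's forward vector and destroys itself after a short delay.
; The stored damage is never applied in this graph.
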(event OnComponentBeginOverlap(Sphere)
  (params (OverlappedComponent :type Primitive%20Component%20Object%20Reference) (OtherActor :type Actor%20Object%20Reference) (OtherComp :type Primitive%20Component%20Object%20Reference) (OtherBodyIndex :type Integer) (bFromSweep :type Boolean) (SweepResult :type Hit%20Result%20Structure%20%28by%20ref%29))
  (bind _returnvalue (Utilities|GetClass OtherActor))
  (bind _returnvalue_2 (Transformation|GetActorTransform))
  ;[0.15 0.15 0.15 0.5] Spawns effect on collision/lifetime
  (if (not (== OtherActor (Game|Player|GetPlayerPawn 0)))
    (if (not (== _returnvalue "BP_PulseBeam_C"))
      (Development|PrintString (Utilities|GetClassDisplayName _returnvalue))
      (if (Actor|ActorHasTag OtherActor "Enemy")
        (Niagara|SpawnSystemAttached "/Game/Weapons/MagicAttacks/OfficialSpells/PulseBeam/NS_PulseImpact.NS_PulseImpact" (Actor|GetComponentbyClass OtherActor "/Script/Engine.CapsuleComponent") "None" (.location _returnvalue_2) (.rotation _returnvalue_2) "KeepWorldPosition" false)
        (Utilities|FlowControl|Delay 0.025)
        (else
          (Niagara|SpawnSystematLocation "/Game/Weapons/MagicAttacks/OfficialSpells/PulseBeam/NS_PulseImpact.NS_PulseImpact" (.location _returnvalue_2) (.rotation _returnvalue_2))))
      (Physics|AddImpulse OtherComp (* (Math|Vector|GetForwardVector (Variables|Default|GetArrow)) 2.5e+05) "None" false)
      (Utilities|FlowControl|Delay 0.2)
      (Actor|DestroyActor))))

(event EventBeginPlay
  ;[0.15 0.15 0.15 0.5] Initialize projectile
  (bind _returnvalue (Utilities|GetDataTableRow "/Game/DataTables/Spells/DT_Spells.DT_Spells" (Variables|Default|GetDataTableName))
    (:then
      (Variables|Default|SetDamage (.spelldamage _returnvalue))
      (Actor|SetLifeSpan (.lifetime _returnvalue)))
    (:RowNotFound
      (Development|PrintString "You did something wrong idiot"))))

(fn ConstructionScript)