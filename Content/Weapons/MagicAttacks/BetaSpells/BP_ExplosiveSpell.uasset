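; BP_ExplosiveSpell is a spell actor that explodes on overlapping anything but the player, or when its lifetime expires.
; The blast scales the actor up, sets CanHurtPlayer, enables CheckBox overlap events, then destroys it after a brief delay.
; Player overlaps on the actor or CheckBox call Explode on BP_FirstPersonCharacter only while CanHurtPlayer is set, passing the spell.
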(event OnComponentBeginOverlap(CheckBox)
  (params (OverlappedComponent :type Primitive%20Component%20Object%20Reference) (OtherActor :type Actor%20Object%20Reference) (OtherComp :type Primitive%20Component%20Object%20Reference) (OtherBodyIndex :type Integer) (bFromSweep :type Boolean) (SweepResult :type Hit%20Result%20Structure%20%28by%20ref%29))
  (Utilities|Casting|CastToBP_FirstPersonCharacter OtherActor)
  ;[0.15 0.15 0.15 0.5] Destroys spell on collision or after set delay
  (if (Variables|Default|GetCanHurtPlayer)
    (bind _asbp_first_person_character (Utilities|Casting|CastToBP_FirstPersonCharacter (Game|Player|GetPlayerPawn 0)))
    (Default|Explode _asbp_first_person_character self)))

(event Collision|EventActorBeginOverlap
  (params (OtherActor :type Actor%20Object%20Reference))
  (bind _returnvalue (Game|Player|GetPlayerPawn 0))
  ;[0.15 0.15 0.15 0.5] Destroys spell on collision or after set delay
  (if (== OtherActor _returnvalue)
    (if (Variables|Default|GetCanHurtPlayer)
      (bind _asbp_first_person_character (Utilities|Casting|CastToBP_FirstPersonCharacter _returnvalue))
      (Default|Explode _asbp_first_person_character self))
    (else
      (Transformation|SetActorRelativeScale3D "10.000000,10.000000,10.000000")
      (Variables|Default|SetCanHurtPlayer true)
      (Variables|/Script/Engine.PrimitiveComponent|SetbGenerateOverlapEvents (Variables|Default|GetCheckBox) true)
      (Utilities|FlowControl|Delay 0.1)
      (Actor|DestroyActor))))

(event EventBeginPlay
  ;[0.15 0.15 0.15 0.5] Destroys spell on collision or after set delay
  (Utilities|FlowControl|Delay (Variables|Default|GetLifetime))
  (Transformation|SetActorRelativeScale3D "10.000000,10.000000,10.000000")
  (Variables|Default|SetCanHurtPlayer true)
  (Variables|/Script/Engine.PrimitiveComponent|SetbGenerateOverlapEvents (Variables|Default|GetCheckBox) true)
  (Utilities|FlowControl|Delay 0.1)
  (Actor|DestroyActor))

(fn ConstructionScript)