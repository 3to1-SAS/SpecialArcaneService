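; Boss fight VFX manager that links the level's Niagara energy orb to each totem and to the Fallen Angel with beams.
; A looping timer tracks the boss beam to the boss, while Niagara particle callbacks feed direction vectors into each totem beam's dynamic material.
; Each totem death removes the last beam, retargets the rest to living totems and timer-steps orb Stability to shrink it.
; The final death destroys the orb with a burst.
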(event Custom|DestroyOrb
  (bind _energyorb (Variables|Default|GetEnergyOrb))
  (bind _niagaracomponent (Variables|/Script/Niagara.NiagaraActor|GetNiagaraComponent _energyorb))
  ;[0.15 0.15 0.15 0.5] Destroys the orb
  (bind _returnvalue (Utilities|Time|SetTimerbyFunctionName 0 "SlowDecrease" 0.025 true))
  (bind _output_get (Variables|Default|SetDecreaseTimer _returnvalue))
  (if (Utilities|Time|IsValidTimerHandle _output_get) :!label _label
    (Utilities|FlowControl|Delay 0.1)
    (goto _label)
    (else
      (Class|NiagaraComponent|SetVariableBool _niagaracomponent "ShouldDestroy" true)
      (Niagara|SpawnSystemAttached "/Game/ArtAssets/VFX/BossBeamVFX/NS_OrbBurst.NS_OrbBurst" _niagaracomponent "None" "0, 0, 0" "0, 0, 0" "SnapToTargetIncludingScale" false))))

(event Custom|DecreaseStability
  ;[0.15 0.15 0.15 0.5] When one of the totems is destroyed, shrinks the orb
  (bind _returnvalue (Utilities|Time|SetTimerbyFunctionName 0 "SlowDecrease" 0.025 true))
  (Variables|Default|SetDecreaseTimer _returnvalue))

(event EventBeginPlay
  (Utilities|FlowControl|Sequence
    (:then_0
      ;[0.15 0.15 0.15 0.5] Finds the energy orb in the level
      (bind _outactors (Actor|GetAllActorsOfClass "/Script/Niagara.NiagaraActor"))
      (bind _array_element (Utilities|Array|ForEachLoopwithBreak _outactors :!label _label)
        (:LoopBody
          (if (== (AssetData|GetAsset (Variables|/Script/Niagara.NiagaraActor|GetNiagaraComponent _array_element)) "/Game/ArtAssets/VFX/BossBeamVFX/NS_BossEnergyOrb.NS_BossEnergyOrb")
            (Variables|Default|SetEnergyOrb _array_element)
            (goto _label Break)
            (else
              (goto _label))))))
    (:then_1
      ;[0.15 0.15 0.15 0.5] Spawns a beam for each totem in the level
      (Utilities|IsValid (Variables|Default|GetEnergyOrb)
        (:Is%20Valid
          (bind _outactors_2 (Actor|GetAllActorsOfClass "/Game/Enemies/FallenAngel/BP_BossTotem.BP_BossTotem_C"))
          (for _array_element_2 _outactors_2
            (bind _returnvalue (Niagara|SpawnSystematLocation "/Game/ArtAssets/VFX/BossBeamVFX/NS_TotemBeams.NS_TotemBeams" (Transformation|GetActorLocation (Variables|Default|GetEnergyOrb))))
            (bind _returnvalue_2 (Utilities|Array|Add (Variables|Default|GetSpawnedSystems) _returnvalue))
            (Class|NiagaraComponent|SetVariableInt _returnvalue "SystemIndex" _returnvalue_2)
            (Niagara|SetNiagaraVariable(Vector3) _returnvalue "EndTarget" (Transformation|GetWorldLocation (Variables|/Game/Enemies/FallenAngel/BP_BossTotem.BP_BossTotem_C|GetHeart _array_element_2)))
            (Niagara|SetNiagaraVariable(Float) _returnvalue "FieldScale" 2.5)
            (Class|NiagaraComponent|SetVariableObject _returnvalue "Callback" self)
            (bind _returnvalue_3 (Rendering|Material|CreateDynamicMaterialInstance (Variables|Default|GetMAT) "None" "None" :!class /Script/Engine.KismetMaterialLibrary))
            (Utilities|Array|Add (Variables|Default|GetBeamMaterial) _returnvalue_3)
            (Class|NiagaraComponent|SetVariableMaterial _returnvalue "BeamMaterial" _returnvalue_3)
            (Game|BindEventtoOnDestroyed _array_element_2 (EventDispatchers|CreateEvent :!event TotemDestroyed))))
        (:Is%20Not%20Valid
          (Development|PrintString "Something isn't WORKING"))))
    (:then_2
      ;[0.15 0.15 0.15 0.5] Spawns a beam for the boss and constantly updates its end point based on the boss' location.
      (bind _returnvalue_4 (Actor|GetActorOfClass "/Game/Enemies/FallenAngel/BP_FallenAngel.BP_FallenAngel_C"))
      (Variables|Default|SetFallenAngel _returnvalue_4)
      (bind _returnvalue_5 (Niagara|SpawnSystematLocation "/Game/ArtAssets/VFX/BossBeamVFX/NS_BossBeam.NS_BossBeam" (Math|Vector|MakeVector (.X (Math|Vector|BreakVector (Transformation|GetActorLocation (Variables|Default|GetEnergyOrb)))) (.Y (Math|Vector|BreakVector (Transformation|GetActorLocation (Variables|Default|GetEnergyOrb)))) (+ (.Z (Math|Vector|BreakVector (Transformation|GetActorLocation (Variables|Default|GetEnergyOrb)))) 5e+02))))
      (bind _output_get (Variables|Default|SetBossBeam _returnvalue_5))
      (bind _output_get_2 (Variables|/Game/Enemies/FallenAngel/BP_FallenAngel.BP_FallenAngel_C|SetBossBeam (Variables|Default|GetFallenAngel) _output_get))
      (Niagara|SetNiagaraVariable(Vector3) _output_get_2 "StartTarget" (Transformation|GetActorLocation (Variables|Default|GetEnergyOrb)))
      (Niagara|SetNiagaraVariable(Vector3) _output_get_2 "FinalEndTarget" (Transformation|GetActorLocation (Variables|Default|GetEnergyOrb)))
      (bind _returnvalue_6 (Utilities|Time|SetTimerbyFunctionName 0 "UpdateBeamLoc" 0.0025 true))
      (Variables|Default|SetUpdateTimer _returnvalue_6)
      (Variables|/Game/Enemies/FallenAngel/BP_FallenAngel.BP_FallenAngel_C|SetBossEnergyOrb (Variables|Default|GetFallenAngel) (Variables|Default|GetEnergyOrb)))))

(event EventParticleData
  (params (Data :type Array%20of%20Basic%20Particle%20Data%20Structures) (NiagaraSystem :type Niagara%20System%20Object%20Reference) (SimulationPositionOffset :type Vector%20%28by%20ref%29 :default "0, 0, 0"))
  (if (== NiagaraSystem "/Game/ArtAssets/VFX/BossBeamVFX/NS_TotemBeams.NS_TotemBeams")
    (for _array_element Data
      (bind (_array_element_2 _array_index) (Utilities|Array|ForEachLoopwithBreak (Variables|Default|GetBeamMaterial) :!label _label)
        (:LoopBody
          (if (== _array_index (Math|Float|Truncate (.Size (Utilities|Struct|BreakBasicParticleData _array_element))))
            (Variables|Default|SetTempMat _array_element_2)
            (goto _label Break)))
        (:Completed
          (Rendering|Material|SetVectorParameterValue (Variables|Default|GetTempMat) "MoveDirection" (* (Math|Color|MakeColor (.X (Math|Vector|BreakVector (.Position (Utilities|Struct|BreakBasicParticleData _array_element)))) (.Y (Math|Vector|BreakVector (.Position (Utilities|Struct|BreakBasicParticleData _array_element)))) (.Z (Math|Vector|BreakVector (.Position (Utilities|Struct|BreakBasicParticleData _array_element))))) 5e+01) :!class /Script/Engine.MaterialInstanceDynamic)
          (Rendering|Material|SetVectorParameterValue (Variables|Default|GetTempMat) "StretchDirection" (* (Math|Color|MakeColor (.X (Math|Vector|BreakVector (.Position (Utilities|Struct|BreakBasicParticleData _array_element)))) (.Y (Math|Vector|BreakVector (.Position (Utilities|Struct|BreakBasicParticleData _array_element)))) (.Z (Math|Vector|BreakVector (.Position (Utilities|Struct|BreakBasicParticleData _array_element))))) 1e+01) :!class /Script/Engine.MaterialInstanceDynamic))))
    (Development|PrintString "aw fart")))

(fn UpdateBeamLoc
  (bind _fallenangel (Variables|Default|GetFallenAngel))
  (bind _returnvalue (Transformation|GetActorLocation _fallenangel))
  (bind (_x _y _z) (Math|Vector|BreakVector _returnvalue))
  ;[0.15 0.15 0.15 0.5] Continuously updates the end target of the boss beam
  (Niagara|SetNiagaraVariable(Vector3) (Variables|Default|GetBossBeam) "EndTarget" (Math|Vector|MakeVector _x _y (+ _z 5e+02))))

(fn TotemDestroyed
  (params (DestroyedActor :type Actor%20Object%20Reference))
  (bind _spawnedsystems (Variables|Default|GetSpawnedSystems))
  (bind _returnvalue (Utilities|Array|LastIndex _spawnedsystems))
  (bind _output (Utilities|Array|Get(acopy) _spawnedsystems _returnvalue))
  ;[0.15 0.15 0.15 0.5] Destroys one of the beams when a totem is destroyed.
  (Components|DestroyComponent _output)
  (Utilities|Array|RemoveItem _spawnedsystems _output)
  (if (> (Utilities|Array|Length _spawnedsystems) 0)
    (bind _outactors (Actor|GetAllActorsOfClass "/Game/Enemies/FallenAngel/BP_BossTotem.BP_BossTotem_C"))
    ;[0.15 0.15 0.15 0.5] Repositions each other beam to match the existing totems.
    (for _array_element _outactors
      (if (Variables|/Game/Enemies/FallenAngel/BP_BossTotem.BP_BossTotem_C|GetIsAlive _array_element)
        (Niagara|SetNiagaraVariable(Vector3) (Utilities|Array|Get(acopy) (Variables|Default|GetSpawnedSystems) (LocalVariables|GetIndex)) "EndTarget" (Transformation|GetWorldLocation (Variables|/Game/Enemies/FallenAngel/BP_BossTotem.BP_BossTotem_C|GetHeart _array_element)))
        (LocalVariables|SetIndex (+ (LocalVariables|GetIndex) 1))))
    (LocalVariables|SetIndex 0)
    (Variables|Default|SetMaxStability (+ (Variables|Default|GetMaxStability) 1.0))
    (CallFunction|DecreaseStability)
    (Development|PrintString "Chaching")
    (else
      ;[0.15 0.15 0.15 0.5] Destroys the orb once there are no totems left
      (Variables|Default|SetMaxStability (+ (Variables|Default|GetMaxStability) 1.0))
      (CallFunction|DestroyOrb))))

(fn SlowDecrease
  (if (< (+ (Variables|Default|GetStabilitiy) (LocalVariables|GetSubtractionRate)) (Variables|Default|GetMaxStability))
    (bind _output_get (Variables|Default|SetStabilitiy (+ (Variables|Default|GetStabilitiy) (LocalVariables|GetSubtractionRate))))
    (Niagara|SetNiagaraVariable(Float) (Variables|/Script/Niagara.NiagaraActor|GetNiagaraComponent (Variables|Default|GetEnergyOrb)) "Stability" _output_get)
    (else
      (Utilities|Time|ClearandInvalidateTimerbyHandle (Variables|Default|GetDecreaseTimer)))))