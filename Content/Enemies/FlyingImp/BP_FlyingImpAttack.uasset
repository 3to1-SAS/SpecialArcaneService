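; Flying Imp attack actor that explodes on overlapping any actor not tagged "enemy", or when its lifespan runs out.
; The lifespan comes from the FlyingImpAttack row of DT_EnemySpells, and its expiry feeds the same explosion sequence as overlap.
; The explosion hides and enlarges the actor, spawns a system effect, enables CheckBox overlap events, then destroys the actor after a brief delay.
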(event Collision|EventActorBeginOverlap
  (params (OtherActor :type Actor%20Object%20Reference))
  ;[0.15 0.15 0.15 0.5] Explode with effect
  (if (not (Actor|ActorHasTag OtherActor "enemy"))
    (Rendering|SetActorHiddenInGame true)
    (Transformation|SetActorRelativeScale3D "5.000000,5.000000,5.000000")
    (Niagara|SpawnSystematLocation "/Game/Weapons/MagicAttacks/OfficialSpells/CombustionSpell/NS_ComExplosion.NS_ComExplosion" (Transformation|GetActorLocation) (Transformation|GetActorRotation) (Math|Conversions|ToVector(Float) 0.0))
    (Variables|/Script/Engine.PrimitiveComponent|SetbGenerateOverlapEvents (Variables|Default|GetCheckBox) true)
    (Utilities|FlowControl|Delay 0.1)
    (Actor|DestroyActor)))

(event EventBeginPlay
  ;[0.15 0.15 0.15 0.5] Explode with effect
  (bind _returnvalue (Utilities|GetDataTableRow "/Game/DataTables/Enemies/EnemySpells/DT_EnemySpells.DT_EnemySpells" "FlyingImpAttack")
    (:then
      (Utilities|FlowControl|Delay (.lifespan _returnvalue))
      (Rendering|SetActorHiddenInGame true)
      (Transformation|SetActorRelativeScale3D "5.000000,5.000000,5.000000")
      (Niagara|SpawnSystematLocation "/Game/Weapons/MagicAttacks/OfficialSpells/CombustionSpell/NS_ComExplosion.NS_ComExplosion" (Transformation|GetActorLocation) (Transformation|GetActorRotation) (Math|Conversions|ToVector(Float) 0.0))
      (Variables|/Script/Engine.PrimitiveComponent|SetbGenerateOverlapEvents (Variables|Default|GetCheckBox) true)
      (Utilities|FlowControl|Delay 0.1)
      (Actor|DestroyActor))))

(fn ConstructionScript)