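; Flying imp enemy that runs on a behavior tree and takes damage from spells and the sword.
; On BeginPlay it configures its AI controller, then a tick later loads HP from DT_Enemies and fills the Blackboard with combat, patrol and hearing settings.
; Capsule overlaps apply DT_Spells damage or fixed sword damage and turn it toward the source.
; At zero HP it is destroyed and the game mode updates the enemy count.
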(event OnComponentBeginOverlap(CapsuleComponent)
  (params (OverlappedComponent :type Primitive%20Component%20Object%20Reference) (OtherActor :type Actor%20Object%20Reference) (OtherComp :type Primitive%20Component%20Object%20Reference) (OtherBodyIndex :type Integer) (bFromSweep :type Boolean) (SweepResult :type Hit%20Result%20Structure%20%28by%20ref%29))
  (bind _returnvalue (Utilities|GetClass OtherActor))
  ;[0.15 0.15 0.15 0.5] Calculates damage taken based on spell
  (if (Actor|ActorHasTag OtherActor "Spell")
    (bind _name (Default|GetRow (.AsBP%20AIController (Utilities|Casting|CastToBP_AIController (AI|GetAIController self))) _returnvalue))
    (bind _returnvalue_2 (Utilities|GetDataTableRow "/Game/DataTables/Spells/DT_Spells.DT_Spells" _name)
      (:then
        (Variables|Default|SetHP (- (Variables|Default|GetHP) (.SpellDamage (Utilities|Struct|BreakSpellStructure _returnvalue_2))))
        ;[0.15 0.15 0.15 0.5] Faces towards location of damage
        (Transformation|SetActorRotation (Math|Rotator|MakeRotator 0.0 0.0 (.yaw (Math|Rotator|FindLookatRotation (Transformation|GetActorLocation) (Transformation|GetActorLocation OtherActor)))) :!label _label)
        ;[0.15 0.15 0.15 0.5] Destroys enemy when health is 0
        (if (<= (Variables|Default|GetHP) 0.0)
          (Actor|DestroyActor)
          (Default|UpdateEnemyCount (.AsBP%20First%20Person%20Game%20Mode (Utilities|Casting|CastToBP_FirstPersonGameMode (Game|GetGameMode)))))))
    (elif (== _returnvalue "/Game/Weapons/MeleeAttacks/BP_Sword.BP_Sword_C")
      (Variables|Default|SetHP (- (Variables|Default|GetHP) 6e+02))
      (goto _label))))

(event EventBeginPlay
  (bind _returnvalue (AI|GetBlackboard 0))
  ;[0.15 0.15 0.15 0.5] Sets The Data Table Row, Spell Cooldown, And Line of Sight Time On Blackboard
  (bind _asbp_aicontroller (Utilities|Casting|CastToBP_AIController (AI|GetAIController self))
    (:then
      (Variables|/Game/NPC_Comp/BP_AIController.BP_AIController_C|SetBehaviorTreeAsset _asbp_aicontroller "/Game/Enemies/FlyingImp/BT_FlyingImp.BT_FlyingImp")
      (Variables|/Game/NPC_Comp/BP_AIController.BP_AIController_C|SetDetectionRadius _asbp_aicontroller (Variables|Default|GetDetectionRange))
      (Utilities|FlowControl|DelayUntilNextTick)
      (Class|BlackboardComponent|SetValueasName _returnvalue (Variables|Default|GetDataTableRow) "FlyingImp")
      (bind _returnvalue_2 (Utilities|GetDataTableRow "/Game/DataTables/Enemies/DT_Enemies.DT_Enemies" "FlyingImp")
        (:then
          (Variables|Default|SetHP (.MaxHP (Utilities|Struct|BreakEnemiesStructure _returnvalue_2)))
          (AI|Components|Blackboard|SetValueasFloat _returnvalue (Variables|Default|GetSpellCooldown) (.AttackCooldown (Utilities|Struct|BreakEnemiesStructure _returnvalue_2)))
          (AI|Components|Blackboard|SetValueasFloat _returnvalue (Variables|Default|GetLOSTime) (.ChaseTime (Utilities|Struct|BreakEnemiesStructure _returnvalue_2)))
          (AI|Components|Blackboard|SetValueasFloat _returnvalue (Variables|Default|GetAttackRange) (.AttackRange (Utilities|Struct|BreakEnemiesStructure _returnvalue_2)))
          (AI|Components|Blackboard|SetValueasEnum _returnvalue (Variables|Default|GetPatrols) (Variables|Default|GetPatrolBehavior))
          (AI|Components|Blackboard|SetValueasFloat _returnvalue (Variables|Default|GetRadius) (Variables|Default|GetPatrolRadius))
          (AI|Components|Blackboard|SetValueasBool _returnvalue (Variables|Default|GetBBCanHear) (Variables|Default|GetCanHear)))))
    (:CastFailed
      (Development|PrintString "Cast failed"))))

(fn ConstructionScript)