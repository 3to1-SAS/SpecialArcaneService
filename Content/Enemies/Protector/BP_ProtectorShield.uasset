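; Protector enemy's shield actor that follows its owner, takes damage from spells and destroys itself when HP runs out or the owner is gone.
; Health and size come from DT_EnemySpells, while overlapping spells are matched by class in DT_Spells.
; BoltStrike deals fixed heavy damage; charge spells either scale by size or start a timed health drain scaled by remaining lifespan.
; Sphere overlaps switch collision responses when the player is inside.
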(event OnComponentBeginOverlap(Sphere1)
  (params (OverlappedComponent :type Primitive%20Component%20Object%20Reference) (OtherActor :type Actor%20Object%20Reference) (OtherComp :type Primitive%20Component%20Object%20Reference) (OtherBodyIndex :type Integer) (bFromSweep :type Boolean) (SweepResult :type Hit%20Result%20Structure%20%28by%20ref%29))
  (bind _sphere1 (Variables|Default|GetSphere1))
  ;[0.15 0.15 0.15 0.5] Disables collision while player is inside of shield
  (Utilities|FlowControl|DoOnce false :!label _label
    (:Completed
      (bind _array_element (Utilities|Array|ForEachLoopwithBreak (Collision|GetOverlappingActors 0 :!class /Script/Engine.Actor) :!label _label_2)
        (:LoopBody
          (if (== (Utilities|GetClass _array_element) "/Game/FirstPerson/Blueprints/BP_FirstPersonCharacter.BP_FirstPersonCharacter_C")
            (Collision|SetCollisionResponsetoAllChannels _sphere1 "ECR_Ignore")
            (Collision|SetCollisionResponsetoChannel _sphere1 "ECC_Pawn" "ECR_Overlap")
            (goto _label_2 Break)
            (else
              (Collision|SetCollisionResponsetoAllChannels _sphere1 "ECR_Overlap")
              (Collision|SetCollisionResponsetoChannel _sphere1 "ECC_Visibility" "ECR_Ignore")
              (Collision|SetCollisionResponsetoChannel _sphere1 "ECC_Camera" "ECR_Block"))))
        (:Completed
          (goto _label Reset))))))

(event OnComponentEndOverlap(Sphere1)
  (params (OverlappedComponent :type Primitive%20Component%20Object%20Reference) (OtherActor :type Actor%20Object%20Reference) (OtherComp :type Primitive%20Component%20Object%20Reference) (OtherBodyIndex :type Integer))
  (bind _sphere1 (Variables|Default|GetSphere1))
  ;[0.15 0.15 0.15 0.5] Disables collision while player is inside of shield
  (Utilities|FlowControl|Delay 0.2)
  (Utilities|FlowControl|DoOnce false :!label _label
    (:Completed
      (bind _array_element (Utilities|Array|ForEachLoopwithBreak (Collision|GetOverlappingActors 0 :!class /Script/Engine.Actor) :!label _label_2)
        (:LoopBody
          (if (== (Utilities|GetClass _array_element) "/Game/FirstPerson/Blueprints/BP_FirstPersonCharacter.BP_FirstPersonCharacter_C")
            (Collision|SetCollisionResponsetoAllChannels _sphere1 "ECR_Ignore")
            (Collision|SetCollisionResponsetoChannel _sphere1 "ECC_Pawn" "ECR_Overlap")
            (goto _label_2 Break)
            (else
              (Collision|SetCollisionResponsetoAllChannels _sphere1 "ECR_Overlap")
              (Collision|SetCollisionResponsetoChannel _sphere1 "ECC_Visibility" "ECR_Ignore")
              (Collision|SetCollisionResponsetoChannel _sphere1 "ECC_Camera" "ECR_Block"))))
        (:Completed
          (goto _label Reset))))))

(event Custom|DrainHealth
  (params (HealthDrain :type Float%20%28double-precision%29) (TimesToDrain :type Integer))
  ;[0.15 0.15 0.15 0.5] Drains health over a period of time
  (bind _output_get (Variables|Default|SetTimesDrained 0))
  (if (and (< _output_get TimesToDrain) (> (Variables|Default|GetHP) 0.0)) :!label _label
    (Variables|Default|SetHP (- (Variables|Default|GetHP) HealthDrain))
    (Development|PrintString "Damaged" true true "(R=0.000000,G=0.660000,B=1.000000,A=1.000000)" 2.5)
    (Variables|Default|SetTimesDrained (+ (Variables|Default|GetTimesDrained) 1))
    (Utilities|FlowControl|Delay 1.0)
    (goto _label)
    (elif (not (> (Variables|Default|GetHP) 0.0))
      (CallFunction|HealthDrained))))

(event Custom|HealthDrained
  ;[0.15 0.15 0.15 0.5] Calculates damage taken based on spell
  (if (<= (Variables|Default|GetHP) 0.0)
    (Actor|DestroyActor)))

(event EventBeginPlay
  ;[0.15 0.15 0.15 0.5] Sets the shield's HP and size from the data table
  (bind _returnvalue (Utilities|GetDataTableRow "/Game/DataTables/Enemies/EnemySpells/DT_EnemySpells.DT_EnemySpells" "ProtectorShield")
    (:then
      (Variables|Default|SetHP (.SHIELD-Health (Utilities|Struct|BreakEnemySpellStructure _returnvalue)))
      (Transformation|SetActorScale3D (Math|Conversions|ToVector(Float) (.SHIELD-Size (Utilities|Struct|BreakEnemySpellStructure _returnvalue)))))))

(event EventTick
  (params (DeltaSeconds :type Float%20%28single-precision%29))
  (bind _ownerenemy (Variables|Default|GetOwnerEnemy))
  ;[0.15 0.15 0.15 0.5] Moves the shield along with the enemy
  (if (Utilities|IsValid _ownerenemy)
    (Transformation|SetActorLocation (Transformation|GetActorLocation _ownerenemy) false false)
    (else
      (Actor|DestroyActor))))

(event Collision|EventActorBeginOverlap
  (params (OtherActor :type Actor%20Object%20Reference))
  ;[0.15 0.15 0.15 0.5] Calculates damage taken based on spell
  (if (Actor|ActorHasTag OtherActor "Spell")
    (bind _name (CallFunction|GetRow (Utilities|GetClass OtherActor)))
    (if (== _name "BoltStrike")
      (Variables|Default|SetHP (- (Variables|Default|GetHP) 2e+03))
      (else
        (bind _damage (CallFunction|ScaleDamage _name OtherActor))
        (Variables|Default|SetHP (- (Variables|Default|GetHP) _damage))))
    (if (<= (Variables|Default|GetHP) 0.0)
      (Actor|DestroyActor))))

(fn ConstructionScript)

(fn GetRow
  (params (Class :type Actor%20Class%20Reference))
  ;[0.15 0.15 0.15 0.5] Checks each row on the data table to find which one the enemy collided with
  (bind _outrownames (DataTable|GetDataTableRowNames "/Game/DataTables/Spells/DT_Spells.DT_Spells"))
  (for _array_element _outrownames
    (bind _returnvalue (Utilities|GetDataTableRow "/Game/DataTables/Spells/DT_Spells.DT_Spells" _array_element)
      (:then
        (if (== (.Spell (Utilities|Struct|BreakSpellStructure _returnvalue)) Class)
          (return _array_element))))))

(fn ScaleDamage
  (params (SpellRow :type Name) (SpellActor :type Actor%20Object%20Reference))
  (bind _returnvalue (Actor|GetLifeSpan SpellActor))
  (bind _returnvalue_2 (Math|Random|RandomIntegerinRange 3 7))
  (bind _returnvalue_3 (- 7.0 _returnvalue))
  (bind _returnvalue_4 (/ _returnvalue_3 3.0))
  ;[0.15 0.15 0.15 0.5] Checks if the spell is a charge spell. If so, scales its damage accordingly. If Toxic Thorn, initiates health drain.
  (bind _returnvalue_5 (Utilities|GetDataTableRow "/Game/DataTables/Spells/DT_Spells.DT_Spells" SpellRow)
    (:then
      (if (Utilities|Enum|Equal(Enum) (.SpellType (Utilities|Struct|BreakSpellStructure _returnvalue_5)) "NewEnumerator3")
        (if (== (.Spell (Utilities|Struct|BreakSpellStructure _returnvalue_5)) "/Game/Weapons/MagicAttacks/OfficialSpells/CombustionSpell/BP_Combustion.BP_Combustion_C")
          (return (.X (Math|Vector|BreakVector (* (/ (Transformation|GetActorScale3D SpellActor) 1e+01) (.SpellDamage (Utilities|Struct|BreakSpellStructure _returnvalue_5))))))
          (elif (> _returnvalue_4 1.0)
            (CallFunction|DrainHealth (.SpellDamage (Utilities|Struct|BreakSpellStructure _returnvalue_5)) _returnvalue_2)
            (return 0.0)
            (else
              (CallFunction|DrainHealth (* _returnvalue_4 (.SpellDamage (Utilities|Struct|BreakSpellStructure _returnvalue_5))) _returnvalue_2)
              (return 0.0))))
        (else
          (return (.SpellDamage (Utilities|Struct|BreakSpellStructure _returnvalue_5))))))))