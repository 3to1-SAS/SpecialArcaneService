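; Summoner enemy character that runs BT_Summoner, seeding its blackboard from DT_Enemies and instance settings.
; Capsule overlaps with spells or the sword reduce HP, with ScaleDamage using DT_Spells to scale charge spells, start timed health drain or trigger Pulse Wave stuns.
; Stun pauses the behavior tree and notifies the summon indicator.
; Death also notifies it, ragdolls with spell impulse, rolls a health pickup from the "Arcane" row, updates enemy count and optionally despawns.
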(event OnComponentBeginOverlap(CapsuleComponent)
  (params (OverlappedComponent :type Primitive%20Component%20Object%20Reference) (OtherActor :type Actor%20Object%20Reference) (OtherComp :type Primitive%20Component%20Object%20Reference) (OtherBodyIndex :type Integer) (bFromSweep :type Boolean) (SweepResult :type Hit%20Result%20Structure%20%28by%20ref%29))
  (bind _returnvalue (Utilities|GetClass OtherActor))
  (bind _self self)
  (bind _self_2 self)
  (bind _returnvalue_2 (AI|GetAIController _self_2))
  (bind _returnvalue_3 (AI|GetAIController _self))
  (bind _asbp_aicontroller (Utilities|Casting|CastToBP_AIController _returnvalue_3))
  (bind _asbp_aicontroller_2 (Utilities|Casting|CastToBP_AIController _returnvalue_2))
  (bind _behaviortree (Variables|/Game/NPC_Comp/BP_AIController.BP_AIController_C|GetBehaviorTree _asbp_aicontroller_2))
  ;[0.15 0.15 0.15 0.5] Calculates damage taken based on spell
  (if (Actor|ActorHasTag OtherActor "Spell")
    (bind _name (Default|GetRow _asbp_aicontroller _returnvalue))
    (bind _damage (CallFunction|ScaleDamage _name OtherActor))
    (Variables|Default|SetHP (- (Variables|Default|GetHP) _damage))
    ;[0.15 0.15 0.15 0.5] Destroys enemy when health is 0
    (Default|Damage _asbp_aicontroller (Game|Player|GetPlayerPawn 0) :!label _label)
    (if (<= (Variables|Default|GetHP) 0.0)
      (Utilities|FlowControl|DoOnce false
        (:Completed
          (bind _asbp_summon_indicator (Utilities|Casting|CastToBP_SummonIndicator (AI|Components|Blackboard|GetValueasObject (Variables|Default|GetBlackboard) (Variables|Default|GetSummonIndicator)))
            (:then
              (Default|EnemyKilled _asbp_summon_indicator))
            (:CastFailed
              _))
          (Physics|SetSimulatePhysics (Variables|Character|GetMesh) true)
          (CallFunction|GetYeeted OtherActor)
          (CallFunction|SpawnHealthup)
          (Components|DestroyComponent (Variables|Collision|GetCapsuleComponent))
          (Utilities|Array|Add (Variables|Actor|GetTags) "Dead")
          (Variables|/Game/FirstPerson/Blueprints/BP_FirstPersonPlayerController.BP_FirstPersonPlayerController_C|SetSouls (Variables|Default|GetPlayerController) 0)
          (AI|Logic|StopLogic _behaviortree "")
          (Default|UpdateEnemyCount (.AsBP%20First%20Person%20Game%20Mode (Utilities|Casting|CastToBP_FirstPersonGameMode (Game|GetGameMode))))
          (Utilities|FlowControl|Delay 1e+01)
          (if (Variables|Default|GetCanDespawn)
            (Game|AddComponentbyClass "/Game/FirstPerson/Blueprints/BP_TransitionComponent.BP_TransitionComponent_C")
            (Utilities|FlowControl|Delay 7.0)
            (Actor|DestroyActor)
            (else
              (Components|DestroyComponent _behaviortree))))))
    (elif (== _returnvalue "/Game/Weapons/MeleeAttacks/BP_Sword.BP_Sword_C")
      (Variables|Default|SetHP (- (Variables|Default|GetHP) 6e+02))
      (goto _label))))

(event Custom|SpawnHealthup
  (if (Variables|Default|GetHealthupSpawned)
    (Development|PrintString "Unlucky" :!label _label)
    (else
      (Variables|Default|SetHealthupSpawned true)
      (bind _returnvalue (Utilities|GetDataTableRow "/Game/DataTables/Enemies/DT_Enemies.DT_Enemies" "Arcane")
        (:then
          (if (== (Math|Random|RandomIntegerinRange 0 (.DropHealthChance (Utilities|Struct|BreakEnemiesStructure _returnvalue))) (.DropHealthChance (Utilities|Struct|BreakEnemiesStructure _returnvalue)))
            (Game|SpawnActorfromClass "/Game/Inventory/Loot/HealthUp.HealthUp_C" (Transformation|GetActorTransform) "AlwaysSpawn" "MultiplyWithRoot" 0 0)))
        (:RowNotFound
          (goto _label))))))

(event Custom|GetYeeted
  (params (Spell :type Actor%20Object%20Reference))
  (bind _mesh (Variables|Character|GetMesh))
  (bind _rootcomponent (Variables|/Script/Engine.Actor|GetRootComponent Spell))
  (bind _returnvalue (Transformation|GetWorldLocation _rootcomponent))
  (bind _returnvalue_2 (Math|Vector|GetForwardVector _rootcomponent))
  ;[0.15 0.15 0.15 0.5] Adds the impulse based on the spell that hit it
  (bind _spellref1 (CallFunction|UglyAhhhCheckSpell Spell))
  (bind _returnvalue_3 (Utilities|GetDataTableRow "/Game/DataTables/Spells/DT_Spells.DT_Spells" _spellref1)
    (:then
      (if (== (.Spell (Utilities|Struct|BreakSpellStructure _returnvalue_3)) "/Game/Weapons/MagicAttacks/OfficialSpells/CombustionSpell/BP_Combustion.BP_Combustion_C")
        (Class|PhysicsObjectBlueprintLibrary|ApplyRadialImpulse _mesh _returnvalue 1e+03 (.x (* (* (/ (Transformation|GetWorldScale _rootcomponent) 1e+01) (.Impulse (Utilities|Struct|BreakSpellStructure _returnvalue_3))) (- 1.0 (/ (Math|Vector|Distance(Vector) _returnvalue (Transformation|GetWorldLocation (Variables|Default|GetHeart))) 7.5e+02)))) "RIF_Constant" false 0.0 false 0.0 1.0)
        (else
          (Utilities|IsValid Spell
            (:Is%20Valid
              (Physics|AddImpulseatLocation _mesh (* (.Impulse (Utilities|Struct|BreakSpellStructure _returnvalue_3)) _returnvalue_2) _returnvalue_2 "None"))))))))

(event Custom|DrainHealth
  (params (HealthDrain :type Float%20%28double-precision%29) (TimesToDrain :type Integer))
  ;[0.15 0.15 0.15 0.5] Drains health over a period of time
  (AI|Components|Blackboard|SetValueasBool (Variables|Default|GetBlackboard) (Variables|Default|GetPoisoned) true)
  (Variables|/Script/Engine.CharacterMovementComponent|SetMaxWalkSpeed (Variables|Character|GetCharacterMovement) 3e+02)
  (bind _output_get (Variables|Default|SetTimesDrained 0))
  (if (and (< _output_get TimesToDrain) (> (Variables|Default|GetHP) 0.0)) :!label _label
    (Variables|Default|SetHP (- (Variables|Default|GetHP) (* (Variables|/Game/FirstPerson/Blueprints/BP_FirstPersonPlayerController.BP_FirstPersonPlayerController_C|GetDrainBuff%25 (.AsBP%20First%20Person%20Player%20Controller (Utilities|Casting|CastToBP_FirstPersonPlayerController (Game|GetPlayerController 0)))) HealthDrain)))
    (Development|PrintString "Damaged" true true "(R=0.000000,G=0.660000,B=1.000000,A=1.000000)" 2.5)
    (Variables|Default|SetTimesDrained (+ (Variables|Default|GetTimesDrained) 1))
    (Utilities|FlowControl|Delay 1.0)
    (goto _label)
    (else
      (if (> (Variables|Default|GetHP) 0.0)
        _
        (else
          (CallFunction|HealthDrained)))
      (AI|Components|Blackboard|SetValueasBool (Variables|Default|GetBlackboard) (Variables|Default|GetPoisoned) false))))

(event Custom|HealthDrained
  (bind _self self)
  (bind _returnvalue (AI|GetAIController _self))
  (bind _asbp_aicontroller (Utilities|Casting|CastToBP_AIController _returnvalue))
  (bind _behaviortree (Variables|/Game/NPC_Comp/BP_AIController.BP_AIController_C|GetBehaviorTree _asbp_aicontroller))
  ;[0.15 0.15 0.15 0.5] Destroys enemy when health is 0
  (if (<= (Variables|Default|GetHP) 0.0)
    (Utilities|FlowControl|DoOnce false
      (:Completed
        (bind _asbp_summon_indicator (Utilities|Casting|CastToBP_SummonIndicator (AI|Components|Blackboard|GetValueasObject (Variables|Default|GetBlackboard) (Variables|Default|GetSummonIndicator)))
          (:then
            (Default|EnemyKilled _asbp_summon_indicator))
          (:CastFailed
            _))
        (Physics|SetSimulatePhysics (Variables|Character|GetMesh) true)
        (CallFunction|GetYeeted (stale OnComponentBeginOverlap(CapsuleComponent) OtherActor))
        (CallFunction|SpawnHealthup)
        (Components|DestroyComponent (Variables|Collision|GetCapsuleComponent))
        (Utilities|Array|Add (Variables|Actor|GetTags) "Dead")
        (Variables|/Game/FirstPerson/Blueprints/BP_FirstPersonPlayerController.BP_FirstPersonPlayerController_C|SetSouls (Variables|Default|GetPlayerController) 0)
        (AI|Logic|StopLogic _behaviortree "")
        (Default|UpdateEnemyCount (.AsBP%20First%20Person%20Game%20Mode (Utilities|Casting|CastToBP_FirstPersonGameMode (Game|GetGameMode))))
        (Utilities|FlowControl|Delay 1e+01)
        (if (Variables|Default|GetCanDespawn)
          (Game|AddComponentbyClass "/Game/FirstPerson/Blueprints/BP_TransitionComponent.BP_TransitionComponent_C")
          (Utilities|FlowControl|Delay 7.0)
          (Actor|DestroyActor)
          (else
            (Components|DestroyComponent _behaviortree)))))))

(event Custom|Stun
  (params (Origin :type Vector) (Impulse :type Float%20%28double-precision%29))
  ;[0.15 0.15 0.15 0.5] Stuns enemy for a short amount of time
  (Character|LaunchCharacter (* Impulse (Math|Vector|GetUnitDirection(Vector) Origin (Transformation|GetActorLocation))) false false)
  (bind _asbp_aicontroller (Utilities|Casting|CastToBP_AIController (AI|GetAIController self)))
  (Variables|/Game/NPC_Comp/BP_AIController.BP_AIController_C|SetStunned _asbp_aicontroller true)
  (AI|Logic|StopLogic (Variables|/Game/NPC_Comp/BP_AIController.BP_AIController_C|GetBehaviorTree _asbp_aicontroller) "")
  (Default|EnemyKilled (.AsBP%20Summon%20Indicator (Utilities|Casting|CastToBP_SummonIndicator (AI|Components|Blackboard|GetValueasObject (Variables|Default|GetBlackboard) (Variables|Default|GetSummonIndicator)))))
  (bind _returnvalue (Utilities|GetDataTableRow "/Game/DataTables/Enemies/DT_Enemies.DT_Enemies" "Summoner")
    (:then
      (Utilities|FlowControl|Delay (.PulseWaveStunTime (Utilities|Struct|BreakEnemiesStructure _returnvalue)))
      (Class|BrainComponent|RestartLogic (Variables|/Game/NPC_Comp/BP_AIController.BP_AIController_C|GetBehaviorTree _asbp_aicontroller))
      (Variables|/Game/NPC_Comp/BP_AIController.BP_AIController_C|SetStunned _asbp_aicontroller false))))

(event EventBeginPlay
  (bind _returnvalue (AI|GetBlackboard 0))
  ;[0.15 0.15 0.15 0.5] Sets all necessary blackboard values
  (Variables|Default|SetPlayerController (.AsBP%20First%20Person%20Player%20Controller (Utilities|Casting|CastToBP_FirstPersonPlayerController (Game|GetPlayerController 0))))
  (bind _asbp_aicontroller (Utilities|Casting|CastToBP_AIController (AI|GetAIController self))
    (:then
      (Variables|/Game/NPC_Comp/BP_AIController.BP_AIController_C|SetBehaviorTreeAsset _asbp_aicontroller "/Game/Enemies/Summoner/BT_Summoner.BT_Summoner")
      (Variables|/Game/NPC_Comp/BP_AIController.BP_AIController_C|SetDetectionRadius _asbp_aicontroller (Variables|Default|GetDetectionRange))
      (Utilities|FlowControl|DelayUntilNextTick)
      (Variables|Default|SetBlackboard _returnvalue)
      (Class|BlackboardComponent|SetValueasName _returnvalue (Variables|Default|GetDataTableRow) "Summoner")
      (bind _returnvalue_2 (Utilities|GetDataTableRow "/Game/DataTables/Enemies/DT_Enemies.DT_Enemies" "Summoner")
        (:then
          (Variables|Default|SetHP (.MaxHP (Utilities|Struct|BreakEnemiesStructure _returnvalue_2)))
          (Variables|Default|SetSoul%20Drop (.SoulDrop (Utilities|Struct|BreakEnemiesStructure _returnvalue_2)))
          (AI|Components|Blackboard|SetValueasFloat (Variables|Default|GetBlackboard) (Variables|Default|GetSpellCooldown) (.AttackCooldown (Utilities|Struct|BreakEnemiesStructure _returnvalue_2)))
          (AI|Components|Blackboard|SetValueasFloat (Variables|Default|GetBlackboard) (Variables|Default|GetLOSTime) (.ChaseTime (Utilities|Struct|BreakEnemiesStructure _returnvalue_2)))
          (AI|Components|Blackboard|SetValueasFloat (Variables|Default|GetBlackboard) (Variables|Default|GetAttackRange) (.AttackRange (Utilities|Struct|BreakEnemiesStructure _returnvalue_2)))
          (AI|Components|Blackboard|SetValueasEnum (Variables|Default|GetBlackboard) (Variables|Default|GetPatrols) (Variables|Default|GetPatrolBehavior))
          (AI|Components|Blackboard|SetValueasFloat (Variables|Default|GetBlackboard) (Variables|Default|GetRadius) (Variables|Default|GetPatrolRadius))
          (AI|Components|Blackboard|SetValueasBool (Variables|Default|GetBlackboard) (Variables|Default|GetBBCanHear) (Variables|Default|GetCanHear))
          (AI|Components|Blackboard|SetValueasEnum (Variables|Default|GetBlackboard) (Variables|Default|GetBBSpell) (Variables|Default|GetSecondarySpell))
          (AI|Components|Blackboard|SetValueasEnum (Variables|Default|GetBlackboard) (Variables|Default|GetBBSecondaryBehavior) (Variables|Default|GetSecondaryBehavior))
          (AI|Components|Blackboard|SetValueasFloat (Variables|Default|GetBlackboard) (Variables|Default|GetBBSecondaryCooldown) (Variables|Default|GetSecondaryCooldown))
          (AI|Components|Blackboard|SetValueasFloat (Variables|Default|GetBlackboard) (Variables|Default|GetBBSightRadius) (Variables|Default|GetSightRadius)))))
    (:CastFailed
      (Development|PrintString "Cast failed"))))

(fn ConstructionScript)

(fn UglyAhhhCheckSpell
  (params (Spell :type Actor%20Object%20Reference))
  (bind _returnvalue (Utilities|GetClass Spell))
  (bind _outrownames (DataTable|GetDataTableRowNames "/Game/DataTables/Spells/DT_Spells.DT_Spells"))
  (bind _array_element (Utilities|Array|ForEachLoopwithBreak _outrownames :!label _label)
    (:LoopBody
      (bind _returnvalue_2 (Utilities|GetDataTableRow "/Game/DataTables/Spells/DT_Spells.DT_Spells" _array_element)
        (:then
          (if (== (.Spell (Utilities|Struct|BreakSpellStructure _returnvalue_2)) _returnvalue)
            (LocalVariables|SetSpellFound true)
            (LocalVariables|SetSpellRef _array_element)
            (goto _label Break)))))
    (:Completed
      (if (LocalVariables|GetSpellFound)
        (return (LocalVariables|GetSpellRef))
        (else
          (Development|PrintString (Utilities|GetClassDisplayName _returnvalue)))))))

(fn ScaleDamage
  (params (SpellRow :type Name) (SpellActor :type Actor%20Object%20Reference))
  (bind _returnvalue (Math|Random|RandomIntegerinRange 8 12))
  ;[0.15 0.15 0.15 0.5] Checks if the spell is a charge spell. If so, scales its damage accordingly. If Toxic Thorn, initiates health drain.
  (bind _returnvalue_2 (Utilities|GetDataTableRow "/Game/DataTables/Spells/DT_Spells.DT_Spells" SpellRow)
    (:then
      (if (Utilities|Enum|Equal(Enum) (.SpellType (Utilities|Struct|BreakSpellStructure _returnvalue_2)) "NewEnumerator3")
        (if (== (.Spell (Utilities|Struct|BreakSpellStructure _returnvalue_2)) "/Game/Weapons/MagicAttacks/OfficialSpells/CombustionSpell/BP_Combustion.BP_Combustion_C")
          (return (.X (Math|Vector|BreakVector (* (/ (Transformation|GetActorScale3D SpellActor) 1e+01) (.SpellDamage (Utilities|Struct|BreakSpellStructure _returnvalue_2))))))
          (elif (> (/ (- (.Lifetime (Utilities|Struct|BreakSpellStructure _returnvalue_2)) (Actor|GetLifeSpan SpellActor)) 3.0) 1.0)
            (CallFunction|DrainHealth (.SpellDamage (Utilities|Struct|BreakSpellStructure _returnvalue_2)) _returnvalue)
            (return 0.0)
            (else
              (CallFunction|DrainHealth (* (/ (- (.Lifetime (Utilities|Struct|BreakSpellStructure _returnvalue_2)) (Actor|GetLifeSpan SpellActor)) 3.0) (.SpellDamage (Utilities|Struct|BreakSpellStructure _returnvalue_2))) _returnvalue)
              (return 0.0))))
        (else
          (if (== (.Spell (Utilities|Struct|BreakSpellStructure _returnvalue_2)) "/Game/Weapons/MagicAttacks/OfficialSpells/PulseWave/BP_PulseWave.BP_PulseWave_C")
            (CallFunction|Stun (Transformation|GetActorLocation SpellActor) (.Impulse (Utilities|Struct|BreakSpellStructure _returnvalue_2))))
          (return (.SpellDamage (Utilities|Struct|BreakSpellStructure _returnvalue_2))))))))