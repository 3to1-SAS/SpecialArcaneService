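; Summoner indicator actor that marks a spot and spawns a random enemy there after a delay.
; On BeginPlay it waits, then checks that the owner enemy's capsule component is valid before spawning from EnemyClasses, slightly raised and facing the player.
; Shortly after spawning, it calls Damage on the new enemy's AI controller with the player pawn, then destroys itself.
; EnemyKilled or a failed owner check destroys it without spawning.
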(event Custom|EnemyKilled
  (Actor|DestroyActor))

(event EventBeginPlay
  (bind _returnvalue (Transformation|GetActorLocation))
  (bind _returnvalue_2 (+ (.z _returnvalue) 1e+02))
  ;[0.15 0.15 0.15 0.5] Spawns a random enemy after 5 seconds
  (Utilities|FlowControl|DelayUntilNextTick)
  (Utilities|FlowControl|Delay (Variables|Default|GetDelay))
  (Utilities|IsValid (Actor|GetComponentbyClass (Variables|Default|GetOwnerEnemy) "/Script/Engine.CapsuleComponent")
    (:Is%20Valid
      (bind _returnvalue_3 (Game|SpawnActorfromClass (.OutItem (Utilities|Array|Random (Variables|Default|GetEnemyClasses))) (Math|Transform|MakeTransform (Math|Vector|MakeVector (.x _returnvalue) (.y _returnvalue) _returnvalue_2) (Math|Rotator|FindLookatRotation (Math|Vector|MakeVector (.x _returnvalue) (.y _returnvalue) _returnvalue_2) (Transformation|GetActorLocation (Game|Player|GetPlayerPawn 0))) "1.000000,1.000000,1.000000") "Undefined" "MultiplyWithRoot" 0 0))
      (Utilities|FlowControl|Delay 0.2)
      (Default|Damage (.AsBP%20AIController (Utilities|Casting|CastToBP_AIController (AI|GetAIController _returnvalue_3))) (Game|Player|GetPlayerPawn 0))
      (Actor|DestroyActor))
    (:Is%20Not%20Valid
      (Actor|DestroyActor))))

(fn ConstructionScript)