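; Tank enemy that runs BT_Tank, seeding its health and blackboard from the "Tank" row of DT_Enemies and its own patrol settings.
; Spell overlaps deal DT_Spells damage, scaled by actor size for one spell type, while the sword deals fixed damage.
; Death ragdolls it with a spell-based impulse (radial for Combustion), rolls a health drop using the "Knight" row, updates the enemy count and destroys it after a delay.
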(event OnComponentBeginOverlap(CapsuleComponent)
  (params (OverlappedComponent :type Primitive%20Component%20Object%20Reference) (OtherActor :type Actor%20Object%20Reference) (OtherComp :type Primitive%20Component%20Object%20Reference) (OtherBodyIndex :type Integer) (bFromSweep :type Boolean) (SweepResult :type Hit%20Result%20Structure%20%28by%20ref%29))
  (bind _returnvalue (Utilities|GetClass OtherActor))
  (bind _self self)
  (bind _returnvalue_2 (AI|GetAIController _self))
  (bind _asbp_aicontroller (Utilities|Casting|CastToBP_AIController _returnvalue_2))
  ;[0.15 0.15 0.15 0.5] Calculates damage taken based on spell
  (if (Actor|ActorHasTag OtherActor "Spell")
    (bind _name (Default|GetRow _asbp_aicontroller _returnvalue))
    (bind _damage (CallFunction|ScaleDamage _name OtherActor))
    (Variables|Default|SetHP (- (Variables|Default|GetHP) _damage))
    (Default|Damage _asbp_aicontroller (Game|Player|GetPlayerPawn 0) :!label _label)
    ;[0.15 0.15 0.15 0.5] Destroys enemy when health is 0
    (if (<= (Variables|Default|GetHP) 0.0)
      (Physics|SetSimulatePhysics (Variables|Character|GetMesh) true)
      (CallFunction|GetYeeted OtherActor)
      (CallFunction|SpawnHealthup)
      (Components|DestroyComponent (Variables|Collision|GetCapsuleComponent))
      (AI|Logic|StopLogic (Variables|/Game/NPC_Comp/BP_AIController.BP_AIController_C|GetBehaviorTree (.AsBP%20AIController (Utilities|Casting|CastToBP_AIController (AI|GetAIController self)))) "")
      (Default|UpdateEnemyCount (.AsBP%20First%20Person%20Game%20Mode (Utilities|Casting|CastToBP_FirstPersonGameMode (Game|GetGameMode))))
      (Utilities|FlowControl|Delay 3e+01)
      (Actor|DestroyActor))
    (elif (== _returnvalue "/Game/Weapons/MeleeAttacks/BP_Sword.BP_Sword_C")
      (Variables|Default|SetHP (- (Variables|Default|GetHP) 6e+02))
      (goto _label))))

(event Custom|SpawnHealthup
  (if (Variables|Default|GetHealthupSpawned)
    (Development|PrintString "Unlucky" true true "(R=1.000000,G=0.000000,B=0.026847,A=1.000000)")
    (else
      (Variables|Default|SetHealthupSpawned true)
      (bind _returnvalue (Utilities|GetDataTableRow "/Game/DT_EnemiesCSV.DT_EnemiesCSV" "Knight")
        (:then
          (if (== (Math|Random|RandomIntegerinRange 0 (.DropHealthChance (Utilities|Struct|BreakEnemiesStructure _returnvalue))) (.DropHealthChance (Utilities|Struct|BreakEnemiesStructure _returnvalue)))
            (Game|SpawnActorfromClass "/Game/Inventory/Loot/HealthUp.HealthUp_C" (Transformation|GetActorTransform) "AlwaysSpawn" "MultiplyWithRoot" 0 0)))))))

(event Custom|GetYeeted
  (params (Spell :type Actor%20Object%20Reference))
  (bind _mesh (Variables|Character|GetMesh))
  (bind _rootcomponent (Variables|/Script/Engine.Actor|GetRootComponent Spell))
  (bind _returnvalue (Transformation|GetWorldLocation _rootcomponent))
  (bind _returnvalue_2 (Math|Vector|GetForwardVector _rootcomponent))
  ;[0.15 0.15 0.15 0.5] Adds the impulse based on the spell that hit it. If it's the combustion spell, it will apply forces different
  (bind _spellref1 (CallFunction|UglyAhhhCheckSpell Spell))
  (bind _returnvalue_3 (Utilities|GetDataTableRow "/Game/DataTables/Spells/DT_Spells.DT_Spells" _spellref1)
    (:then
      (if (== (.Spell (Utilities|Struct|BreakSpellStructure _returnvalue_3)) "/Game/Weapons/MagicAttacks/OfficialSpells/CombustionSpell/BP_Combustion.BP_Combustion_C")
        (Class|PhysicsObjectBlueprintLibrary|ApplyRadialImpulse _mesh _returnvalue 1e+03 (.x (* (* (/ (Transformation|GetWorldScale _rootcomponent) 1e+01) (.Impulse (Utilities|Struct|BreakSpellStructure _returnvalue_3))) (- 1.0 (/ (Math|Vector|Distance(Vector) _returnvalue (Transformation|GetWorldLocation (Variables|Default|GetHeart))) 7.5e+02)))) "RIF_Constant" false 0.0 false 0.0 1.0)
        (else
          (Physics|AddImpulseatLocation _mesh (* (.Impulse (Utilities|Struct|BreakSpellStructure _returnvalue_3)) _returnvalue_2) _returnvalue_2 "None"))))))

(event EventBeginPlay
  (bind _returnvalue (AI|GetBlackboard 0))
  (bind _self self)
  (bind _returnvalue_2 (AI|GetAIController _self))
  (bind _asbp_aicontroller (Utilities|Casting|CastToBP_AIController _returnvalue_2))
  ;[0.15 0.15 0.15 0.5] Sets The Data Table Row, Spell Cooldown, And Line of Sight Time On Blackboard
  (Variables|/Game/NPC_Comp/BP_AIController.BP_AIController_C|SetBehaviorTreeAsset _asbp_aicontroller "/Game/Enemies/Tank/BT_Tank.BT_Tank")
  (Variables|/Game/NPC_Comp/BP_AIController.BP_AIController_C|SetDetectionRadius _asbp_aicontroller (Variables|Default|GetDetectionRange))
  (Utilities|FlowControl|DelayUntilNextTick)
  (Class|BlackboardComponent|SetValueasName _returnvalue (Variables|Default|GetDataTableRow) "Tank")
  (bind _returnvalue_3 (Utilities|GetDataTableRow "/Game/DataTables/Enemies/DT_Enemies.DT_Enemies" "Tank")
    (:then
      (Variables|Default|SetHP (.maxhp _returnvalue_3))
      (AI|Components|Blackboard|SetValueasFloat _returnvalue (Variables|Default|GetSpellCooldown) (.attackcooldown _returnvalue_3))
      (AI|Components|Blackboard|SetValueasFloat _returnvalue (Variables|Default|GetLOSTime) (.chasetime _returnvalue_3))
      (AI|Components|Blackboard|SetValueasEnum _returnvalue (Variables|Default|GetPatrols) (Variables|Default|GetPatrolBehavior))
      (AI|Components|Blackboard|SetValueasFloat _returnvalue (Variables|Default|GetRadius) (Variables|Default|GetPatrolRadius))
      (AI|Components|Blackboard|SetValueasBool _returnvalue (Variables|Default|GetBBCanHear) (Variables|Default|GetCanHear)))))

(fn ConstructionScript)

(fn UglyAhhhCheckSpell
  (params (Spell :type Actor%20Object%20Reference))
  (bind _returnvalue (Utilities|GetClass Spell))
  (bind _outrownames (DataTable|GetDataTableRowNames "/Game/DataTables/Spells/DT_Spells.DT_Spells"))
  (bind _array_element (Utilities|Array|ForEachLoopwithBreak _outrownames :!label _label)
    (:LoopBody
      (bind _returnvalue_2 (Utilities|GetDataTableRow "/Game/DataTables/Spells/DT_Spells.DT_Spells" _array_element)
        (:then
          (if (== (.Spell (Utilities|Struct|BreakSpellStructure _returnvalue_2)) _returnvalue)
            (LocalVariables|SetSpellFound true)
            (LocalVariables|SetSpellRef _array_element)
            (goto _label Break)))))
    (:Completed
      (if (LocalVariables|GetSpellFound)
        (return (LocalVariables|GetSpellRef))
        (else
          (Development|PrintString (Utilities|GetClassDisplayName _returnvalue)))))))

(fn ScaleDamage
  (params (SpellRow :type Name) (SpellActor :type Actor%20Object%20Reference))
  ;[0.15 0.15 0.15 0.5] Checks if the spell is a charge spell. If so, scales its damage accordingly.
  (bind _returnvalue (Utilities|GetDataTableRow "/Game/DataTables/Spells/DT_Spells.DT_Spells" SpellRow)
    (:then
      (if (Utilities|Enum|Equal(Enum) (.SpellType (Utilities|Struct|BreakSpellStructure _returnvalue)) "NewEnumerator3")
        (return (.X (Math|Vector|BreakVector (* (/ (Transformation|GetActorScale3D SpellActor) 1e+01) (.SpellDamage (Utilities|Struct|BreakSpellStructure _returnvalue))))))
        (else
          (return (.SpellDamage (Utilities|Struct|BreakSpellStructure _returnvalue))))))))