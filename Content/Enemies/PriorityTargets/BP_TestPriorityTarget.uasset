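; BP_TestPriorityTarget is an enemy that loses HP when spells or the sword overlap its capsule.
; Spell damage comes from DT_Spells using a row name mapped from the spell class, while sword hits deal fixed damage.
; At zero HP it sometimes spawns an actor carrying random mana, then destroys itself.
; Its Priority flag adds a tag and selects which game mode update death triggers: priority target or enemy count.
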(event OnComponentBeginOverlap(Capsule)
  (params (OverlappedComponent :type Primitive%20Component%20Object%20Reference) (OtherActor :type Actor%20Object%20Reference) (OtherComp :type Primitive%20Component%20Object%20Reference) (OtherBodyIndex :type Integer) (bFromSweep :type Boolean) (SweepResult :type Hit%20Result%20Structure%20%28by%20ref%29))
  (bind _returnvalue (Game|GetGameMode))
  (bind _returnvalue_2 (Utilities|GetClass OtherActor))
  (bind _asbp_first_person_game_mode (Utilities|Casting|CastToBP_FirstPersonGameMode _returnvalue))
  ;[0.15 0.15 0.15 0.5] Reduce enemy HP on hit based on spell or sword
  (if (Actor|ActorHasTag OtherActor "Spell")
    (bind _returnname (CallFunction|GetRowName _returnvalue_2))
    (bind _returnvalue_3 (Utilities|GetDataTableRow "/Game/DataTables/Spells/DT_Spells.DT_Spells" _returnname)
      (:then
        (Variables|Default|SetHP (- (Variables|Default|GetHP) (.SpellDamage (Utilities|Struct|BreakSpellStructure _returnvalue_3))))
        ;[0.15 0.15 0.15 0.5] Destroy enemy when HP reaches 0
        (if (<= (Variables|Default|GetHP) 0.0) :!label _label
          (if (>= (Math|Random|RandomFloatinRange 0.0 1e+02) 75.0)
            (bind _returnvalue_4 (Game|SpawnActorfromClass 0 (Transformation|GetActorTransform) "Undefined" "MultiplyWithRoot" 0 0))
            (Variables|Default|SetManaValue _returnvalue_4 (Math|Random|RandomFloatinRange 3e+02 1.2e+03)))
          (Actor|DestroyActor)
          (if (Variables|Default|GetPriority)
            (Default|UpdatePriorityTarget _asbp_first_person_game_mode "Big Enemy")
            (else
              (Default|UpdateEnemyCount _asbp_first_person_game_mode))))))
    (elif (== _returnvalue_2 "/Game/Weapons/MeleeAttacks/BP_Sword.BP_Sword_C")
      (Variables|Default|SetHP (- (Variables|Default|GetHP) 6e+02))
      (goto _label))))

(event EventBeginPlay
  (if (Variables|Default|GetPriority)
    (Utilities|Array|Add (Variables|Actor|GetTags) "priority")))

(fn ConstructionScript)

(fn GetRowName
  (params (Class :type Actor%20Class%20Reference))
  (if (== Class 0)
    (return "BasicSpell")
    (elif (== Class 0)
      (return "RapidSpell")
      (elif (== Class 0)
        (return "ExplosiveSpell")))))