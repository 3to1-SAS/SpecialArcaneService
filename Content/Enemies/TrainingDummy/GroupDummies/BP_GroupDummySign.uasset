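; BP_GroupDummySign is a training dummy sign that displays a running damage total, apparently for a group of dummies.
; On BeginPlay it caches its widget as UI_SignText.
; UpdateDamage adds incoming damage to the total, writes the rounded value to the text and restarts a reset timer.
; When no new damage arrives before the timer fires, ResetDamage zeroes the total and refreshes the display.
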(event Custom|UpdateDamage
  (params (Damage :type Float%20%28double-precision%29))
  ;[0.15 0.15 0.15 0.5] Updates the text on the widget
  (Utilities|Time|ClearandInvalidateTimerbyHandle (Variables|Default|GetResetTimer))
  (bind _output_get (Variables|Default|SetTotalDamage (+ (Variables|Default|GetTotalDamage) Damage)))
  (Variables|/Script/UMG.TextBlock|SetText (Variables|/Game/Enemies/TrainingDummy/UI_SignText.UI_SignText_C|GetDamageText (Variables|Default|GetText)) (Utilities|Text|ToText(Integer) (Math|Float|Round _output_get)))
  (bind _returnvalue (Utilities|Time|SetTimerbyEvent (delegate Custom|ResetDamage) 5.0))
  (Variables|Default|SetResetTimer _returnvalue))

(event Custom|ResetDamage
  (bind _output_get (Variables|Default|SetTotalDamage 0.0))
  (Variables|/Script/UMG.TextBlock|SetText (Variables|/Game/Enemies/TrainingDummy/UI_SignText.UI_SignText_C|GetDamageText (Variables|Default|GetText)) (Utilities|Text|ToText(Integer) (Math|Float|Round _output_get))))

(event EventBeginPlay
  ;[0.15 0.15 0.15 0.5] Sets the widget as a variable
  (Variables|Default|SetText (.AsUI%20Sign%20Text (Utilities|Casting|CastToUI_SignText (UserInterface|GetWidget (Variables|Default|GetWidget))))))

(fn ConstructionScript)