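; AI controller for the Fallen Angel final boss, running its behavior trees and managing the fight's start and phase change.
; On possess it starts the phase 1 tree and loads stun time from a data table.
; Fight start focuses the player and creates the boss HP bar; perception updates line of sight.
; Phase 2 swaps trees, destroys thrown spears, removes the shield bar, resets the damage multiplier and stuns the boss.
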(event OnTargetPerceptionUpdated(AIPerception)
  (params (Actor :type Actor%20Object%20Reference) (Stimulus :type AI%20Stimulus%20Structure))
  ;[0.15 0.15 0.15 0.5] Checks line of sight to player
  (if (Actor|ActorHasTag Actor "Player")
    (AI|Components|Blackboard|SetValueasBool (Variables|Default|GetBlackboard) (Variables|Default|GetHasLOS) (Controller|LineOfSightTo Actor "0, 0, 0" false))))

(event Custom|BossFightStart
  (bind _returnvalue (Game|Player|GetPlayerPawn 0))
  (bind _blackboard (Variables|Default|GetBlackboard))
  ;[0.15 0.15 0.15 0.5] Sets blackboard values to begin boss fight
  (AI|Components|Blackboard|SetValueasBool _blackboard (Variables|Default|GetAttackingPlayer) true)
  (AI|Components|Blackboard|SetValueasObject _blackboard (Variables|Default|GetPlayerActor) _returnvalue)
  (AI|SetFocus _returnvalue)
  (bind _returnvalue_2 (UserInterface|CreateWidget "/Game/UIWidgets/BossHPBar.BossHPBar_C"))
  (UserInterface|Viewport|AddtoViewport _returnvalue_2 0)
  (Variables|/Game/Enemies/FallenAngel/BP_FallenAngel.BP_FallenAngel_C|SetHPBar (.AsBP%20Fallen%20Angel (Utilities|Casting|CastToBP_FallenAngel (Pawn|GetControlledPawn))) _returnvalue_2))

(event Custom|SpearThrown
  (AI|Components|Blackboard|SetValueasBool (Variables|Default|GetBlackboard) (Variables|Default|GetSpearHit) true))

(event Custom|Phase2
  (bind _returnvalue (Pawn|GetControlledPawn))
  (bind _returnvalue_2 (Pawn|GetControlledPawn))
  (bind _asbp_fallen_angel (Utilities|Casting|CastToBP_FallenAngel _returnvalue))
  (bind _asbp_fallen_angel_2 (Utilities|Casting|CastToBP_FallenAngel _returnvalue_2))
  (bind _hpbar (Variables|/Game/Enemies/FallenAngel/BP_FallenAngel.BP_FallenAngel_C|GetHPBar _asbp_fallen_angel))
  ;[0.15 0.15 0.15 0.5] Runs the phase 2 behavior tree once the second phase begins
  (AI|Logic|StopLogic (Variables|Default|GetBehaviorTree) "")
  (AI|RunBehaviorTree "/Game/Enemies/FallenAngel/BehaviorTrees/BT_FallenAngelPhase2.BT_FallenAngelPhase2")
  (Variables|/Game/Enemies/FallenAngel/BP_FallenAngel.BP_FallenAngel_C|SetPhase2 _asbp_fallen_angel true)
  (bind _outactors (Actor|GetAllActorsOfClass "/Game/Enemies/FallenAngel/Attacks/BP_SpearThrow.BP_SpearThrow_C"))
  (for _array_element _outactors
    (Actor|DestroyActor _array_element))
  (Class|ProgressBar|SetFillColorandOpacity (Variables|/Game/UIWidgets/BossHPBar.BossHPBar_C|GetHPBar _hpbar) "(R=1.000000,G=0.000000,B=0.002428,A=1.000000)")
  (Widget|RemovefromParent (Variables|/Game/UIWidgets/BossHPBar.BossHPBar_C|GetShieldBar _hpbar))
  (Variables|/Game/Enemies/FallenAngel/BP_FallenAngel.BP_FallenAngel_C|SetDamageMultiplier _asbp_fallen_angel_2 1.0)
  (Default|Stun _asbp_fallen_angel_2 0.0))

(event EventPossess
  (params (PossessedPawn :type Pawn%20Object%20Reference))
  (bind _blackboard (Variables|Default|GetBlackboard))
  ;[0.15 0.15 0.15 0.5] Runs the behavior tree and sets self actor on blackboard
  (AI|RunBehaviorTree "/Game/Enemies/FallenAngel/BehaviorTrees/BT_FallenAngel.BT_FallenAngel")
  (AI|Components|Blackboard|SetValueasObject _blackboard (Variables|Default|GetSelfActor) PossessedPawn)
  (bind _returnvalue (Utilities|GetDataTableRow "/Game/DataTables/Enemies/FinalBoss/DT_FinalBoss.DT_FinalBoss" "FallenAngel")
    (:then
      (AI|Components|Blackboard|SetValueasFloat _blackboard (Variables|Default|GetStunTime) (.StunTime (Utilities|Struct|BreakFinalBossStructure _returnvalue))))))

(fn ConstructionScript)