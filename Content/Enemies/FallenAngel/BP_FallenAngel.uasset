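; Final boss Fallen Angel, which loads its stats from DT_FinalBoss and takes hits through capsule overlaps.
; Spell damage is looked up by class in DT_Spells and scaled by player buffs and charge, with drains pausing movement and AI.
; In phase 1, hits trigger an orb beam, force-field overlay and HP regeneration.
; In phase 2, zero HP waits for the CanDie blackboard flag, then kills remaining enemies and stops AI.
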(event OnComponentBeginOverlap(CapsuleComponent)
  (params (OverlappedComponent :type Primitive%20Component%20Object%20Reference) (OtherActor :type Actor%20Object%20Reference) (OtherComp :type Primitive%20Component%20Object%20Reference) (OtherBodyIndex :type Integer) (bFromSweep :type Boolean) (SweepResult :type Hit%20Result%20Structure%20%28by%20ref%29))
  (bind _returnvalue (Utilities|GetClass OtherActor))
  (bind _self self)
  (bind _hpbar (Variables|Default|GetHPBar))
  (bind _maxhp (Variables|Default|GetMaxHP))
  (bind _returnvalue_2 (AI|GetAIController _self))
  (bind _shieldbar (Variables|/Game/UIWidgets/BossHPBar.BossHPBar_C|GetShieldBar _hpbar))
  (bind _asbp_fallen_angel_controller (Utilities|Casting|CastToBP_FallenAngelController _returnvalue_2))
  ;[0.15 0.15 0.15 0.5] Calculates damage taken based on spell
  (if (Actor|ActorHasTag OtherActor "Spell")
    (bind _name (CallFunction|GetRow _returnvalue))
    (if (== _name "Bolt!Strike")
      (Variables|Default|SetHP (- (Variables|Default|GetHP) (* (* (.BoltStrikeDamage (Utilities|Struct|BreakFinalBossStructure (Variables|Default|GetDataTableRow))) (Variables|/Game/FirstPerson/Blueprints/BP_FirstPersonPlayerController.BP_FirstPersonPlayerController_C|GetDrainBuff%25 (.AsBP%20First%20Person%20Player%20Controller (Utilities|Casting|CastToBP_FirstPersonPlayerController (Game|GetPlayerController 0))))) (Variables|Default|GetDamageMultiplier))))
      (else
        (bind _damage (CallFunction|ScaleDamage _name OtherActor))
        (bind _output_get (Variables|Default|SetHP (- (Variables|Default|GetHP) (* _damage (Variables|Default|GetDamageMultiplier)))))))
    (if (Variables|Default|GetPhase2) :!label _label
      ;[0.15 0.15 0.15 0.5] Kills the boss when HP reaches 0
      (Progress|SetPercent (Variables|/Game/UIWidgets/BossHPBar.BossHPBar_C|GetHPBar _hpbar) (/ (Variables|Default|GetHP) (Variables|Default|GetMaxHP)))
      (if (<= _output_get 0.0)
        (if (ScalableFloat|GetValueasBool (Variables|Default|GetBlackboard) (Variables|Default|GetCanDie)) :!label _label_2
          (bind _outactors (Actor|GetAllActorsOfClass "/Game/Enemies/FallenAngel/Attacks/Summon/BP_FallenAngelSummon.BP_FallenAngelSummon_C"))
          (for _array_element _outactors
            (Variables|/Game/Enemies/FallenAngel/Attacks/Summon/BP_FallenAngelSummon.BP_FallenAngelSummon_C|SetHP _array_element 0.0)
            (Default|HealthDrained _array_element))
          (bind _outactors_2 (Actor|GetAllActorsOfClass "/Game/Enemies/Arcane/BP_Arcane.BP_Arcane_C"))
          ;[0.15 0.01218 0.01555 0.5] Kills all enemies once boss dies
          (for _array_element_2 _outactors_2
            (Variables|/Game/Enemies/Arcane/BP_Arcane.BP_Arcane_C|SetCanDespawn _array_element_2 false)
            (Variables|/Game/Enemies/Arcane/BP_Arcane.BP_Arcane_C|SetHP _array_element_2 0.0)
            (Default|HealthDrained _array_element_2))
          (bind _outactors_3 (Actor|GetAllActorsOfClass "/Game/Enemies/Knight/BP_Knight.BP_Knight_C"))
          (for _array_element_3 _outactors_3
            (Variables|/Game/Enemies/Knight/BP_Knight.BP_Knight_C|SetCanDespawn _array_element_3 false)
            (Variables|/Game/Enemies/Knight/BP_Knight.BP_Knight_C|SetHP _array_element_3 0.0)
            (Default|HealthDrained _array_element_3))
          (for _array_element_4 (Variables|Default|GetTanks)
            (Variables|/Game/Enemies/Tank/BP_Tank.BP_Tank_C|SetCanDespawn _array_element_4 false)
            (Variables|/Game/Enemies/Tank/BP_Tank.BP_Tank_C|SetHP _array_element_4 0.0)
            (Default|HealthDrained _array_element_4))
          (for _array_element_5 (Variables|Default|GetSummoners)
            (Variables|/Game/Enemies/Summoner/BP_Summoner.BP_Summoner_C|SetCanDespawn _array_element_5 false)
            (Variables|/Game/Enemies/Summoner/BP_Summoner.BP_Summoner_C|SetHP _array_element_5 0.0)
            (Default|HealthDrained _array_element_5))
          (for _array_element_6 (Variables|Default|GetProtectors)
            (Variables|/Game/Enemies/Protector/BP_Protector.BP_Protector_C|SetCanDespawn _array_element_6 false)
            (Variables|/Game/Enemies/Protector/BP_Protector.BP_Protector_C|SetHP _array_element_6 0.0)
            (Default|HealthDrained _array_element_6))
          (Widget|RemovefromParent (Variables|Default|GetHPBar))
          (Components|DestroyComponent (Variables|Collision|GetCapsuleComponent))
          (AI|Logic|StopLogic (Variables|/Game/Enemies/FallenAngel/BP_FallenAngelController.BP_FallenAngelController_C|GetBehaviorTree _asbp_fallen_angel_controller) "")
          (Variables|/Game/Enemies/FallenAngel/BP_FallenAngelController.BP_FallenAngelController_C|SetDead _asbp_fallen_angel_controller true)
          (else
            (Utilities|FlowControl|Delay 0.2)
            (goto _label_2))))
      (else
        ;[0.15 0.15 0.15 0.5] Regens boss HP during phase 1
        (CallFunction|ShowField)
        (Progress|SetPercent _shieldbar (* (/ (Variables|Default|GetHP) (Variables|Default|GetMaxHP)) (Variables|Default|GetMaxShield)))
        (if (< (Variables|Default|GetHP) _maxhp) :!label _label_3
          (Variables|Default|SetHP (+ (Variables|Default|GetHP) 2e+01))
          (Progress|SetPercent _shieldbar (* (/ (Variables|Default|GetHP) (Variables|Default|GetMaxHP)) (Variables|Default|GetMaxShield)))
          (Utilities|FlowControl|DelayUntilNextTick)
          (goto _label_3)
          (else
            (Variables|Default|SetHP _maxhp)))))
    (elif (== _returnvalue "/Game/Weapons/MeleeAttacks/BP_Sword.BP_Sword_C")
      (Variables|Default|SetHP (- (Variables|Default|GetHP) 6e+02))
      (goto _label))))

(event Custom|HealthDrained
  (bind _self self)
  (bind _hpbar (Variables|Default|GetHPBar))
  (bind _maxhp (Variables|Default|GetMaxHP))
  (bind _returnvalue (AI|GetAIController _self))
  (bind _shieldbar (Variables|/Game/UIWidgets/BossHPBar.BossHPBar_C|GetShieldBar _hpbar))
  (bind _asbp_fallen_angel_controller (Utilities|Casting|CastToBP_FallenAngelController _returnvalue))
  (if (Variables|Default|GetPhase2)
    ;[0.15 0.15 0.15 0.5] Kills the boss when HP reaches 0
    (Progress|SetPercent (Variables|/Game/UIWidgets/BossHPBar.BossHPBar_C|GetHPBar _hpbar) (/ (Variables|Default|GetHP) (Variables|Default|GetMaxHP)))
    (if (<= (stale OnComponentBeginOverlap(CapsuleComponent) _output_get) 0.0)
      (if (ScalableFloat|GetValueasBool (Variables|Default|GetBlackboard) (Variables|Default|GetCanDie)) :!label _label
        (bind _outactors (Actor|GetAllActorsOfClass "/Game/Enemies/FallenAngel/Attacks/Summon/BP_FallenAngelSummon.BP_FallenAngelSummon_C"))
        (for _array_element _outactors
          (Variables|/Game/Enemies/FallenAngel/Attacks/Summon/BP_FallenAngelSummon.BP_FallenAngelSummon_C|SetHP _array_element 0.0)
          (Default|HealthDrained _array_element))
        (bind _outactors_2 (Actor|GetAllActorsOfClass "/Game/Enemies/Arcane/BP_Arcane.BP_Arcane_C"))
        ;[0.15 0.01218 0.01555 0.5] Kills all enemies once boss dies
        (for _array_element_2 _outactors_2
          (Variables|/Game/Enemies/Arcane/BP_Arcane.BP_Arcane_C|SetCanDespawn _array_element_2 false)
          (Variables|/Game/Enemies/Arcane/BP_Arcane.BP_Arcane_C|SetHP _array_element_2 0.0)
          (Default|HealthDrained _array_element_2))
        (bind _outactors_3 (Actor|GetAllActorsOfClass "/Game/Enemies/Knight/BP_Knight.BP_Knight_C"))
        (for _array_element_3 _outactors_3
          (Variables|/Game/Enemies/Knight/BP_Knight.BP_Knight_C|SetCanDespawn _array_element_3 false)
          (Variables|/Game/Enemies/Knight/BP_Knight.BP_Knight_C|SetHP _array_element_3 0.0)
          (Default|HealthDrained _array_element_3))
        (for _array_element_4 (Variables|Default|GetTanks)
          (Variables|/Game/Enemies/Tank/BP_Tank.BP_Tank_C|SetCanDespawn _array_element_4 false)
          (Variables|/Game/Enemies/Tank/BP_Tank.BP_Tank_C|SetHP _array_element_4 0.0)
          (Default|HealthDrained _array_element_4))
        (for _array_element_5 (Variables|Default|GetSummoners)
          (Variables|/Game/Enemies/Summoner/BP_Summoner.BP_Summoner_C|SetCanDespawn _array_element_5 false)
          (Variables|/Game/Enemies/Summoner/BP_Summoner.BP_Summoner_C|SetHP _array_element_5 0.0)
          (Default|HealthDrained _array_element_5))
        (for _array_element_6 (Variables|Default|GetProtectors)
          (Variables|/Game/Enemies/Protector/BP_Protector.BP_Protector_C|SetCanDespawn _array_element_6 false)
          (Variables|/Game/Enemies/Protector/BP_Protector.BP_Protector_C|SetHP _array_element_6 0.0)
          (Default|HealthDrained _array_element_6))
        (Widget|RemovefromParent (Variables|Default|GetHPBar))
        (Components|DestroyComponent (Variables|Collision|GetCapsuleComponent))
        (AI|Logic|StopLogic (Variables|/Game/Enemies/FallenAngel/BP_FallenAngelController.BP_FallenAngelController_C|GetBehaviorTree _asbp_fallen_angel_controller) "")
        (Variables|/Game/Enemies/FallenAngel/BP_FallenAngelController.BP_FallenAngelController_C|SetDead _asbp_fallen_angel_controller true)
        (else
          (Utilities|FlowControl|Delay 0.2)
          (goto _label))))
    (else
      ;[0.15 0.15 0.15 0.5] Regens boss HP during phase 1
      (CallFunction|ShowField)
      (Progress|SetPercent _shieldbar (* (/ (Variables|Default|GetHP) (Variables|Default|GetMaxHP)) (Variables|Default|GetMaxShield)))
      (if (< (Variables|Default|GetHP) _maxhp) :!label _label_2
        (Variables|Default|SetHP (+ (Variables|Default|GetHP) 2e+01))
        (Progress|SetPercent _shieldbar (* (/ (Variables|Default|GetHP) (Variables|Default|GetMaxHP)) (Variables|Default|GetMaxShield)))
        (Utilities|FlowControl|DelayUntilNextTick)
        (goto _label_2)
        (else
          (Variables|Default|SetHP _maxhp))))))

(event Custom|Stun
  (params (HealAmount :type Float%20%28double-precision%29))
  ;[0.15 0.15 0.15 0.5] Deals damage and stuns the enemy
  (Variables|/Game/Enemies/FallenAngel/BP_FallenAngelController.BP_FallenAngelController_C|SetAnimation (.AsBP%20Fallen%20Angel%20Controller (Utilities|Casting|CastToBP_FallenAngelController (AI|GetAIController self))) "NewEnumerator7")
  (if (<= (- (Variables|Default|GetHP) (+ HealAmount (.ShieldOrbDamage (Utilities|Struct|BreakFinalBossStructure (Variables|Default|GetDataTableRow))))) 0.0)
    (Variables|Default|SetHP (* (Variables|Default|GetMaxHP) 0.04))
    (else
      (Variables|Default|SetHP (- (Variables|Default|GetHP) (+ HealAmount (.ShieldOrbDamage (Utilities|Struct|BreakFinalBossStructure (Variables|Default|GetDataTableRow))))))))
  (AI|Components|Blackboard|SetValueasBool (Variables|Default|GetBlackboard) (Variables|Default|GetStunned) true)
  (Progress|SetPercent (Variables|/Game/UIWidgets/BossHPBar.BossHPBar_C|GetHPBar (Variables|Default|GetHPBar)) (/ (Variables|Default|GetHP) (Variables|Default|GetMaxHP))))

(event Custom|DrainHealth
  (params (HealthDrain :type Float%20%28double-precision%29) (TimesToDrain :type Integer))
  (bind _returnvalue (Game|GetPlayerController 0))
  (bind _asbp_first_person_player_controller (Utilities|Casting|CastToBP_FirstPersonPlayerController _returnvalue))
  ;[0.15 0.15 0.15 0.5] Drains health over a period of time
  (Components|Activation|SetActive (Variables|Character|GetCharacterMovement) false false)
  (bind _asbp_fallen_angel_controller (Utilities|Casting|CastToBP_FallenAngelController (AI|GetAIController self)))
  (AI|Logic|StopLogic (Variables|/Game/Enemies/FallenAngel/BP_FallenAngelController.BP_FallenAngelController_C|GetBehaviorTree _asbp_fallen_angel_controller) "")
  (bind _output_get (Variables|Default|SetTimesDrained 0))
  (if (and (< _output_get TimesToDrain) (> (Variables|Default|GetHP) 0.0)) :!label _label
    (Variables|Default|SetHP (- (Variables|Default|GetHP) (* (Variables|/Game/FirstPerson/Blueprints/BP_FirstPersonPlayerController.BP_FirstPersonPlayerController_C|GetDrainBuff%25 _asbp_first_person_player_controller) HealthDrain)))
    (CallFunction|HealthDrained)
    (Development|PrintString "Damaged" true true "(R=0.000000,G=0.660000,B=1.000000,A=1.000000)" 2.5)
    (Variables|Default|SetTimesDrained (+ (Variables|Default|GetTimesDrained) 1))
    (Utilities|FlowControl|Delay (/ 1.5 (Variables|/Game/FirstPerson/Blueprints/BP_FirstPersonPlayerController.BP_FirstPersonPlayerController_C|GetDrainPerTime _asbp_first_person_player_controller)))
    (goto _label)
    (else
      (if (> (Variables|Default|GetHP) 0.0)
        _
        (else
          (CallFunction|HealthDrained)))
      (Class|BrainComponent|RestartLogic (Variables|/Game/Enemies/FallenAngel/BP_FallenAngelController.BP_FallenAngelController_C|GetBehaviorTree _asbp_fallen_angel_controller))
      (Components|Activation|SetActive (Variables|Character|GetCharacterMovement) true false))))

(event Custom|Damage
  (bind _hpbar (Variables|Default|GetHPBar))
  (bind _maxhp (Variables|Default|GetMaxHP))
  (bind _shieldbar (Variables|/Game/UIWidgets/BossHPBar.BossHPBar_C|GetShieldBar _hpbar))
  ;[0.15 0.15 0.15 0.5] Regens boss HP during phase 1
  (Progress|SetPercent _shieldbar (* (/ (Variables|Default|GetHP) (Variables|Default|GetMaxHP)) (Variables|Default|GetMaxShield)))
  (if (< (Variables|Default|GetHP) _maxhp) :!label _label
    (Variables|Default|SetHP (+ (Variables|Default|GetHP) 2e+01))
    (Progress|SetPercent _shieldbar (* (/ (Variables|Default|GetHP) (Variables|Default|GetMaxHP)) (Variables|Default|GetMaxShield)))
    (Utilities|FlowControl|DelayUntilNextTick)
    (goto _label)
    (else
      (Variables|Default|SetHP _maxhp))))

(event Custom|ShowField
  (bind _bossbeam (Variables|Default|GetBossBeam))
  (bind _bossbeam_2 (Variables|Default|GetBossBeam))
  (bind _bossenergyorb (Variables|Default|GetBossEnergyOrb))
  (bind _returnvalue (Transformation|GetActorLocation _bossenergyorb))
  ;[0.15 0.15 0.15 0.5] Shows the force field when hit in phase 1
  (Variables|Default|SetInitialStartTarget (Transformation|GetActorLocation (Variables|Default|GetBossEnergyOrb)))
  (bind _lerp (Timeline|BeamShoot PlayFromStart)
    (:Update
      (Niagara|SetNiagaraVariable(Vector3) _bossbeam_2 "FinalEndTarget" (Math|Vector|Lerp(Vector) (Variables|Default|GetInitialStartTarget) (.ReturnValue (Class|NiagaraComponent|GetVariableVec3 _bossbeam_2 "EndTarget")) _lerp)))
    (:Finished
      (Rendering|Material|SetScalarParameterValue (Variables|Default|GetForceField) "Scale" 1.0 :!class /Script/Engine.MaterialInstanceDynamic)
      (bind (_direction _scale _lerp_2) (Timeline|ScaleDown PlayFromStart)
        (:Update
          (Rendering|Material|SetScalarParameterValue (Variables|Default|GetForceField) "Scale" _scale :!class /Script/Engine.MaterialInstanceDynamic)
          (Niagara|SetNiagaraVariable(Vector3) _bossbeam "StartTarget" (Math|Vector|Lerp(Vector) (Variables|Default|GetInitialStartTarget) (.ReturnValue (Class|NiagaraComponent|GetVariableVec3 _bossbeam "FinalEndTarget")) _lerp_2)))
        (:Finished
          (Niagara|SetNiagaraVariable(Vector3) _bossbeam "StartTarget" _returnvalue)
          (Niagara|SetNiagaraVariable(Vector3) _bossbeam "FinalEndTarget" _returnvalue))))))

(event EventBeginPlay
  ;[0.15 0.15 0.15 0.5] Sets necessary blackboard values
  (bind _returnvalue (Utilities|GetDataTableRow "/Game/DataTables/Enemies/FinalBoss/DT_FinalBoss.DT_FinalBoss" "FallenAngel")
    (:then
      (Variables|Default|SetDataTableRow _returnvalue)
      (bind _output_get (Variables|Default|SetHP (.HP (Utilities|Struct|BreakFinalBossStructure _returnvalue))))
      (Variables|Default|SetMaxHP _output_get)
      (Variables|Default|SetBlackboard (AI|GetBlackboard 0))
      (bind _outactors (Actor|GetAllActorsOfClass "/Game/Enemies/Tank/BP_Tank.BP_Tank_C"))
      (Variables|Default|SetTanks _outactors)
      (bind _outactors_2 (Actor|GetAllActorsOfClass "/Game/Enemies/Summoner/BP_Summoner.BP_Summoner_C"))
      (Variables|Default|SetSummoners _outactors_2)
      (bind _outactors_3 (Actor|GetAllActorsOfClass "/Game/Enemies/Protector/BP_Protector.BP_Protector_C"))
      (Variables|Default|SetProtectors _outactors_3)
      ;[0.15 0.15 0.15 0.5] Creates the force field material instance
      (bind _returnvalue_2 (Rendering|Material|CreateDynamicMaterialInstance "/Game/ArtAssets/VFX/BossBeamVFX/MI_BossField.MI_BossField" "None" "None" :!class /Script/Engine.KismetMaterialLibrary))
      (bind _output_get_2 (Variables|Default|SetForceField _returnvalue_2))
      (Rendering|Material|SetScalarParameterValue _output_get_2 "Scale" 0.0 :!class /Script/Engine.MaterialInstanceDynamic)
      (Rendering|Material|SetOverlayMaterial (Variables|Character|GetMesh) _output_get_2 :!class /Script/Engine.MeshComponent))))

(fn ConstructionScript)

(fn ScaleDamage
  (params (SpellRow :type Name) (SpellActor :type Actor%20Object%20Reference))
  (bind _returnvalue (Game|GetPlayerController 0))
  (bind _returnvalue_2 (Math|Random|RandomIntegerinRange 8 12))
  (bind _asbp_first_person_player_controller (Utilities|Casting|CastToBP_FirstPersonPlayerController _returnvalue))
  (bind _drainpertime (Variables|/Game/FirstPerson/Blueprints/BP_FirstPersonPlayerController.BP_FirstPersonPlayerController_C|GetDrainPerTime _asbp_first_person_player_controller))
  (bind _returnvalue_3 (* _returnvalue_2 _drainpertime))
  (bind _returnvalue_4 (Math|Float|Round _returnvalue_3))
  ;[0.15 0.15 0.15 0.5] Checks if the spell is a charge spell. If so, scales its damage accordingly. If Toxic Thorn, initiates health drain.
  (bind _returnvalue_5 (Utilities|GetDataTableRow "/Game/DataTables/Spells/DT_Spells.DT_Spells" SpellRow)
    (:then
      (if (Utilities|Enum|Equal(Enum) (.SpellType (Utilities|Struct|BreakSpellStructure _returnvalue_5)) "NewEnumerator3")
        (if (== (.Spell (Utilities|Struct|BreakSpellStructure _returnvalue_5)) "/Game/Weapons/MagicAttacks/OfficialSpells/CombustionSpell/BP_Combustion.BP_Combustion_C")
          (return (* (.X (Math|Vector|BreakVector (* (/ (Transformation|GetActorScale3D SpellActor) 1e+01) (.SpellDamage (Utilities|Struct|BreakSpellStructure _returnvalue_5))))) (Variables|/Game/FirstPerson/Blueprints/BP_FirstPersonPlayerController.BP_FirstPersonPlayerController_C|GetForceBuff%25 (.AsBP%20First%20Person%20Player%20Controller (Utilities|Casting|CastToBP_FirstPersonPlayerController (Game|GetPlayerController 0))))))
          (elif (> (/ (- (.Lifetime (Utilities|Struct|BreakSpellStructure _returnvalue_5)) (Actor|GetLifeSpan SpellActor)) 3.0) 1.0)
            (CallFunction|DrainHealth (.SpellDamage (Utilities|Struct|BreakSpellStructure _returnvalue_5)) _returnvalue_4)
            (return 0.0)
            (else
              (CallFunction|DrainHealth (* (/ (- (.Lifetime (Utilities|Struct|BreakSpellStructure _returnvalue_5)) (Actor|GetLifeSpan SpellActor)) 3.0) (.SpellDamage (Utilities|Struct|BreakSpellStructure _returnvalue_5))) _returnvalue_4)
              (return 0.0))))
        (else
          (switch Utilities|FlowControl|Switch|SwitchonDamageTypeEnum (.DamageType (Utilities|Struct|BreakSpellStructure _returnvalue_5))
            (:NewEnumerator0
              (Variables|Default|SetDamagetoDeal (* (.SpellDamage (Utilities|Struct|BreakSpellStructure _returnvalue_5)) (Variables|/Game/FirstPerson/Blueprints/BP_FirstPersonPlayerController.BP_FirstPersonPlayerController_C|GetForceBuff%25 _asbp_first_person_player_controller))))
            (:NewEnumerator1
              (Variables|Default|SetDamagetoDeal (* (.SpellDamage (Utilities|Struct|BreakSpellStructure _returnvalue_5)) (Variables|/Game/FirstPerson/Blueprints/BP_FirstPersonPlayerController.BP_FirstPersonPlayerController_C|GetPierceBuff%25 _asbp_first_person_player_controller))))
            (:NewEnumerator2
              (Variables|Default|SetDamagetoDeal (* (.SpellDamage (Utilities|Struct|BreakSpellStructure _returnvalue_5)) (Variables|/Game/FirstPerson/Blueprints/BP_FirstPersonPlayerController.BP_FirstPersonPlayerController_C|GetDrainBuff%25 _asbp_first_person_player_controller)))))
          (return (Variables|Default|GetDamagetoDeal)))))))

(fn GetRow
  (params (Class :type Actor%20Class%20Reference))
  ;[0.15 0.15 0.15 0.5] Checks each row on the data table to find which one the enemy collided with
  (bind _outrownames (DataTable|GetDataTableRowNames "/Game/DataTables/Spells/DT_Spells.DT_Spells"))
  (for _array_element _outrownames
    (bind _returnvalue (Utilities|GetDataTableRow "/Game/DataTables/Spells/DT_Spells.DT_Spells" _array_element)
      (:then
        (if (== (.Spell (Utilities|Struct|BreakSpellStructure _returnvalue)) Class)
          (return _array_element))))))