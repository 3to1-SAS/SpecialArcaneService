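; Destructible totem in the Fallen Angel boss fight, with HP loaded from DT_FinalBoss.
; Spell and sword overlaps reduce HP; spells are matched by class in DT_Spells and scaled by player buffs.
; Charge spells scale damage by actor size (Combustion) or lifetime, the latter as a delay-looped health drain.
; On death it lowers the boss's MaxShield, damages it, increments the controller's totem count and triggers Phase 2 after three.
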(event OnComponentBeginOverlap(CapsuleComponent)
  (params (OverlappedComponent :type Primitive%20Component%20Object%20Reference) (OtherActor :type Actor%20Object%20Reference) (OtherComp :type Primitive%20Component%20Object%20Reference) (OtherBodyIndex :type Integer) (bFromSweep :type Boolean) (SweepResult :type Hit%20Result%20Structure%20%28by%20ref%29))
  (bind _returnvalue (Utilities|GetClass OtherActor))
  ;[0.15 0.15 0.15 0.5] Calculates damage taken based on spell
  (if (Actor|ActorHasTag OtherActor "Spell")
    (bind _name (CallFunction|GetRow _returnvalue))
    (if (== _name "Bolt!Strike")
      (Variables|Default|SetHP (- (Variables|Default|GetHP) 1e+03))
      (else
        (bind _damage (CallFunction|ScaleDamage _name OtherActor))
        (Variables|Default|SetHP (- (Variables|Default|GetHP) _damage))))
    (if (<= (Variables|Default|GetHP) 0.0) :!label _label
      (bind _returnvalue_2 (Actor|GetActorOfClass "/Game/Enemies/FallenAngel/BP_FallenAngel.BP_FallenAngel_C"))
      (bind _result (Math|Integer|IncrementInt (Variables|/Game/Enemies/FallenAngel/BP_FallenAngelController.BP_FallenAngelController_C|GetTotemsDestroyed (.AsBP%20Fallen%20Angel%20Controller (Utilities|Casting|CastToBP_FallenAngelController (AI|GetAIController _returnvalue_2)))))
        (:%20%20
          (Variables|/Game/Enemies/FallenAngel/BP_FallenAngel.BP_FallenAngel_C|SetMaxShield _returnvalue_2 (- (Variables|/Game/Enemies/FallenAngel/BP_FallenAngel.BP_FallenAngel_C|GetMaxShield _returnvalue_2) 0.33))
          (Default|Damage _returnvalue_2)
          (if (>= _result 3)
            (Default|Phase2 (.AsBP%20Fallen%20Angel%20Controller (Utilities|Casting|CastToBP_FallenAngelController (AI|GetAIController _returnvalue_2)))))
          (Actor|DestroyActor))))
    (elif (== _returnvalue "/Game/Weapons/MeleeAttacks/BP_Sword.BP_Sword_C")
      (Variables|Default|SetHP (- (Variables|Default|GetHP) 6e+02))
      (goto _label))))

(event Custom|DrainHealth
  (params (HealthDrain :type Float%20%28double-precision%29) (TimesToDrain :type Integer))
  (bind _returnvalue (Game|GetPlayerController 0))
  (bind _asbp_first_person_player_controller (Utilities|Casting|CastToBP_FirstPersonPlayerController _returnvalue))
  ;[0.15 0.15 0.15 0.5] Drains health over a period of time
  (bind _output_get (Variables|Default|SetTimesDrained 0))
  (if (and (< _output_get TimesToDrain) (> (Variables|Default|GetHP) 0.0)) :!label _label
    (Variables|Default|SetHP (- (Variables|Default|GetHP) (* (Variables|/Game/FirstPerson/Blueprints/BP_FirstPersonPlayerController.BP_FirstPersonPlayerController_C|GetDrainBuff%25 _asbp_first_person_player_controller) HealthDrain)))
    (Development|PrintString "Damaged" true true "(R=0.000000,G=0.660000,B=1.000000,A=1.000000)" 2.5)
    (Variables|Default|SetTimesDrained (+ (Variables|Default|GetTimesDrained) 1))
    (Utilities|FlowControl|Delay (/ 2.0 (Variables|/Game/FirstPerson/Blueprints/BP_FirstPersonPlayerController.BP_FirstPersonPlayerController_C|GetDrainPerTime _asbp_first_person_player_controller)))
    (goto _label)
    (elif (not (> (Variables|Default|GetHP) 0.0))
      (CallFunction|HealthDrained))))

(event Custom|Health%20Drained
  (if (<= (Variables|Default|GetHP) 0.0)
    (bind _returnvalue (Actor|GetActorOfClass "/Game/Enemies/FallenAngel/BP_FallenAngel.BP_FallenAngel_C"))
    (bind _result (Math|Integer|IncrementInt (Variables|/Game/Enemies/FallenAngel/BP_FallenAngelController.BP_FallenAngelController_C|GetTotemsDestroyed (.AsBP%20Fallen%20Angel%20Controller (Utilities|Casting|CastToBP_FallenAngelController (AI|GetAIController _returnvalue)))))
      (:%20%20
        (Variables|/Game/Enemies/FallenAngel/BP_FallenAngel.BP_FallenAngel_C|SetMaxShield _returnvalue (- (Variables|/Game/Enemies/FallenAngel/BP_FallenAngel.BP_FallenAngel_C|GetMaxShield _returnvalue) 0.33))
        (Default|Damage _returnvalue)
        (if (>= _result 3)
          (Default|Phase2 (.AsBP%20Fallen%20Angel%20Controller (Utilities|Casting|CastToBP_FallenAngelController (AI|GetAIController _returnvalue)))))
        (Actor|DestroyActor)))))

(event EventBeginPlay
  (bind _returnvalue (Utilities|GetDataTableRow "/Game/DataTables/Enemies/FinalBoss/DT_FinalBoss.DT_FinalBoss" "FallenAngel")
    (:then
      (Variables|Default|SetHP (.BossTotemHP (Utilities|Struct|BreakFinalBossStructure _returnvalue))))))

(event EventDestroyed
  (Variables|Default|SetIsAlive false))

(fn ConstructionScript)

(fn UglyAhhhCheckSpell
  (params (Spell :type Actor%20Object%20Reference))
  (bind _returnvalue (Utilities|GetClass Spell))
  (bind _outrownames (DataTable|GetDataTableRowNames "/Game/DataTables/Spells/DT_Spells.DT_Spells"))
  (bind _array_element (Utilities|Array|ForEachLoopwithBreak _outrownames :!label _label)
    (:LoopBody
      (bind _returnvalue_2 (Utilities|GetDataTableRow "/Game/DataTables/Spells/DT_Spells.DT_Spells" _array_element)
        (:then
          (if (== (.Spell (Utilities|Struct|BreakSpellStructure _returnvalue_2)) _returnvalue)
            (LocalVariables|SetSpellFound true)
            (LocalVariables|SetSpellRef _array_element)
            (goto _label Break)))))
    (:Completed
      (if (LocalVariables|GetSpellFound)
        (return (LocalVariables|GetSpellRef))
        (else
          (Development|PrintString (Utilities|GetClassDisplayName _returnvalue)))))))

(fn ScaleDamage
  (params (SpellRow :type Name) (SpellActor :type Actor%20Object%20Reference))
  (bind _returnvalue (Game|GetPlayerController 0))
  (bind _returnvalue_2 (Math|Random|RandomIntegerinRange 10 13))
  (bind _asbp_first_person_player_controller (Utilities|Casting|CastToBP_FirstPersonPlayerController _returnvalue))
  ;[0.15 0.15 0.15 0.5] Checks if the spell is a charge spell. If so, scales its damage accordingly. If Toxic Thorn, initiates health drain.
  (bind _returnvalue_3 (Utilities|GetDataTableRow "/Game/DataTables/Spells/DT_Spells.DT_Spells" SpellRow)
    (:then
      (if (Utilities|Enum|Equal(Enum) (.SpellType (Utilities|Struct|BreakSpellStructure _returnvalue_3)) "NewEnumerator3")
        (if (== (.Spell (Utilities|Struct|BreakSpellStructure _returnvalue_3)) "/Game/Weapons/MagicAttacks/OfficialSpells/CombustionSpell/BP_Combustion.BP_Combustion_C")
          (return (* (.X (Math|Vector|BreakVector (* (/ (Transformation|GetActorScale3D SpellActor) 1e+01) (.SpellDamage (Utilities|Struct|BreakSpellStructure _returnvalue_3))))) (Variables|/Game/FirstPerson/Blueprints/BP_FirstPersonPlayerController.BP_FirstPersonPlayerController_C|GetForceBuff%25 (.AsBP%20First%20Person%20Player%20Controller (Utilities|Casting|CastToBP_FirstPersonPlayerController (Game|GetPlayerController 0))))))
          (elif (> (/ (- (.Lifetime (Utilities|Struct|BreakSpellStructure _returnvalue_3)) (Actor|GetLifeSpan SpellActor)) 3.0) 1.0)
            (CallFunction|DrainHealth (.SpellDamage (Utilities|Struct|BreakSpellStructure _returnvalue_3)) _returnvalue_2)
            (return 0.0)
            (else
              (CallFunction|DrainHealth (* (/ (- (.Lifetime (Utilities|Struct|BreakSpellStructure _returnvalue_3)) (Actor|GetLifeSpan SpellActor)) 3.0) (.SpellDamage (Utilities|Struct|BreakSpellStructure _returnvalue_3))) _returnvalue_2)
              (return 0.0))))
        (else
          (switch Utilities|FlowControl|Switch|SwitchonDamageTypeEnum (.DamageType (Utilities|Struct|BreakSpellStructure _returnvalue_3))
            (:NewEnumerator0
              (Variables|Default|SetDamagetoDeal (* (.SpellDamage (Utilities|Struct|BreakSpellStructure _returnvalue_3)) (Variables|/Game/FirstPerson/Blueprints/BP_FirstPersonPlayerController.BP_FirstPersonPlayerController_C|GetForceBuff%25 _asbp_first_person_player_controller))))
            (:NewEnumerator1
              (Variables|Default|SetDamagetoDeal (* (.SpellDamage (Utilities|Struct|BreakSpellStructure _returnvalue_3)) (Variables|/Game/FirstPerson/Blueprints/BP_FirstPersonPlayerController.BP_FirstPersonPlayerController_C|GetPierceBuff%25 _asbp_first_person_player_controller))))
            (:NewEnumerator2
              (Variables|Default|SetDamagetoDeal (* (.SpellDamage (Utilities|Struct|BreakSpellStructure _returnvalue_3)) (Variables|/Game/FirstPerson/Blueprints/BP_FirstPersonPlayerController.BP_FirstPersonPlayerController_C|GetDrainBuff%25 _asbp_first_person_player_controller)))))
          (return (Variables|Default|GetDamagetoDeal)))))))

(fn GetRow
  (params (SpellClass :type Actor%20Class%20Reference))
  ;[0.15 0.15 0.15 0.5] Checks each row on the data table to find which one the enemy collided with
  (bind _outrownames (DataTable|GetDataTableRowNames "/Game/DataTables/Spells/DT_Spells.DT_Spells"))
  (for _array_element _outrownames
    (bind _returnvalue (Utilities|GetDataTableRow "/Game/DataTables/Spells/DT_Spells.DT_Spells" _array_element)
      (:then
        (if (== (.Spell (Utilities|Struct|BreakSpellStructure _returnvalue)) SpellClass)
          (return _array_element))))))