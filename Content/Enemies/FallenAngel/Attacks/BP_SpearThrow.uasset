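; BP_SpearThrow is the spear projectile for the Fallen Angel boss's throw attack.
; On BeginPlay it reads its velocity from the BossSpearThrow row of DT_EnemySpells and applies it as local forward velocity and max speed.
; After a short delay, its Cube starts blocking WorldStatic.
; When the Cube hits something, it removes the EnemySpell tag and notifies its owning enemy through SpearThrown.
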(event OnComponentHit(Cube)
  (params (HitComponent :type Primitive%20Component%20Object%20Reference) (OtherActor :type Actor%20Object%20Reference) (OtherComp :type Primitive%20Component%20Object%20Reference) (NormalImpulse :type Vector :default "0, 0, 0") (Hit :type Hit%20Result%20Structure%20%28by%20ref%29))
  (Utilities|Array|RemoveItem (Variables|Actor|GetTags) "EnemySpell")
  (Default|SpearThrown (Variables|Default|GetOwnerEnemy)))

(event EventBeginPlay
  (bind _projectilemovement (Variables|Default|GetProjectileMovement))
  ;[0.15 0.15 0.15 0.5] Sets velocity from data table
  (bind _returnvalue (Utilities|GetDataTableRow "/Game/DataTables/Enemies/EnemySpells/DT_EnemySpells.DT_EnemySpells" "BossSpearThrow")
    (:then
      (Game|Components|ProjectileMovement|SetVelocityinLocalSpace _projectilemovement (Math|Vector|MakeVector (.velocity _returnvalue) 0.0 0.0))
      (Variables|/Script/Engine.ProjectileMovementComponent|SetMaxSpeed _projectilemovement (.velocity _returnvalue))
      (Utilities|FlowControl|Delay 0.2)
      (Collision|SetCollisionResponsetoChannel (Variables|Default|GetCube) "ECC_WorldStatic" "ECR_Block"))))

(fn ConstructionScript)