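; Shield orb for the Fallen Angel boss fight that repeatedly heals the boss until it expires or is destroyed.
; Timing, HP and Bolt Strike damage come from DT_FinalBoss; other spell hits look up DT_Spells, scaling charge spells or starting damage over time.
; Sword hits deal flat damage.
; Hits flash the orb red; at zero HP it explodes and stuns the boss, passing along the total healed.
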(event OnComponentBeginOverlap(Sphere)
  (params (OverlappedComponent :type Primitive%20Component%20Object%20Reference) (OtherActor :type Actor%20Object%20Reference) (OtherComp :type Primitive%20Component%20Object%20Reference) (OtherBodyIndex :type Integer) (bFromSweep :type Boolean) (SweepResult :type Hit%20Result%20Structure%20%28by%20ref%29))
  (bind _returnvalue (Utilities|GetClass OtherActor))
  ;[0.15 0.15 0.15 0.5] Calculates damage taken based on spell
  (if (Actor|ActorHasTag OtherActor "Spell")
    (bind _name (CallFunction|GetRow _returnvalue))
    (if (== _name "Bolt!Strike")
      (Variables|Default|SetHP (- (Variables|Default|GetHP) (.BoltStrikeDamage (Utilities|Struct|BreakFinalBossStructure (Variables|Default|GetDataTableRow)))))
      (else
        (bind _damage (CallFunction|ScaleDamage _name OtherActor))
        (Variables|Default|SetHP (- (Variables|Default|GetHP) _damage))))
    (if (<= (Variables|Default|GetHP) 0.0) :!label _label
      (Default|Stun (Variables|Default|GetBoss) (Variables|Default|GetTotalHealed))
      (Niagara|SpawnSystematLocation "/Game/Enemies/FallenAngel/Attacks/NS_OrbExplosion.NS_OrbExplosion" (Transformation|GetActorLocation))
      (Actor|DestroyActor)
      (else
        (Rendering|Material|SetMaterial (Variables|Default|GetSphere) 0 "/Game/ArtAssets/Decorations/Orb/RedOrbFloter.RedOrbFloter")
        (Utilities|FlowControl|Delay 0.1)
        (Rendering|Material|SetMaterial (Variables|Default|GetSphere) 0 "/Game/ArtAssets/Decorations/Orb/BlueOrbFloater.BlueOrbFloater")))
    (elif (== _returnvalue "/Game/Weapons/MeleeAttacks/BP_Sword.BP_Sword_C")
      (Variables|Default|SetHP (- (Variables|Default|GetHP) 6e+02))
      (goto _label))))

(event Custom|Heal
  (bind _boss (Variables|Default|GetBoss))
  (bind _maxhp (Variables|/Game/Enemies/FallenAngel/BP_FallenAngel.BP_FallenAngel_C|GetMaxHP _boss))
  (bind _returnvalue (/ _maxhp 1e+02))
  (Variables|/Game/Enemies/FallenAngel/BP_FallenAngel.BP_FallenAngel_C|SetHP _boss (+ (Variables|/Game/Enemies/FallenAngel/BP_FallenAngel.BP_FallenAngel_C|GetHP _boss) _returnvalue))
  (Variables|Default|SetTotalHealed (+ (Variables|Default|GetTotalHealed) _returnvalue))
  (if (> (Variables|/Game/Enemies/FallenAngel/BP_FallenAngel.BP_FallenAngel_C|GetHP _boss) _maxhp)
    (Variables|/Game/Enemies/FallenAngel/BP_FallenAngel.BP_FallenAngel_C|SetHP _boss _maxhp))
  (Default|HealthDrained _boss)
  (Utilities|FlowControl|Delay (/ (.ShieldOrbTime (Utilities|Struct|BreakFinalBossStructure (stale EventBeginPlay _returnvalue_2))) 1e+01))
  (CallFunction|Heal))

(event Custom|HealthDrained
  (if (<= (Variables|Default|GetHP) 0.0)
    (Default|Stun (Variables|Default|GetBoss) (Variables|Default|GetTotalHealed))
    (Niagara|SpawnSystematLocation "/Game/Enemies/FallenAngel/Attacks/NS_OrbExplosion.NS_OrbExplosion" (Transformation|GetActorLocation))
    (Actor|DestroyActor)
    (else
      (Rendering|Material|SetMaterial (Variables|Default|GetSphere) 0 "/Game/ArtAssets/Decorations/Orb/RedOrbFloter.RedOrbFloter")
      (Utilities|FlowControl|Delay 0.1)
      (Rendering|Material|SetMaterial (Variables|Default|GetSphere) 0 "/Game/ArtAssets/Decorations/Orb/BlueOrbFloater.BlueOrbFloater"))))

(event Custom|DrainHealth
  (params (HealthDrain :type Float%20%28double-precision%29) (TimesToDrain :type Integer))
  ;[0.15 0.15 0.15 0.5] Drains health over a period of time
  (bind _output_get (Variables|Default|SetTimesDrained 0))
  (if (and (< _output_get TimesToDrain) (> (Variables|Default|GetHP) 0.0)) :!label _label
    (Variables|Default|SetHP (- (Variables|Default|GetHP) HealthDrain))
    (Development|PrintString "Damaged" true true "(R=0.000000,G=0.660000,B=1.000000,A=1.000000)" 2.5)
    (Variables|Default|SetTimesDrained (+ (Variables|Default|GetTimesDrained) 1))
    (Utilities|FlowControl|Delay 1.0)
    (goto _label)
    (elif (not (> (Variables|Default|GetHP) 0.0))
      (CallFunction|HealthDrained))))

(event EventBeginPlay
  (bind _returnvalue (Actor|GetActorOfClass "/Game/Enemies/FallenAngel/BP_FallenAngel.BP_FallenAngel_C"))
  (Variables|Default|SetBoss _returnvalue)
  (bind _returnvalue_2 (Utilities|GetDataTableRow "/Game/DataTables/Enemies/FinalBoss/DT_FinalBoss.DT_FinalBoss" "FallenAngel")
    (:then
      (Variables|Default|SetDataTableRow _returnvalue_2)
      (Variables|Default|SetHP (.ShieldOrbHP (Utilities|Struct|BreakFinalBossStructure _returnvalue_2)))
      (CallFunction|Heal)
      (Utilities|FlowControl|Delay (.ShieldOrbTime (Utilities|Struct|BreakFinalBossStructure _returnvalue_2)))
      (Actor|DestroyActor))))

(fn ConstructionScript)

(fn ScaleDamage
  (params (SpellRow :type Name) (SpellActor :type Actor%20Object%20Reference))
  (bind _returnvalue (Math|Random|RandomIntegerinRange 8 12))
  ;[0.15 0.15 0.15 0.5] Checks if the spell is a charge spell. If so, scales its damage accordingly. If Toxic Thorn, initiates health drain.
  (bind _returnvalue_2 (Utilities|GetDataTableRow "/Game/DataTables/Spells/DT_Spells.DT_Spells" SpellRow)
    (:then
      (if (Utilities|Enum|Equal(Enum) (.SpellType (Utilities|Struct|BreakSpellStructure _returnvalue_2)) "NewEnumerator3")
        (if (== (.Spell (Utilities|Struct|BreakSpellStructure _returnvalue_2)) "/Game/Weapons/MagicAttacks/OfficialSpells/CombustionSpell/BP_Combustion.BP_Combustion_C")
          (return (.X (Math|Vector|BreakVector (* (/ (Transformation|GetActorScale3D SpellActor) 1e+01) (.SpellDamage (Utilities|Struct|BreakSpellStructure _returnvalue_2))))))
          (elif (> (/ (- (.Lifetime (Utilities|Struct|BreakSpellStructure _returnvalue_2)) (Actor|GetLifeSpan SpellActor)) 3.0) 1.0)
            (CallFunction|DrainHealth (.SpellDamage (Utilities|Struct|BreakSpellStructure _returnvalue_2)) _returnvalue)
            (return 0.0)
            (else
              (CallFunction|DrainHealth (* (/ (- (.Lifetime (Utilities|Struct|BreakSpellStructure _returnvalue_2)) (Actor|GetLifeSpan SpellActor)) 3.0) (.SpellDamage (Utilities|Struct|BreakSpellStructure _returnvalue_2))) _returnvalue))))
        (elif (not (== (.Spell (Utilities|Struct|BreakSpellStructure _returnvalue_2)) "/Game/Weapons/MagicAttacks/OfficialSpells/PulseWave/BP_PulseWave.BP_PulseWave_C"))
          (return (.SpellDamage (Utilities|Struct|BreakSpellStructure _returnvalue_2))))))))

(fn GetRow
  (params (Class :type Actor%20Class%20Reference))
  ;[0.15 0.15 0.15 0.5] Checks each row on the data table to find which one the enemy collided with
  (bind _outrownames (DataTable|GetDataTableRowNames "/Game/DataTables/Spells/DT_Spells.DT_Spells"))
  (for _array_element _outrownames
    (bind _returnvalue (Utilities|GetDataTableRow "/Game/DataTables/Spells/DT_Spells.DT_Spells" _array_element)
      (:then
        (if (== (.Spell (Utilities|Struct|BreakSpellStructure _returnvalue)) Class)
          (return _array_element))))))