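; Magic sword projectile for the Fallen Angel final boss, which waits and then launches itself at the player.
; The wait is the FallenAngel row's sword delay minus its own Delay variable.
; At launch it aims at the player's predicted position with capped lead time, taking speed and lifespan from DT_EnemySpells.
; It is destroyed when the lifespan ends or on overlaps while active, ignoring enemies, shields and NonBlocking components.
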(event OnComponentBeginOverlap(Collision)
  (params (OverlappedComponent :type Primitive%20Component%20Object%20Reference) (OtherActor :type Actor%20Object%20Reference) (OtherComp :type Primitive%20Component%20Object%20Reference) (OtherBodyIndex :type Integer) (bFromSweep :type Boolean) (SweepResult :type Hit%20Result%20Structure%20%28by%20ref%29))
  ;[0.15 0.15 0.15 0.5] Destroys spell on collision
  (if (Components|Activation|IsActive (Variables|Default|GetProjectileMovement))
    (Utilities|FlowControl|DelayUntilNextTick)
    (Utilities|IsValid OtherActor
      (:Is%20Valid
        (if (not (or (Actor|ActorHasTag OtherActor "enemy") (Actor|ActorHasTag OtherActor "Shield")))
          (if (not (Components|ComponentHasTag OtherComp "NonBlocking"))
            (Actor|DestroyActor)))))))

(event EventBeginPlay
  (bind _returnvalue (Game|Player|GetPlayerPawn 0))
  (bind _projectilemovement (Variables|Default|GetProjectileMovement))
  ;[0.15 0.15 0.15 0.5] Destroys spell on collision
  (Utilities|FlowControl|DelayUntilNextTick)
  (bind _returnvalue_2 (Utilities|GetDataTableRow "/Game/DataTables/Enemies/FinalBoss/DT_FinalBoss.DT_FinalBoss" "FallenAngel")
    (:then
      (Utilities|FlowControl|Delay (- (.MagicSwordDelay (Utilities|Struct|BreakFinalBossStructure _returnvalue_2)) (Variables|Default|GetDelay)))
      (bind _returnvalue_3 (Utilities|GetDataTableRow "/Game/DataTables/Enemies/EnemySpells/DT_EnemySpells.DT_EnemySpells" "BossMagicSwords")
        (:then
          (Transformation|SetActorRotation (Math|Rotator|FindLookatRotation (Transformation|GetActorLocation) (+ (Transformation|GetActorLocation _returnvalue) (* (Transformation|GetVelocity _returnvalue) (Math|Float|Min(Float) (/ (Transformation|GetDistanceTo _returnvalue) (.velocity _returnvalue_3)) 3.0)))))
          (Components|Activation|SetActive (Variables|Default|GetProjectileMovement) true false)
          (Game|Components|ProjectileMovement|SetVelocityinLocalSpace _projectilemovement (Math|Vector|MakeVector (.velocity _returnvalue_3) 0.0 0.0))
          (Variables|/Script/Engine.ProjectileMovementComponent|SetMaxSpeed _projectilemovement (.velocity _returnvalue_3))
          (Utilities|FlowControl|Delay (.lifespan _returnvalue_3))
          (Actor|DestroyActor))))))

(fn ConstructionScript)