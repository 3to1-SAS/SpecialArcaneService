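; BP_FallenAngelMelee is a short-lived melee hitbox for an enemy, destroyed after the KnightAttack Lifespan from DT_EnemySpells.
; Each tick it follows OwnerEnemy, offset along its forward vector.
; On overlapping the player's capsule, it waits a tick, then removes its EnemySpell tag to prevent multihits.
; It also knocks the player forward once through a loop of repeated AddForce calls, scaled by the TankAttack row's knockback.
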(event OnComponentBeginOverlap(Cube)
  (params (OverlappedComponent :type Primitive%20Component%20Object%20Reference) (OtherActor :type Actor%20Object%20Reference) (OtherComp :type Primitive%20Component%20Object%20Reference) (OtherBodyIndex :type Integer) (bFromSweep :type Boolean) (SweepResult :type Hit%20Result%20Structure%20%28by%20ref%29))
  ;[0.15 0.15 0.15 0.5] Removes the tag after hitting to prevent multihits
  (Utilities|FlowControl|DelayUntilNextTick)
  (bind _array_element (Utilities|Array|ForEachLoopwithBreak (Class|Actor|GetOverlappingComponents) :!label _label)
    (:LoopBody
      (if (and (== (Utilities|GetClass (Components|GetOwner _array_element)) "/Game/FirstPerson/Blueprints/BP_FirstPersonCharacter.BP_FirstPersonCharacter_C") (== (Actor|GetComponentbyClass (Components|GetOwner _array_element) "/Script/Engine.CapsuleComponent") _array_element))
        (Utilities|Array|RemoveItem (Variables|Actor|GetTags) "EnemySpell")
        (Utilities|FlowControl|DoOnce false
          (:Completed
            (bind _returnvalue (Utilities|GetDataTableRow "/Game/DataTables/Enemies/EnemySpells/DT_EnemySpells.DT_EnemySpells" "TankAttack")
              (:then
                (for _index (range 0 5000)
                  (Physics|AddForce (Variables|/Script/Engine.Character|GetCharacterMovement (.AsBP%20First%20Person%20Character (Utilities|Casting|CastToBP_FirstPersonCharacter (Components|GetOwner _array_element)))) (* (Transformation|GetActorForwardVector) (Math|Vector|MakeVector (.TANK-Knockback (Utilities|Struct|BreakEnemySpellStructure _returnvalue)) (.TANK-Knockback (Utilities|Struct|BreakEnemySpellStructure _returnvalue)) 1.0))))
                (goto _label Break)))))))))

(event EventTick
  (params (DeltaSeconds :type Float%20%28single-precision%29))
  (bind _ownerenemy (Variables|Default|GetOwnerEnemy))
  (bind _returnvalue (Transformation|GetActorTransform _ownerenemy))
  ;[0.15 0.15 0.15 0.5] Makes the hitbox move with the enemy
  (if (Utilities|IsValid _ownerenemy)
    (Transformation|SetActorTransform (Math|Transform|MakeTransform (+ (.location _returnvalue) (* (Transformation|GetActorForwardVector _ownerenemy) "100.000000,100.000000,0.000000")) (.rotation _returnvalue) (Transformation|GetActorScale3D)))))

(event EventBeginPlay
  ;[0.15 0.15 0.15 0.5] Destroys Hitbox After Short Delay
  (bind _returnvalue (Utilities|GetDataTableRow "/Game/DataTables/Enemies/EnemySpells/DT_EnemySpells.DT_EnemySpells" "KnightAttack")
    (:then
      (Utilities|FlowControl|Delay (.lifespan _returnvalue))
      (Actor|DestroyActor))))

(fn ConstructionScript)