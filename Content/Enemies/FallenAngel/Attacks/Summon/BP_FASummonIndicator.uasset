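; Ground indicator for the Fallen Angel's summon attack that marks where a summoned enemy appears.
; On BeginPlay it waits a short delay, then, if its owner enemy is still valid, spawns BP_FallenAngelSummon slightly above itself, rotated toward the player pawn.
; It destroys itself after spawning, or when the EnemyKilled event fires, which cancels any pending summon.
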(event Custom|EnemyKilled
  (Actor|DestroyActor))

(event EventBeginPlay
  (bind _returnvalue (Transformation|GetActorLocation))
  (bind _returnvalue_2 (+ (.z _returnvalue) 1e+02))
  ;[0.15 0.15 0.15 0.5] Spawns enemy after 2.5 seconds
  (Utilities|FlowControl|Delay 2.5)
  (Utilities|IsValid (Variables|Default|GetOwnerEnemy)
    (:Is%20Valid
      (Game|SpawnActorfromClass "/Game/Enemies/FallenAngel/Attacks/Summon/BP_FallenAngelSummon.BP_FallenAngelSummon_C" (Math|Transform|MakeTransform (Math|Vector|MakeVector (.x _returnvalue) (.y _returnvalue) _returnvalue_2) (Math|Rotator|FindLookatRotation (Math|Vector|MakeVector (.x _returnvalue) (.y _returnvalue) _returnvalue_2) (Transformation|GetActorLocation (Game|Player|GetPlayerPawn 0))) "1.000000,1.000000,1.000000") "Undefined" "MultiplyWithRoot" 0 0)
      (Actor|DestroyActor))))

(fn ConstructionScript)