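; Enemy character summoned by the Fallen Angel that starts out chasing the player under its own behavior tree.
; BeginPlay fills its blackboard from DT_Enemies and instance settings.
; Spell or sword overlaps reduce HP, with DT_Spells driving charge scaling, drain-over-time and Pulse Wave stuns.
; Death triggers ragdoll impulse, a possible health drop, wave and enemy-count updates, and delayed destruction, while stun and drop values read "Knight" rows.
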(event OnComponentBeginOverlap(CapsuleComponent)
  (params (OverlappedComponent :type Primitive%20Component%20Object%20Reference) (OtherActor :type Actor%20Object%20Reference) (OtherComp :type Primitive%20Component%20Object%20Reference) (OtherBodyIndex :type Integer) (bFromSweep :type Boolean) (SweepResult :type Hit%20Result%20Structure%20%28by%20ref%29))
  (bind _returnvalue (Utilities|GetClass OtherActor))
  (bind _self self)
  (bind _capsulecomponent (Variables|Collision|GetCapsuleComponent))
  (bind _tags (Variables|Actor|GetTags))
  (bind _returnvalue_2 (AI|GetAIController _self))
  (bind _asbp_aicontroller (Utilities|Casting|CastToBP_AIController _returnvalue_2))
  ;[0.15 0.15 0.15 0.5] Calculates damage taken based on spell
  (if (Actor|ActorHasTag OtherActor "Spell")
    (bind _name (Default|GetRow _asbp_aicontroller _returnvalue))
    (bind _damage (CallFunction|ScaleDamage _name OtherActor))
    (Variables|Default|SetHP (- (Variables|Default|GetHP) _damage))
    (Default|Damage _asbp_aicontroller (Game|Player|GetPlayerPawn 0) :!label _label)
    ;[0.15 0.15 0.15 0.5] Destroys enemy when health is 0
    (if (<= (Variables|Default|GetHP) 0.0)
      (Physics|SetSimulatePhysics (Variables|Character|GetMesh) true)
      (CallFunction|GetYeeted OtherActor)
      (CallFunction|SpawnHealthup)
      (Utilities|IsValid _capsulecomponent
        (:Is%20Valid
          (Components|DestroyComponent _capsulecomponent))
        (:Is%20Not%20Valid
          _))
      (Utilities|Array|Add _tags "Dead")
      (if (Utilities|Array|ContainsItem _tags "WaveEnemy")
        (Default|FindWaveButton (Variables|Default|GetPlayerCharacter)))
      (AI|Logic|StopLogic (Variables|/Game/NPC_Comp/BP_AIController.BP_AIController_C|GetBehaviorTree (.AsBP%20AIController (Utilities|Casting|CastToBP_AIController (AI|GetAIController self)))) "")
      (Default|UpdateEnemyCount (.AsBP%20First%20Person%20Game%20Mode (Utilities|Casting|CastToBP_FirstPersonGameMode (Game|GetGameMode))))
      (Utilities|FlowControl|Delay 5.0)
      (Game|AddComponentbyClass "/Game/FirstPerson/Blueprints/BP_TransitionComponent.BP_TransitionComponent_C")
      (Utilities|FlowControl|Delay 7.0)
      (Actor|DestroyActor))
    (elif (== _returnvalue "/Game/Weapons/MeleeAttacks/BP_Sword.BP_Sword_C")
      (Variables|Default|SetHP (- (Variables|Default|GetHP) 6e+02))
      (goto _label))))

(event Custom|SpawnHealthup
  (if (Variables|Default|GetHealthupSpawned)
    (Development|PrintString "Unlucky" true true "(R=1.000000,G=0.000000,B=0.026847,A=1.000000)")
    (else
      (Variables|Default|SetHealthupSpawned true)
      (bind _returnvalue (Utilities|GetDataTableRow "/Game/DT_EnemiesCSV.DT_EnemiesCSV" "Knight")
        (:then
          (if (== (Math|Random|RandomIntegerinRange 0 (.DropHealthChance (Utilities|Struct|BreakEnemiesStructure _returnvalue))) (.DropHealthChance (Utilities|Struct|BreakEnemiesStructure _returnvalue)))
            (Game|SpawnActorfromClass "/Game/Inventory/Loot/HealthUp.HealthUp_C" (Transformation|GetActorTransform) "AlwaysSpawn" "MultiplyWithRoot" 0 0)))))))

(event Custom|GetYeeted
  (params (Spell :type Actor%20Object%20Reference))
  (bind _mesh (Variables|Character|GetMesh))
  (bind _rootcomponent (Variables|/Script/Engine.Actor|GetRootComponent Spell))
  (bind _returnvalue (Transformation|GetWorldLocation _rootcomponent))
  (bind _returnvalue_2 (Math|Vector|GetForwardVector _rootcomponent))
  ;[0.15 0.15 0.15 0.5] Adds the impulse based on the spell that hit it. If it's the combustion spell, it will apply forces different
  (bind _spellref1 (CallFunction|UglyAhhhCheckSpell Spell))
  (bind _returnvalue_3 (Utilities|GetDataTableRow "/Game/DataTables/Spells/DT_Spells.DT_Spells" _spellref1)
    (:then
      (if (== (.Spell (Utilities|Struct|BreakSpellStructure _returnvalue_3)) "/Game/Weapons/MagicAttacks/OfficialSpells/CombustionSpell/BP_Combustion.BP_Combustion_C")
        (Class|PhysicsObjectBlueprintLibrary|ApplyRadialImpulse _mesh _returnvalue 1e+03 (.x (* (* (/ (Transformation|GetWorldScale _rootcomponent) 1e+01) (.Impulse (Utilities|Struct|BreakSpellStructure _returnvalue_3))) (- 1.0 (/ (Math|Vector|Distance(Vector) _returnvalue (Transformation|GetWorldLocation (Variables|Default|GetHeart))) 7.5e+02)))) "RIF_Constant" false 0.0 false 0.0 1.0)
        (else
          (Utilities|IsValid Spell
            (:Is%20Valid
              (Physics|AddImpulseatLocation _mesh (* (.Impulse (Utilities|Struct|BreakSpellStructure _returnvalue_3)) _returnvalue_2) _returnvalue_2 "None"))))))))

(event Custom|DrainHealth
  (params (HealthDrain :type Float%20%28double-precision%29) (TimesToDrain :type Integer))
  ;[0.15 0.15 0.15 0.5] Drains health over a period of time
  (Variables|/Script/Engine.CharacterMovementComponent|SetMaxWalkSpeed (Variables|Character|GetCharacterMovement) 4e+02)
  (bind _output_get (Variables|Default|SetTimesDrained 0))
  (if (and (< _output_get TimesToDrain) (> (Variables|Default|GetHP) 0.0)) :!label _label
    (Variables|Default|SetHP (- (Variables|Default|GetHP) (* (Variables|/Game/FirstPerson/Blueprints/BP_FirstPersonPlayerController.BP_FirstPersonPlayerController_C|GetDrainBuff%25 (.AsBP%20First%20Person%20Player%20Controller (Utilities|Casting|CastToBP_FirstPersonPlayerController (Game|GetPlayerController 0)))) HealthDrain)))
    (Development|PrintString "Damaged" true true "(R=0.000000,G=0.660000,B=1.000000,A=1.000000)" 2.5)
    (Variables|Default|SetTimesDrained (+ (Variables|Default|GetTimesDrained) 1))
    (Utilities|FlowControl|Delay 1.0)
    (goto _label)
    (else
      (if (> (Variables|Default|GetHP) 0.0)
        _
        (else
          (CallFunction|HealthDrained)))
      (Variables|/Script/Engine.CharacterMovementComponent|SetMaxWalkSpeed (Variables|Character|GetCharacterMovement) 6e+02))))

(event Custom|Health%20Drained
  (bind _capsulecomponent (Variables|Collision|GetCapsuleComponent))
  (bind _tags (Variables|Actor|GetTags))
  ;[0.15 0.15 0.15 0.5] Destroys enemy when health is 0
  (if (<= (Variables|Default|GetHP) 0.0)
    (Physics|SetSimulatePhysics (Variables|Character|GetMesh) true)
    (CallFunction|GetYeeted (stale OnComponentBeginOverlap(CapsuleComponent) OtherActor))
    (CallFunction|SpawnHealthup)
    (Utilities|IsValid _capsulecomponent
      (:Is%20Valid
        (Components|DestroyComponent _capsulecomponent))
      (:Is%20Not%20Valid
        _))
    (Utilities|Array|Add _tags "Dead")
    (if (Utilities|Array|ContainsItem _tags "WaveEnemy")
      (Default|FindWaveButton (Variables|Default|GetPlayerCharacter)))
    (AI|Logic|StopLogic (Variables|/Game/NPC_Comp/BP_AIController.BP_AIController_C|GetBehaviorTree (.AsBP%20AIController (Utilities|Casting|CastToBP_AIController (AI|GetAIController self)))) "")
    (Default|UpdateEnemyCount (.AsBP%20First%20Person%20Game%20Mode (Utilities|Casting|CastToBP_FirstPersonGameMode (Game|GetGameMode))))
    (Utilities|FlowControl|Delay 5.0)
    (Game|AddComponentbyClass "/Game/FirstPerson/Blueprints/BP_TransitionComponent.BP_TransitionComponent_C")
    (Utilities|FlowControl|Delay 7.0)
    (Actor|DestroyActor)))

(event Custom|Stun
  (params (Origin :type Vector) (Impulse :type Float%20%28double-precision%29))
  ;[0.15 0.15 0.15 0.5] Stuns enemy for a short amount of time.
  (Character|LaunchCharacter (* Impulse (Math|Vector|GetUnitDirection(Vector) Origin (Transformation|GetActorLocation))) false false)
  (bind _asbp_aicontroller (Utilities|Casting|CastToBP_AIController (AI|GetAIController self)))
  (Variables|/Game/NPC_Comp/BP_AIController.BP_AIController_C|SetStunned _asbp_aicontroller true)
  (AI|Logic|StopLogic (Variables|/Game/NPC_Comp/BP_AIController.BP_AIController_C|GetBehaviorTree _asbp_aicontroller) "")
  (bind _returnvalue (Utilities|GetDataTableRow "/Game/DataTables/Enemies/DT_Enemies.DT_Enemies" "Knight")
    (:then
      (Utilities|FlowControl|Delay (.PulseWaveStunTime (Utilities|Struct|BreakEnemiesStructure _returnvalue)))
      (Class|BrainComponent|RestartLogic (Variables|/Game/NPC_Comp/BP_AIController.BP_AIController_C|GetBehaviorTree _asbp_aicontroller))
      (Variables|/Game/NPC_Comp/BP_AIController.BP_AIController_C|SetStunned _asbp_aicontroller false))))

(event EventBeginPlay
  (bind _returnvalue (AI|GetBlackboard 0))
  (for _array_element (Variables|Actor|GetTags)
    (Development|PrintString (Utilities|String|ToString(Name) _array_element)))
  ;[0.15 0.15 0.15 0.5] Sets the necessary blackboard values
  (bind _asbp_first_person_character (Utilities|Casting|CastToBP_FirstPersonCharacter (Game|Player|GetPlayerPawn 0))
    (:then
      (Variables|Default|SetPlayerCharacter _asbp_first_person_character)
      (Variables|Default|SetPlayerController (.AsBP%20First%20Person%20Player%20Controller (Utilities|Casting|CastToBP_FirstPersonPlayerController (Game|GetPlayerController 0)))))
    (:CastFailed
      _))
  (bind _asbp_aicontroller (Utilities|Casting|CastToBP_AIController (AI|GetAIController self))
    (:then
      (Variables|/Game/NPC_Comp/BP_AIController.BP_AIController_C|SetBehaviorTreeAsset _asbp_aicontroller "/Game/Enemies/FallenAngel/Attacks/Summon/BT_FallenAngelSummon.BT_FallenAngelSummon")
      (Variables|/Game/NPC_Comp/BP_AIController.BP_AIController_C|SetDetectionRadius _asbp_aicontroller (Variables|Default|GetDetectionRange))
      (Utilities|FlowControl|Delay 0.2)
      (Variables|Default|SetBlackboard _returnvalue)
      (Class|BlackboardComponent|SetValueasName _returnvalue (Variables|Default|GetDataTableRow) "FallenAngelSummon")
      (bind _returnvalue_2 (Utilities|GetDataTableRow "/Game/DataTables/Enemies/DT_Enemies.DT_Enemies" "FallenAngelSummon")
        (:then
          (Variables|Default|SetHP (.MaxHP (Utilities|Struct|BreakEnemiesStructure _returnvalue_2)))
          (AI|Components|Blackboard|SetValueasFloat (Variables|Default|GetBlackboard) (Variables|Default|GetSpellCooldown) (.AttackCooldown (Utilities|Struct|BreakEnemiesStructure _returnvalue_2)))
          (AI|Components|Blackboard|SetValueasFloat (Variables|Default|GetBlackboard) (Variables|Default|GetLOSTime) (.ChaseTime (Utilities|Struct|BreakEnemiesStructure _returnvalue_2)))
          (AI|Components|Blackboard|SetValueasEnum (Variables|Default|GetBlackboard) (Variables|Default|GetPatrols) (Variables|Default|GetPatrolBehavior))
          (AI|Components|Blackboard|SetValueasFloat (Variables|Default|GetBlackboard) (Variables|Default|GetRadius) (Variables|Default|GetPatrolRadius))
          (AI|Components|Blackboard|SetValueasBool (Variables|Default|GetBlackboard) (Variables|Default|GetBBCanHear) (Variables|Default|GetCanHear))
          (AI|Components|Blackboard|SetValueasFloat (Variables|Default|GetBlackboard) (Variables|Default|GetBBSightRadius) (Variables|Default|GetSightRadius))
          (AI|Components|Blackboard|SetValueasBool (Variables|Default|GetBlackboard) (Variables|Default|GetHasLineOfSight) true)
          (AI|Components|Blackboard|SetValueasObject (Variables|Default|GetBlackboard) (Variables|Default|GetPlayerActor) (Game|Player|GetPlayerPawn 0))
          (AI|Components|Blackboard|SetValueasBool (Variables|Default|GetBlackboard) (Variables|Default|GetChasingPlayer) true))))
    (:CastFailed
      (Development|PrintString "Cast failed"))))

(fn ConstructionScript)

(fn UglyAhhhCheckSpell
  (params (Spell :type Actor%20Object%20Reference))
  (bind _returnvalue (Utilities|GetClass Spell))
  (bind _outrownames (DataTable|GetDataTableRowNames "/Game/DataTables/Spells/DT_Spells.DT_Spells"))
  (bind _array_element (Utilities|Array|ForEachLoopwithBreak _outrownames :!label _label)
    (:LoopBody
      (bind _returnvalue_2 (Utilities|GetDataTableRow "/Game/DataTables/Spells/DT_Spells.DT_Spells" _array_element)
        (:then
          (if (== (.Spell (Utilities|Struct|BreakSpellStructure _returnvalue_2)) _returnvalue)
            (LocalVariables|SetSpellFound true)
            (LocalVariables|SetSpellRef _array_element)
            (goto _label Break)))))
    (:Completed
      (if (LocalVariables|GetSpellFound)
        (return (LocalVariables|GetSpellRef))
        (else
          (Development|PrintString (Utilities|GetClassDisplayName _returnvalue)))))))

(fn ScaleDamage
  (params (SpellRow :type Name) (SpellActor :type Actor%20Object%20Reference))
  (bind _returnvalue (Math|Random|RandomIntegerinRange 8 12))
  ;[0.15 0.15 0.15 0.5] Checks if the spell is a charge spell. If so, scales its damage accordingly. If Toxic Thorn, initiates health drain.
  (bind _returnvalue_2 (Utilities|GetDataTableRow "/Game/DataTables/Spells/DT_Spells.DT_Spells" SpellRow)
    (:then
      (if (Utilities|Enum|Equal(Enum) (.SpellType (Utilities|Struct|BreakSpellStructure _returnvalue_2)) "NewEnumerator3")
        (if (== (.Spell (Utilities|Struct|BreakSpellStructure _returnvalue_2)) "/Game/Weapons/MagicAttacks/OfficialSpells/CombustionSpell/BP_Combustion.BP_Combustion_C")
          (return (.X (Math|Vector|BreakVector (* (/ (Transformation|GetActorScale3D SpellActor) 1e+01) (.SpellDamage (Utilities|Struct|BreakSpellStructure _returnvalue_2))))))
          (elif (> (/ (- (.Lifetime (Utilities|Struct|BreakSpellStructure _returnvalue_2)) (Actor|GetLifeSpan SpellActor)) 3.0) 1.0)
            (CallFunction|DrainHealth (.SpellDamage (Utilities|Struct|BreakSpellStructure _returnvalue_2)) _returnvalue)
            (return 0.0)
            (else
              (CallFunction|DrainHealth (* (/ (- (.Lifetime (Utilities|Struct|BreakSpellStructure _returnvalue_2)) (Actor|GetLifeSpan SpellActor)) 3.0) (.SpellDamage (Utilities|Struct|BreakSpellStructure _returnvalue_2))) _returnvalue)
              (return 0.0))))
        (else
          (if (== (.Spell (Utilities|Struct|BreakSpellStructure _returnvalue_2)) "/Game/Weapons/MagicAttacks/OfficialSpells/PulseWave/BP_PulseWave.BP_PulseWave_C")
            (CallFunction|Stun (Transformation|GetActorLocation SpellActor) (.Impulse (Utilities|Struct|BreakSpellStructure _returnvalue_2))))
          (return (.SpellDamage (Utilities|Struct|BreakSpellStructure _returnvalue_2))))))))