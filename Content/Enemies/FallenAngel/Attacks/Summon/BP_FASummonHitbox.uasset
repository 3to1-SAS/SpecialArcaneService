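; BP_FASummonHitbox is a short-lived attack hitbox for the Fallen Angel boss's summon attack.
; It reads its lifespan from the BossSummonAttack row of DT_EnemySpells, then destroys itself.
; Each tick it snaps just in front of OwnerEnemy, matching its rotation.
; After an overlap it waits a tick and drops its EnemySpell tag if the first-person character is overlapping, preventing multiple hits.
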(event OnComponentBeginOverlap(Cube)
  (params (OverlappedComponent :type Primitive%20Component%20Object%20Reference) (OtherActor :type Actor%20Object%20Reference) (OtherComp :type Primitive%20Component%20Object%20Reference) (OtherBodyIndex :type Integer) (bFromSweep :type Boolean) (SweepResult :type Hit%20Result%20Structure%20%28by%20ref%29))
  ;[0.15 0.15 0.15 0.5] Removes the tag after hitting to prevent multihits
  (Utilities|FlowControl|DelayUntilNextTick)
  (bind _array_element (Utilities|Array|ForEachLoopwithBreak (Collision|GetOverlappingActors 0 :!class /Script/Engine.Actor) :!label _label)
    (:LoopBody
      (if (== (Utilities|GetClass _array_element) "/Game/FirstPerson/Blueprints/BP_FirstPersonCharacter.BP_FirstPersonCharacter_C")
        (Utilities|Array|RemoveItem (Variables|Actor|GetTags) "EnemySpell")
        (goto _label Break)))))

(event EventTick
  (params (DeltaSeconds :type Float%20%28single-precision%29))
  (bind _ownerenemy (Variables|Default|GetOwnerEnemy))
  (bind _returnvalue (Transformation|GetActorTransform _ownerenemy))
  ;[0.15 0.15 0.15 0.5] Makes the hitbox move with the enemy
  (if (Utilities|IsValid _ownerenemy)
    (Transformation|SetActorTransform (Math|Transform|MakeTransform (+ (.location _returnvalue) (* (Transformation|GetActorForwardVector _ownerenemy) "100.000000,100.000000,0.000000")) (.rotation _returnvalue) (Transformation|GetActorScale3D)))))

(event EventBeginPlay
  ;[0.15 0.15 0.15 0.5] Destroys Hitbox After Short Delay
  (bind _returnvalue (Utilities|GetDataTableRow "/Game/DataTables/Enemies/EnemySpells/DT_EnemySpells.DT_EnemySpells" "BossSummonAttack")
    (:then
      (Utilities|FlowControl|Delay (.lifespan _returnvalue))
      (Actor|DestroyActor))))

(fn ConstructionScript)