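; BP_DemoEnemy is a test enemy that fires at the player and spawns an extract through the game mode when killed.
; Capsule overlaps subtract HP, using DT_Spells damage looked up by spell class or a fixed amount for the sword, then share one death check.
; A placeholder attack loop turns it toward the player and spawns BP_DemoEnemyAttack every two seconds by re-calling SpellFire after a delay.
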(event OnComponentBeginOverlap(Capsule)
  (params (OverlappedComponent :type Primitive%20Component%20Object%20Reference) (OtherActor :type Actor%20Object%20Reference) (OtherComp :type Primitive%20Component%20Object%20Reference) (OtherBodyIndex :type Integer) (bFromSweep :type Boolean) (SweepResult :type Hit%20Result%20Structure%20%28by%20ref%29))
  (bind _returnvalue (Utilities|GetClass OtherActor))
  ;[0.15 0.15 0.15 0.5] Reduce enemy HP on hit based on spell or sword
  (if (Actor|ActorHasTag OtherActor "Spell")
    (bind _returnname (CallFunction|GetRowName _returnvalue))
    (bind _returnvalue_2 (Utilities|GetDataTableRow "/Game/Weapons/Spells/DT_Spells.DT_Spells" _returnname)
      (:then
        (Variables|Default|SetHP (- (Variables|Default|GetHP) (.SpellDamage (Utilities|Struct|BreakSpellStructure _returnvalue_2))))
        ;[0.15 0.15 0.15 0.5] Destroy enemy when HP reaches 0
        (if (<= (Variables|Default|GetHP) 0.0) :!label _label
          (Actor|DestroyActor)
          (bind _asbp_first_person_game_mode (Utilities|Casting|CastToBP_FirstPersonGameMode (Game|GetGameMode)))
          (Default|SpawnExtract _asbp_first_person_game_mode))))
    (elif (== _returnvalue "/Game/Weapons/MeleeAttacks/BP_Sword.BP_Sword_C")
      (Variables|Default|SetHP (- (Variables|Default|GetHP) 6e+02))
      (goto _label))))

(event Custom|SpellFire
  (bind _returnvalue (Transformation|GetActorTransform))
  ;[0.15 0.15 0.15 0.5] Fires a spell every second. (only for testing, will be replaced once ai is complete)
  (Transformation|SetActorRotation (Math|Rotator|FindLookatRotation (.location (Transformation|GetActorTransform)) (Transformation|GetActorLocation (Game|Player|GetPlayerPawn 0))))
  (Game|SpawnActorfromClass "/Game/Enemies/BP_DemoEnemyAttack.BP_DemoEnemyAttack_C" (Math|Transform|MakeTransform (.location _returnvalue) (.rotation _returnvalue) "1.000000,1.000000,1.000000") "Undefined" "MultiplyWithRoot" 0 0)
  (Utilities|FlowControl|Delay 2.0)
  (CallFunction|SpellFire))

(event EventBeginPlay
  (Utilities|FlowControl|Delay 2.0)
  (CallFunction|SpellFire))

(fn ConstructionScript)

(fn GetRowName
  (params (Class :type Actor%20Class%20Reference))
  (if (== Class "/Game/Weapons/Spells/BP_BasicSpell.BP_BasicSpell_C")
    (return "BasicSpell")
    (elif (== Class "/Game/Weapons/Spells/BP_RapidSpell.BP_RapidSpell_C")
      (return "RapidSpell")
      (elif (== Class "/Game/Weapons/Spells/BP_ExplosiveSpell.BP_ExplosiveSpell_C")
        (return "ExplosiveSpell")))))