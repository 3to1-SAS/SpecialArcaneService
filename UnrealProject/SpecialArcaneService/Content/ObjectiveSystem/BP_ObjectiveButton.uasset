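; One-shot objective button that the player presses to update their mission and trigger the extraction spawn.
; A box overlap shows or hides the character's interact prompt and stores the player, so "looked at" really means standing in the box.
; The actor takes input directly; InteractWithE while in range calls UpdateObjective on the character, plays a click and calls SpawnExtract on the game mode.
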(event OnComponentBeginOverlap(Box)
  (params (OverlappedComponent :type Primitive%20Component%20Object%20Reference) (OtherActor :type Actor%20Object%20Reference) (OtherComp :type Primitive%20Component%20Object%20Reference) (OtherBodyIndex :type Integer) (bFromSweep :type Boolean) (SweepResult :type Hit%20Result%20Structure%20%28by%20ref%29))
  ;[0.15 0.15 0.15 0.5] Shows prompt when looked at
  (bind _asbp_first_person_character (Utilities|Casting|CastToBP_FirstPersonCharacter OtherActor))
  (Default|DisplayInteractivePrompt _asbp_first_person_character (Variables|Default|GetPromptText) true)
  (Variables|Default|SetIsLookedAt true)
  (Variables|Default|SetplayerLookingAt OtherActor))

(event OnComponentEndOverlap(Box)
  (params (OverlappedComponent :type Primitive%20Component%20Object%20Reference) (OtherActor :type Actor%20Object%20Reference) (OtherComp :type Primitive%20Component%20Object%20Reference) (OtherBodyIndex :type Integer))
  ;[0.15 0.15 0.15 0.5] Shows prompt when looked at
  (bind _asbp_first_person_character (Utilities|Casting|CastToBP_FirstPersonCharacter OtherActor))
  (Default|DisplayInteractivePrompt _asbp_first_person_character (Variables|Default|GetPromptText) false)
  (Variables|Default|SetIsLookedAt false)
  (Variables|Default|SetplayerLookingAt 0))

(event EventBeginPlay
  (Input|EnableInput (Game|GetPlayerController 0)))

(event Input|ActionEvents|InputActionInteractWithE
  (params (Key :type Key%20Structure :default "None"))
  ;[0.15 0.15 0.15 0.5] When interacted with, sets objective and plays sound
  (:Pressed
    ;;[0.15 0.15 0.15 0.5] Checks if the player's looking
    (Development|PrintString "pressed")
    (if (Variables|Default|GetIsLookedAt)
      (bind _asbp_first_person_character (Utilities|Casting|CastToBP_FirstPersonCharacter (Variables|Default|GetplayerLookingAt)))
      (Utilities|FlowControl|DoOnce false
        (:Completed
          (Default|UpdateObjective _asbp_first_person_character (Variables|Default|GetupdateObjective) true)
          (Audio|PlaySound2D "/Game/ObjectiveSystem/buttonclicksoundtrust.buttonclicksoundtrust" 1.0 1.0 0.0 0 0 false)
          (bind _asbp_first_person_game_mode (Utilities|Casting|CastToBP_FirstPersonGameMode (Game|GetGameMode)))
          (Default|SpawnExtract _asbp_first_person_game_mode))))))

(fn ConstructionScript)