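; BP_SpellFiring handles the player's demo spell attack, gated by a disabled flag, a cooldown and a mana cost.
; The SpellAttack event checks the mana on BP_FirstPersonPlayerController, then spawns BP_DemoSpell near the player's eye point along the aim rotation.
; Firing deducts mana from the controller and clears IsFireable until a short delay restores it.
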(event Custom|SpellAttack
  (bind _returnvalue (Game|Player|GetPlayerPawn 0))
  (bind _returnvalue_2 (Pawn|GetBaseAimRotation _returnvalue))
  ;[0.15 0.15 0.15 0.5] Checks if spell is on cooldown and player has enough mana
  (if (not (Variables|Default|GetDisabled))
    (bind _returnvalue_3 (Actor|GetActorOfClass "/Game/FirstPerson/Blueprints/BP_FirstPersonPlayerController.BP_FirstPersonPlayerController_C"))
    (if (and (Variables|Default|GetIsFireable) (>= (Variables|/Game/FirstPerson/Blueprints/BP_FirstPersonPlayerController.BP_FirstPersonPlayerController_C|GetMana _returnvalue_3) 1e+02))
      ;[0.15 0.15 0.15 0.5] Spawn Spell, spend mana, and turn off cooldown after 0.75 seconds
      (Game|SpawnActorfromClass "/Game/Weapons/DemoSpell/BP_DemoSpell.BP_DemoSpell_C" (Math|Transform|MakeTransform (+ (.OutLocation (Actor|GetActorEyesViewPoint _returnvalue)) (* (Math|Vector|GetForwardVector _returnvalue_2) "25.000000,0.000000,0.000000")) _returnvalue_2 "1.000000,1.000000,1.000000") "Undefined" "MultiplyWithRoot" 0 0)
      (Variables|Default|SetIsFireable false)
      (bind _returnvalue_4 (Actor|GetActorOfClass "/Game/FirstPerson/Blueprints/BP_FirstPersonPlayerController.BP_FirstPersonPlayerController_C"))
      (Variables|/Game/FirstPerson/Blueprints/BP_FirstPersonPlayerController.BP_FirstPersonPlayerController_C|SetMana _returnvalue_4 (- (Variables|/Game/FirstPerson/Blueprints/BP_FirstPersonPlayerController.BP_FirstPersonPlayerController_C|GetMana _returnvalue_4) 1e+02))
      (Utilities|FlowControl|Delay 0.75)
      (Variables|Default|SetIsFireable true))))