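; BP_SpellFiring fires the player's equipped spell when BasicSpellShoot runs and the spell is selected.
; It looks up EquippedSpell from the first-person controller in the SpellsData table, then checks cooldown and the controller's mana.
; It spawns the row's spell actor near the eye point along aim rotation, offset only on world X, and deducts mana.
; A Delay using the row's FireRate restores IsFireable, acting as the cooldown.
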(event Custom|BasicSpellShoot
  (bind _returnvalue (Game|Player|GetPlayerPawn 0))
  (bind _returnvalue_2 (Pawn|GetBaseAimRotation _returnvalue))
  ;[0.15 0.15 0.15 0.5] Checks if spell is on cooldown and player has enough mana
  ;;[0.15 0.15 0.15 0.5] Check if spell is selected
  (if (Variables|Default|GetSelected)
    (bind _returnvalue_3 (Actor|GetActorOfClass "/Game/FirstPerson/Blueprints/BP_FirstPersonPlayerController.BP_FirstPersonPlayerController_C"))
    (bind _returnvalue_4 (Utilities|GetDataTableRow (Variables|Default|GetSpellsData) (Variables|/Game/FirstPerson/Blueprints/BP_FirstPersonPlayerController.BP_FirstPersonPlayerController_C|GetEquippedSpell _returnvalue_3))
      (:then
        (Development|PrintString "spell successfully found yay")
        (if (and (Variables|Default|GetIsFireable) (>= (Variables|/Game/FirstPerson/Blueprints/BP_FirstPersonPlayerController.BP_FirstPersonPlayerController_C|GetMana _returnvalue_3) (.ManaConsumption (Utilities|Struct|BreakSpellStructure _returnvalue_4))))
          ;[0.15 0.15 0.15 0.5] Spawn Spell, spend mana, and turn off cooldown after spell's default firerate
          (Game|SpawnActorfromClass (.Spell (Utilities|Struct|BreakSpellStructure _returnvalue_4)) (Math|Transform|MakeTransform (+ (.OutLocation (Actor|GetActorEyesViewPoint _returnvalue)) (* (Math|Vector|GetForwardVector _returnvalue_2) "25.000000,0.000000,0.000000")) _returnvalue_2 "1.000000,1.000000,1.000000") "Undefined" "MultiplyWithRoot" 0 0)
          (Development|PrintString "spell spawned")
          (Variables|Default|SetIsFireable false)
          (bind _returnvalue_5 (Actor|GetActorOfClass "/Game/FirstPerson/Blueprints/BP_FirstPersonPlayerController.BP_FirstPersonPlayerController_C"))
          (Variables|/Game/FirstPerson/Blueprints/BP_FirstPersonPlayerController.BP_FirstPersonPlayerController_C|SetMana _returnvalue_5 (- (Variables|/Game/FirstPerson/Blueprints/BP_FirstPersonPlayerController.BP_FirstPersonPlayerController_C|GetMana _returnvalue_5) (.ManaConsumption (Utilities|Struct|BreakSpellStructure _returnvalue_4))))
          (Utilities|FlowControl|Delay (.FireRate (Utilities|Struct|BreakSpellStructure _returnvalue_4)))
          (Variables|Default|SetIsFireable true))))))